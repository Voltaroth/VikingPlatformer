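; Base Blueprint for destructible objects such as crates, exposing health and damage functions backed by a DamageSystemComponent.
; Health getters and TakeDamage forward to the component, while Heal and SetMaxHealth are stubs that return zero.
; The construction script binds the component's death event, and the OnDeath event only prints a crate-destroyed debug message.
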(event Custom|OnDeath
  (Development|PrintString "CRATE DESTROYED"))

(fn ConstructionScript
  (EventDispatchers|BindEventtoOnDeath (Variables|Default|GetDamageSystemComponent) (EventDispatchers|CreateEvent :!event Custom|OnDeath)))

(fn GetCurrentHealth
  (return (Variables|/Game/Blueprints/DamageSystem/AC_DamageSystemComponent.AC_DamageSystemComponent_C|GetHealthCurrent (Variables|Default|GetDamageSystemComponent))))

(fn GetMaxHealth
  (return (Variables|/Game/Blueprints/DamageSystem/AC_DamageSystemComponent.AC_DamageSystemComponent_C|GetHealthMax (Variables|Default|GetDamageSystemComponent))))

(fn Heal
  (params (Amount :type Integer))
  (return 0))

(fn SetMaxHealth
  (params (Amount :type Integer))
  (return 0 0))

(fn TakeDamage
  (params (DamageInfo :type S%20Damage%20Info%20Structure))
  (bind _wasdamaged_ (Default|TakeDamage (Variables|Default|GetDamageSystemComponent) DamageInfo))
  (return _wasdamaged_))