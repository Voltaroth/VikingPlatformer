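; BP_Collectible is a pickup that animates toward whoever collects it, then destroys itself.
; On trigger overlap with an actor holding AC_Collection, a DoOnce gate calls that component's PickUp if CanPickUp allows, otherwise it resets.
; A Height timeline lifts the item, then an Attraction timeline lerps it from its current location toward the collector's live position while driving its scale.
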(event OnComponentBeginOverlap(Trigger)
  (params (OverlappedComponent :type Primitive%20Component%20Object%20Reference) (OtherActor :type Actor%20Object%20Reference) (OtherComp :type Primitive%20Component%20Object%20Reference) (OtherBodyIndex :type Integer) (bFromSweep :type Boolean) (SweepResult :type Hit%20Result%20Structure%20%28by%20ref%29))
  (bind _returnvalue (Actor|GetComponentbyClass OtherActor "/Game/Blueprints/ActorComponents/Player/Collection/AC_Collection.AC_Collection_C"))
  (bind _returnvalue_2 (Transformation|GetActorLocation))
  (Utilities|IsValid _returnvalue
    (:Is%20Valid
      (Variables|Default|SetCollector _returnvalue)
      (Utilities|FlowControl|DoOnce false :!label _label
        (:Completed
          (if (Variables|/Game/Blueprints/ActorComponents/Player/Collection/AC_Collection.AC_Collection_C|GetCanPickUp (Variables|Default|GetCollector))
            (Default|PickUp (Variables|Default|GetCollector))
            (bind _height (Timeline|Height PlayFromStart)
              (:Update
                (Transformation|SetActorLocation (Math|Vector|Lerp(Vector) _returnvalue_2 (+ _returnvalue_2 "0.000000,0.000000,15.000000") _height) false false))
              (:Finished
                (bind (_direction _distance_normalized_ _scale) (Timeline|Attraction PlayFromStart)
                  (:Update
                    (Transformation|SetActorLocation (Math|Vector|Lerp(Vector) (Transformation|GetActorLocation) (Transformation|GetActorLocation (Components|GetOwner (Variables|Default|GetCollector))) _distance_normalized_) false false)
                    (Transformation|SetActorScale3D (Math|Conversions|ToVector(Float) _scale)))
                  (:Finished
                    (Actor|DestroyActor)))))
            (else
              (goto _label Reset))))))))

(event EventBeginPlay
  (Variables|Default|SetPickupLocation (Transformation|GetActorLocation)))

(fn ConstructionScript)