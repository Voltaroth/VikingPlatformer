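; A health pack collectible that calls SetMaxHealth with a fixed value on the player's damage system component.
; On actor overlap, it gets the player through the BPI_Interact interface and reads that component's Health.
; The pickup applies and destroys itself only when Health is below that same hardcoded threshold, otherwise it stays in the level.
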(event Collision|EventActorBeginOverlap
  (params (OtherActor :type Actor%20Object%20Reference))
  (if (Utilities|DoesObjectImplementInterface OtherActor "/Game/Blueprints/AbilityActorComponents/Player/Collection/BPI_Interact.BPI_Interact_C")
    (bind _player (Class|BPIInteract|GetPlayer(Message) OtherActor))
    (Utilities|IsValid _player
      (:Is%20Valid
        (bind _output_get (Variables|Default|SetActorToHeal (Variables|/Game/Blueprints/Character/BP_Player.BP_Player_C|GetDamageSystemComponent _player)))
        (if (< (Variables|/Game/Blueprints/DamageSystem/AC_DamageSystemComponent.AC_DamageSystemComponent_C|GetHealth (Variables|/Game/Blueprints/Character/BP_Player.BP_Player_C|GetDamageSystemComponent _player)) 6)
          (Default|SetMaxHealth _output_get 6)
          (Actor|DestroyActor))))))

(fn ConstructionScript)