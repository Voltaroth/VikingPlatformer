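; Health pack collectible that restores health to the player when overlapped.
; On begin overlap it uses the BPI_Interact interface to get a player reference from the other actor, then reads that player's DamageSystemComponent.
; If health is below maximum, it heals by a single point and destroys itself; at full health the pack stays in place.
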(event Collision|EventActorBeginOverlap
  (params (OtherActor :type Actor%20Object%20Reference))
  (if (Utilities|DoesObjectImplementInterface OtherActor "/Game/Blueprints/AbilityActorComponents/Player/Collection/BPI_Interact.BPI_Interact_C")
    (bind _player (Class|BPIInteract|GetPlayer(Message) OtherActor))
    (Utilities|IsValid _player
      (:Is%20Valid
        (bind _output_get (Variables|Default|SetActorToHeal (Variables|/Game/Blueprints/Character/BP_Player.BP_Player_C|GetDamageSystemComponent _player)))
        (if (< (Variables|/Game/Blueprints/DamageSystem/AC_DamageSystemComponent.AC_DamageSystemComponent_C|GetHealth _output_get) (Variables|/Game/Blueprints/DamageSystem/AC_DamageSystemComponent.AC_DamageSystemComponent_C|GetMaxHealth _output_get))
          (Default|Heal _output_get 1)
          (Actor|DestroyActor))))))

(fn ConstructionScript)