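; Actor component that manages health, healing, damage and death for its owner.
; TakeDamage routes hits through invincibility, blocking and death checks, then fires blocked, death or damage-response dispatchers, with responses gated by interruptability or forced interrupts.
; Heal clamps to max health, SetMaxHealth refills it, and Die fires the death dispatcher directly.
; A timer-based hit-stop freezes owner and damager through CustomTimeDilation, but its call in TakeDamage is disconnected.
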(event Custom|StartHitStop
  (params (HitStopDuration :type Float%20%28double-precision%29) (DamageActor :type Actor%20Object%20Reference))
  (Utilities|IsValid DamageActor
    (:Is%20Valid
      (Variables|/Script/Engine.Actor|SetCustomTimeDilation DamageActor 0.0)
      (Variables|/Script/Engine.Actor|SetCustomTimeDilation (Components|GetOwner) 0.0)
      (Utilities|Time|SetTimerbyEvent (delegate Custom|EndHitStop) HitStopDuration))))

(event Custom|EndHitStop
  (Variables|/Script/Engine.Actor|SetCustomTimeDilation (stale Custom|StartHitStop DamageActor) 1.0)
  (Variables|/Script/Engine.Actor|SetCustomTimeDilation (Components|GetOwner) 1.0))

(event EventBeginPlay
  (Variables|Default|SetHealthCurrent (Variables|Default|GetHealthCurrent))
  (Variables|Default|SetHealthMax (Variables|Default|GetHealthMax)))

(fn Heal
  (params (Amount :type Integer))
  (if (not (Variables|Default|GetIsDead?))
    (bind _output_get (Variables|Default|SetHealthCurrent (Math|Integer|Clamp(Integer) (+ Amount (Variables|Default|GetHealthCurrent)) 0 (Variables|Default|GetHealthMax))))
    (return _output_get)))

(fn TakeDamage
  (params (DamageInfo :type S%20Damage%20Info%20Structure))
  (bind (_amount _damagetype _damageresponse _shoulddamageinvincible_ _shouldforceinterrupt_ _damagingactor _hitstopduration) (Utilities|Struct|BreakS_DamageInfo DamageInfo))
  (Utilities|CanbeDamaged _shoulddamageinvincible_
    (:BlockDamage
      (Default|CallOnBlocked)
      (return false))
    (:DoDamage
      (bind _output_get (Variables|Default|SetHealthCurrent (- (Variables|Default|GetHealthCurrent) _amount)))
      (if (<= _output_get 0)
        (Variables|Default|SetIsDead? true)
        (Default|CallOnDeath)
        (return true)
        (elif (or (Variables|Default|GetIsInterruptable?) _shouldforceinterrupt_)
          (Default|CallOnDamageResponse _damageresponse)
          (return true))))
    (:NoDamage
      (return false))))

(fn Die
  (if (not (Variables|Default|GetIsDead?))
    (Default|CallOnDeath)))

(fn SetMaxHealth
  (params (Amount :type Integer))
  (bind _output_get (Variables|Default|SetHealthMax Amount))
  (bind _output_get_2 (Variables|Default|SetHealthCurrent _output_get))
  (return _output_get _output_get_2))