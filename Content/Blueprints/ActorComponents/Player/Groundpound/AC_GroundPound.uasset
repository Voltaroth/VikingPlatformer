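; Player actor component that implements the Mjölnir ground pound, bound to BP_Player's ground pound call and landed delegates.
; With the hammer in hand, a jumping, double-jumping or falling player loses input, slows and plays paired character and hammer montages.
; A montage notify triggers a fast downward launch after a short delay; landing adds squeeze and a bounce, stops montages and restores input.
; DashCooldown gates reuse.
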(event Custom|GroundPound
  (bind _movementcomponent (Variables|Default|GetMovementComponent))
  (bind _player (Variables|Default|GetPlayer))
  (bind _returnvalue (Transformation|GetVelocity _player))
  (if (and (Variables|/Game/Blueprints/Character/BP_Player.BP_Player_C|GetIsMjölnirInHand? (Variables|Default|GetPlayer)) (Variables|Default|GetCanGroundPound))
    (switch Utilities|FlowControl|Switch|SwitchonENUM_MovementState (Variables|/Game/Blueprints/ActorComponents/Player/MovementState/AC_MovementStateComponent.AC_MovementStateComponent_C|GetMovementState (Variables|/Game/Blueprints/Character/BP_Player.BP_Player_C|GetMovementStateComponent (Variables|Default|GetPlayer)))
      (:NewEnumerator1
        _)
      (:NewEnumerator5
        _)
      (:NewEnumerator0
        _))
    (Input|DisableInput (Variables|Default|GetPlayer) (Game|GetPlayerController 0))
    (Variables|Default|SetCanGroundPound false)
    (Variables|Default|SetDidGroundPound true)
    (Variables|/Script/Engine.MovementComponent|SetVelocity _movementcomponent (Math|Vector|MakeVector (.x (Variables|/Script/Engine.MovementComponent|GetVelocity _movementcomponent)) (.y (Variables|/Script/Engine.MovementComponent|GetVelocity _movementcomponent)) 0.0))
    (Character|LaunchCharacter _player (Math|Vector|MakeVector (/ (.x _returnvalue) 8.0) (/ (.y _returnvalue) 8.0) 0.0) true false)
    (Variables|/Game/Blueprints/ActorComponents/Player/MovementState/AC_MovementStateComponent.AC_MovementStateComponent_C|SetMovementState (Variables|/Game/Blueprints/Character/BP_Player.BP_Player_C|GetMovementStateComponent (Variables|Default|GetPlayer)) "NewEnumerator19")
    (bind _notifyname (Animation|Montage|PlayMontage (Variables|/Script/Engine.Character|GetMesh (Variables|Default|GetPlayer)) "/Game/Assets/Characters/Leif/Skeletal_Mesh/Leif_Animations/ANIM_Leif_GroundPound_Montage.ANIM_Leif_GroundPound_Montage")
      (:then
        (Animation|Montage|PlayMontage (Variables|/Game/Blueprints/Character/BP_Player.BP_Player_C|GetSKM_Mjölnir (Variables|Default|GetPlayer)) "/Game/Assets/Characters/Leif/Skeletal_Mesh/Mjölnir/Mjölnir_Animations/ANIM_Mjölnir_GroundPound_Montage.ANIM_Mjölnir_GroundPound_Montage"
          (:then
            (Default|JumpSqueeze (Variables|Default|GetPlayer))
            (Utilities|FlowControl|Delay (Variables|Default|GetDashCooldown))
            (Variables|Default|SetCanGroundPound true))))
      (:OnNotifyBegin
        (switch name _notifyname
          (:BeginDrop
            (Utilities|FlowControl|Delay 0.1)
            (Character|LaunchCharacter (Variables|Default|GetPlayer) "0.000000,0.000000,-5000.000000" false true)))))))

(event Custom|Landed
  (params (Hit :type Hit%20Result%20Structure%20%28by%20ref%29))
  (bind _player (Variables|Default|GetPlayer))
  (if (Variables|Default|GetDidGroundPound)
    (Variables|Default|SetDidGroundPound false)
    (Default|LandSqueeze _player)
    (Utilities|FlowControl|Delay 0.1)
    (Character|LaunchCharacter (Variables|Default|GetPlayer) "0.000000,0.000000,400.000000" false true)
    (Animation|Montage|MontageStop (Components|SkeletalMesh|GetAnimInstance (Variables|/Script/Engine.Character|GetMesh _player)) 0.2 "/Game/Assets/Characters/Leif/Skeletal_Mesh/Leif_Animations/ANIM_Leif_GroundPound_Montage.ANIM_Leif_GroundPound_Montage")
    (Animation|Montage|MontageStop (Components|SkeletalMesh|GetAnimInstance (Variables|/Game/Blueprints/Character/BP_Player.BP_Player_C|GetSKM_Mjölnir (Variables|Default|GetPlayer))) 0.2 "/Game/Assets/Characters/Leif/Skeletal_Mesh/Mjölnir/Mjölnir_Animations/ANIM_Mjölnir_GroundPound_Montage.ANIM_Mjölnir_GroundPound_Montage")
    (Input|EnableInput (Variables|Default|GetPlayer) (Game|GetPlayerController 0))))

(event EventBeginPlay
  (bind _returnvalue (Components|GetOwner))
  (bind _returnvalue_2 (Actor|GetComponentbyClass _returnvalue "/Script/Engine.CharacterMovementComponent"))
  (Utilities|IsValid _returnvalue_2
    (:Is%20Valid
      (Variables|Default|SetMovementComponent _returnvalue_2)
      (Utilities|IsValid (Actor|GetComponentbyClass _returnvalue "AC_GroundPound_C")
        (:Is%20Valid
          (bind _asbp_player (Utilities|Casting|CastToBP_Player _returnvalue))
          (bind _output_get (Variables|Default|SetPlayer _asbp_player))
          (EventDispatchers|BindEventtoStartGroundPoundCall _output_get (EventDispatchers|CreateEvent :!event Custom|GroundPound))
          (EventDispatchers|BindEventtoLandedDelegate _output_get (EventDispatchers|CreateEvent :!event Custom|Landed)))))))

(event EventTick
  (params (DeltaSeconds :type Float%20%28single-precision%29)))