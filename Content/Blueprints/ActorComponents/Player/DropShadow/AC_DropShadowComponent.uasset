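; Actor component that projects a downward decal drop shadow beneath its owner, as either a blob or a captured shape.
; Setup disables decals on owner meshes and, in render-texture mode, adds an owner-only orthographic depth capture feeding the material.
; Each tick, a ring of downward traces finds the closest and furthest ground.
; These distances size and position the decal and drive opacity plus curve-based blur or density, recapturing manually when updated.
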(event EventBeginPlay
  (CallFunction|Initialize))

(event EventTick
  (params (DeltaSeconds :type Float%20%28single-precision%29))
  (CallFunction|Update))

(fn Initialize
  (bind _rendertextureresolution (Variables|DropShadowSettings|RenderTexture|GetRenderTextureResolution))
  ;[0.2 0.16 0.16] Set Owner's Mesh Components to not recieve Decals (otherwise we'd draw shadows on them)
  (for _array_element (Actor|GetComponentsByClass (Components|GetOwner) "/Script/Engine.MeshComponent")
    (Rendering|SetReceivesDecals _array_element false))
  ;[0.2 0.16 0.16] Add Decal Component
  (bind _returnvalue (Game|AddComponentbyClass (Components|GetOwner) "/Script/Engine.DecalComponent" false (Math|Transform|MakeTransform "0, 0, 0" "-90.000000,0.000000,90.000000" "1.000000,1.000000,1.000000")))
  (Variables|Components|SetDecalComponent _returnvalue)
  ;[0.2 0.16 0.16] Select Material (M_BlobShadow_Decal or M_DropShadow_Decal) & create a Dynamic Instance
  (Rendering|Components|Decal|SetDecalMaterial (Variables|Components|GetDecalComponent) (select (Variables|DropShadowSettings|RenderTexture|GetbUseRenderTexture) "/Game/Assets/Materials/BlobShadow/MMAT_DEC_Dropshadow.MMAT_DEC_Dropshadow" "/Game/Assets/Materials/BlobShadow/MMAT_DEC_BlobShadow.MMAT_DEC_BlobShadow"))
  (bind _returnvalue_2 (Rendering|Material|CreateDynamicMaterialInstance (Variables|Components|GetDecalComponent) :!class /Script/Engine.DecalComponent))
  (Variables|Components|SetMaterial _returnvalue_2)
  ;[0.2 0.16 0.16] Add Scene Capture Component if necessary
  (if (Variables|DropShadowSettings|RenderTexture|GetbUseRenderTexture)
    (bind _returnvalue_3 (Game|AddComponentbyClass (Components|GetOwner) "/Script/Engine.SceneCaptureComponent2D" false (Math|Transform|MakeTransform (Math|Vector|MakeVector 0.0 0.0 (Variables|DropShadowSettings|RenderTexture|GetSceneCaptureHeight)) "-90.000000,0.000000,0.000000" "1.000000,1.000000,1.000000")))
    (bind _output_get (Variables|Components|SetSceneCaptureComponent _returnvalue_3))
    (Variables|/Script/Engine.SceneCaptureComponent2D|SetProjectionType _output_get "Orthographic")
    (Variables|/Script/Engine.SceneCaptureComponent2D|SetOrthoWidth _output_get (Variables|DropShadowSettings|RenderTexture|GetSceneCaptureOrthoWidth))
    (Variables|/Script/Engine.SceneCaptureComponent|SetPrimitiveRenderMode _output_get "PRM_UseShowOnlyList")
    (Variables|/Script/Engine.SceneCaptureComponent|SetCaptureSource _output_get "SCS_SceneDepth")
    (Variables|/Script/Engine.SceneCaptureComponent|SetbCaptureEveryFrame _output_get false)
    (Variables|/Script/Engine.SceneCaptureComponent|SetbCaptureOnMovement _output_get false)
    ;[0.2 0.16 0.16] Create a new Render Target and apply it to our Material
    (bind _returnvalue_4 (Rendering|CreateRenderTarget2D _rendertextureresolution _rendertextureresolution "RTF_R16f"))
    (bind _output_get_2 (Variables|/Script/Engine.SceneCaptureComponent2D|SetTextureTarget (Variables|Components|GetSceneCaptureComponent) _returnvalue_4))
    (Variables|/Script/Engine.SceneCaptureComponent|SetShowOnlyActors (Variables|Components|GetSceneCaptureComponent) (Utilities|Array|MakeArray (Components|GetOwner)))
    (Rendering|Material|SetTextureParameterValue (Variables|Components|GetMaterial) "Render target" _output_get_2)))

(fn Update
  (bind _returnvalue (Components|GetOwner))
  (bind _decalsize (Variables|DropShadowSettings|GetDecalSize))
  (bind _decalcomponent (Variables|Components|GetDecalComponent))
  (bind _material (Variables|Components|GetMaterial))
  (bind _returnvalue_2 (Transformation|GetWorldLocation _decalcomponent))
  (bind _returnvalue_3 (/ _decalsize 256.0))
  ;[0.2 0.16 0.16] Draw Drop Shadow Traces
  (bind _return (CallFunction|DrawTraces))
  (if _return
    ;[0.2 0.16 0.16] Do we need to update?
    (if (or (!= (Variables|Default|GetCurrentDistance) (Variables|Default|GetClosestDistance)) (Variables|DropShadowSettings|GetbAlwaysUpdate))
      ;[0.2 0.16 0.16] Interp to Closest Distance
      (Variables|Default|SetCurrentDistance (Math|Interpolation|FInterpTo (Variables|Default|GetCurrentDistance) (Variables|Default|GetClosestDistance) (Utilities|Time|GetWorldDeltaSeconds) (Variables|DropShadowSettings|GetFadeSpeed)))
      ;[0.2 0.16 0.16] Set Decal Component's scale and location based on closest/furthest distance
      (Transformation|SetWorldScale3D (Variables|Components|GetDecalComponent) (Math|Vector|MakeVector (/ (Variables|Default|GetFurthestDistance) 128.0) _returnvalue_3 _returnvalue_3))
      (Transformation|SetWorldLocation _decalcomponent (Math|Vector|MakeVector (.x _returnvalue_2) (.y _returnvalue_2) (- (.z (Transformation|GetActorLocation (Components|GetOwner))) (* (Variables|Default|GetClosestDistance) 0.5))) false false)
      ;[0.2 0.16 0.16] Update the material parameters
      (Rendering|Material|SetScalarParameterValue (Variables|Components|GetMaterial) "Cutoff mask distance" (- (+ (.z (Transformation|GetActorLocation _returnvalue)) 32.0) (.z (.BoxExtent (Collision|GetActorBounds _returnvalue true false)))) :!class /Script/Engine.MaterialInstanceDynamic)
      (Rendering|Material|SetScalarParameterValue (Variables|Components|GetMaterial) "Opacity" (Math|Float|Lerp 0.0 (Variables|DropShadowSettings|GetOpacity) (Math|Float|MapRangeClamped (Variables|Default|GetCurrentDistance) (Variables|DropShadowSettings|GetOpacityMinDistance) (Variables|DropShadowSettings|GetOpacityMaxDistance) 0.0 1.0)) :!class /Script/Engine.MaterialInstanceDynamic)
      (if (Variables|DropShadowSettings|RenderTexture|GetbUseRenderTexture)
        (Rendering|Material|SetScalarParameterValue _material "Blur" (Math|Curves|GetFloatValue (Variables|DropShadowSettings|RenderTexture|GetBlurCurve) (Math|Float|MapRangeClamped (Variables|Default|GetCurrentDistance) (Variables|DropShadowSettings|GetBlurAndDensityMinDistance) (Variables|DropShadowSettings|GetBlurAndDensityMaxDistance) 0.0 1.0)) :!class /Script/Engine.MaterialInstanceDynamic)
        (Rendering|Material|SetScalarParameterValue (Variables|Components|GetMaterial) "UseMask?" (Math|Float|SelectFloat 0.0 1.0 (Math|Float|NearlyEqual(Float) (Variables|Default|GetClosestDistance) (Variables|Default|GetFurthestDistance) 5e+01)) :!class /Script/Engine.MaterialInstanceDynamic)
        ;[0.2 0.16 0.16] Capture scene
        (Rendering|SceneCapture|CaptureScene (Variables|Components|GetSceneCaptureComponent) :!class /Script/Engine.SceneCaptureComponent2D)
        (else
          (Rendering|Material|SetScalarParameterValue _material "Density" (Math|Curves|GetFloatValue (Variables|DropShadowSettings|Blob|GetDensityCurve) (Math|Float|MapRangeClamped (Variables|Default|GetCurrentDistance) (Variables|DropShadowSettings|GetBlurAndDensityMinDistance) (Variables|DropShadowSettings|GetBlurAndDensityMaxDistance) 0.0 1.0)) :!class /Script/Engine.MaterialInstanceDynamic))))))

(fn DrawTraces
  (bind _returnvalue (Components|GetOwner))
  (bind _returnvalue_2 (Components|GetOwner))
  (bind _returnvalue_3 (Components|GetOwner))
  (bind _tracecount (Variables|DropShadowSettings|GetTraceCount))
  (bind _returnvalue_4 (Transformation|GetActorLocation _returnvalue_3))
  (bind _returnvalue_5 (Transformation|GetActorLocation _returnvalue_2))
  (bind _returnvalue_6 (Transformation|GetActorLocation _returnvalue))
  ;[0.2 0.16 0.16] Loop through vector rotations to draw a circle of line traces around the character
  (for _index (range 1 _tracecount)
    (bind (_outhit _returnvalue_7) (Collision|LineTraceByChannel (+ (Transformation|GetActorLocation (Components|GetOwner)) (* (Math|Vector|RotateVectorAroundAxis "1.000000,0.000000,0.000000" (* (/ (Math|Conversions|ToFloat(Integer) _index) (Math|Conversions|ToFloat(Integer) _tracecount)) 3.6e+02) "0, 0,1.000000") 2e+01)) (- (+ (Transformation|GetActorLocation (Components|GetOwner)) (* (Math|Vector|RotateVectorAroundAxis "1.000000,0.000000,0.000000" (* (/ (Math|Conversions|ToFloat(Integer) _index) (Math|Conversions|ToFloat(Integer) _tracecount)) 3.6e+02) "0, 0,1.000000") 2e+01)) (Math|Vector|MakeVector 0.0 0.0 (Variables|DropShadowSettings|GetTraceLength))) "TraceTypeQuery1" false 0 (select (Variables|DropShadowSettings|GetbDebugMode) "ForOneFrame" "None") true "(R=1.000000,G=0.000000,B=0.000000,A=1.000000)" "(R=0.000000,G=1.000000,B=0.000000,A=1.000000)" 0.01))
    ;[0.2 0.16 0.16] Update Closest/Furthest Point if applicable
    (if (not (.binitialoverlap _outhit))
      (if _returnvalue_7
        (LocalVariables|SetbReturn_Local true)
        (Utilities|FlowControl|Sequence
          (:then_0
            (if (> (.z (.location _outhit)) (LocalVariables|GetClosestImpactPoint_Local))
              (LocalVariables|SetClosestImpactPoint_Local (.z (.location _outhit)))))
          (:then_1
            (if (> (LocalVariables|GetFurthestImpactPoint_Local) (.z (.location _outhit)))
              (LocalVariables|SetFurthestImpactPoint_Local (.z (.location _outhit)))))))))
  (Utilities|FlowControl|Sequence
    (:then_0
      ;[0.2 0.16 0.16] Draw shortest and longest point (Debug)
      (if (Variables|DropShadowSettings|GetbDebugMode)
        (Rendering|Debug|DrawDebugPoint (Math|Vector|MakeVector (.x _returnvalue_4) (.y _returnvalue_4) (LocalVariables|GetClosestImpactPoint_Local)) 16.0 "(R=0.000000,G=1.000000,B=0.000000,A=1.000000)" 0.0)
        (Rendering|Debug|DrawDebugPoint (Math|Vector|MakeVector (.x _returnvalue_6) (.y _returnvalue_6) (LocalVariables|GetFurthestImpactPoint_Local)) 16.0 "(R=0.000000,G=0.000000,B=1.000000,A=1.000000)" 0.0)))
    (:then_1
      ;[0.2 0.16 0.16] Set Closest/Furthest Distance
      (Variables|Default|SetClosestDistance (- (.z _returnvalue_5) (LocalVariables|GetClosestImpactPoint_Local)))
      (Variables|Default|SetFurthestDistance (- (.z _returnvalue_5) (LocalVariables|GetFurthestImpactPoint_Local)))
      (return (LocalVariables|GetbReturn_Local)))))