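; Player dash actor component that launches the character along its forward vector from idle or walking, gated by a cooldown.
; Dash zeroes friction, braking and air control, then a looping timer sets curve-scaled horizontal velocity, keeping Z for dash jumps, and plays a spin montage.
; When ground or air duration expires, it restores friction, rotation rate and movement state.
; Setup caching references and binding the player's dash call is disconnected from BeginPlay.
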(event Custom|DoDash
  (bind _movementcomponent (Variables|Default|GetMovementComponent))
  ;[1 1 1] DASH
  (Variables|/Script/Engine.MovementComponent|SetVelocity _movementcomponent (Math|Vector|MakeVector (.x (Variables|/Script/Engine.MovementComponent|GetVelocity _movementcomponent)) (.y (Variables|/Script/Engine.MovementComponent|GetVelocity _movementcomponent)) 0.0))
  (bind _returnvalue (Utilities|Time|SetTimerbyEvent (delegate Custom|DashTick) (Utilities|Time|GetWorldDeltaSeconds) true))
  (Variables|Default|SetDashTimerHandle _returnvalue))

(event Custom|Dash
  (bind _movementcomponent (Variables|Default|GetMovementComponent))
  ;[1 1 1] DASH
  (if (Variables|Default|GetCanDash)
    (switch Utilities|FlowControl|Switch|SwitchonENUM_MovementState (Variables|/Game/Blueprints/ActorComponents/Player/MovementState/AC_MovementStateComponent.AC_MovementStateComponent_C|GetMovementState (Variables|/Game/Blueprints/Character/BP_Player.BP_Player_C|GetMovementStateComponent (Variables|Default|GetPlayer)))
      (:NewEnumerator2
        (Variables|/Game/Blueprints/ActorComponents/Player/MovementState/AC_MovementStateComponent.AC_MovementStateComponent_C|SetMovementState (Variables|/Game/Blueprints/Character/BP_Player.BP_Player_C|GetMovementStateComponent (Variables|Default|GetPlayer)) "NewEnumerator11")
        (Variables|Default|SetCanDash false)
        (Variables|/Script/Engine.CharacterMovementComponent|SetRotationRate _movementcomponent "0.000000,720.000000,0.000000")
        ;;[1 1 1] Test with Controller
        (Variables|/Script/Engine.CharacterMovementComponent|SetAirControl _movementcomponent 0.0)
        (Variables|/Script/Engine.CharacterMovementComponent|SetBrakingDecelerationWalking _movementcomponent 0.0)
        (Variables|/Script/Engine.CharacterMovementComponent|SetFallingLateralFriction (Variables|Default|GetMovementComponent) 0.0)
        (Variables|Default|SetPlayerForwardVector (Transformation|GetActorForwardVector (Variables|Default|GetPlayer)))
        (Variables|/Script/Engine.CharacterMovementComponent|SetGroundFriction (Variables|Default|GetMovementComponent) 0.0)
        (CallFunction|DoDash)
        (Utilities|FlowControl|Delay (Variables|Default|GetDashCooldown))
        (Variables|Default|SetCanDash true)))))

(event Custom|DashTick
  (bind _player (Variables|Default|GetPlayer))
  (bind _movementstatecomponent (Variables|/Game/Blueprints/Character/BP_Player.BP_Player_C|GetMovementStateComponent _player))
  ;[1 1 1] DASH
  (bind _output_get (Variables|Default|SetElapsedTimer (+ (Utilities|Time|GetWorldDeltaSeconds) (Variables|Default|GetElapsedTimer))))
  (bind _output_get_2 (Variables|Default|SetEffectiveDashTime (select (AI|Components|NavMovement|IsFalling (Variables|/Script/Engine.Character|GetCharacterMovement (Variables|Default|GetPlayer))) (Variables|Default|GetAirDashTime) (Variables|Default|GetDashTime))))
  (if (> _output_get _output_get_2)
    (Utilities|Time|ClearandInvalidateTimerbyHandle (Variables|Default|GetDashTimerHandle))
    (CallFunction|ResetInitialDashValues)
    (switch Utilities|FlowControl|Switch|SwitchonENUM_MovementState (Variables|/Game/Blueprints/ActorComponents/Player/MovementState/AC_MovementStateComponent.AC_MovementStateComponent_C|GetMovementState (Variables|/Game/Blueprints/Character/BP_Player.BP_Player_C|GetMovementStateComponent (Variables|Default|GetPlayer)))
      (:NewEnumerator11
        (if (AI|Components|NavMovement|IsFalling (Variables|Default|GetMovementComponent))
          (Variables|/Game/Blueprints/ActorComponents/Player/MovementState/AC_MovementStateComponent.AC_MovementStateComponent_C|SetMovementState _movementstatecomponent "NewEnumerator0")
          (else
            (Variables|/Game/Blueprints/ActorComponents/Player/MovementState/AC_MovementStateComponent.AC_MovementStateComponent_C|SetMovementState _movementstatecomponent "NewEnumerator2")))))
    (else
      (CallFunction|DetermineDashVelocity)
      (Utilities|FlowControl|DoOnce false :!label _label
        (:Completed
          (Animation|Montage|PlayMontage (Variables|/Script/Engine.Character|GetMesh (Variables|Default|GetPlayer)) "/Game/Assets/Characters/Leif/Skeletal_Mesh/Leif_Animations/ANIM_Leif_Spin_Attack_Montage.ANIM_Leif_Spin_Attack_Montage"
            (:OnCompleted
              (goto _label Reset))
            (:OnBlendOut
              (goto _label Reset))
            (:OnInterrupted
              (goto _label Reset))))))))

(event EventBeginPlay
  ;[1 1 1] BeginPlay
)

(fn DetermineDashVelocity
  (bind _playerforwardvector (Variables|Default|GetPlayerForwardVector))
  (bind _elapsedtimer (Variables|Default|GetElapsedTimer))
  (bind _dashcurve (Variables|Default|GetDashCurve))
  (bind _effectivedashtime (Variables|Default|GetEffectiveDashTime))
  (bind _grounddashvelocity (Variables|Default|GetGroundDashVelocity))
  (bind _returnvalue (/ _elapsedtimer _effectivedashtime))
  (bind _returnvalue_2 (Math|Curves|GetFloatValue _dashcurve _returnvalue))
  (bind _returnvalue_3 (* _returnvalue_2 _grounddashvelocity))
  (bind _returnvalue_4 (* _playerforwardvector _returnvalue_3))
  (Variables|/Script/Engine.MovementComponent|SetVelocity (Variables|Default|GetMovementComponent) (Math|Vector|MakeVector (.x _returnvalue_4) (.y _returnvalue_4) (.z (Transformation|GetVelocity (Variables|Default|GetPlayer))))))

(fn ResetInitialDiveValues
  (bind _movementcomponent (Variables|Default|GetMovementComponent))
  (Variables|/Script/Engine.CharacterMovementComponent|SetGroundFriction (Variables|Default|GetMovementComponent) (Variables|Default|GetInitialGroundFriction))
  (Variables|/Script/Engine.CharacterMovementComponent|SetRotationRate _movementcomponent (Variables|Default|GetInitialRotationRate))
  (Variables|/Script/Engine.CharacterMovementComponent|SetAirControl _movementcomponent (Variables|Default|GetInitialAirControl))
  (Variables|/Script/Engine.CharacterMovementComponent|SetGravityScale _movementcomponent (Variables|Default|GetInitialGravity))
  (Variables|/Script/Engine.CharacterMovementComponent|SetFallingLateralFriction (Variables|Default|GetMovementComponent) 1.0))

(fn ResetInitialDashValues
  (Variables|/Script/Engine.CharacterMovementComponent|SetGroundFriction (Variables|Default|GetMovementComponent) (Variables|Default|GetInitialGroundFriction))
  (Variables|/Script/Engine.CharacterMovementComponent|SetRotationRate (Variables|Default|GetMovementComponent) (Variables|Default|GetInitialRotationRate))
  (Variables|Default|SetElapsedTimer 0.0))