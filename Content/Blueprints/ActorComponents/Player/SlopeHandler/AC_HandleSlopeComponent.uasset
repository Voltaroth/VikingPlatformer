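; Player actor component that adjusts walk speed according to the slope of the ground underfoot.
; Each tick, the dot product of the traced ground normal and player forward vector samples SpeedCurve, using zero while falling.
; MaxWalkSpeed interpolates toward the curve value at an interp rate mapped from that value.
; The should-update check gates nothing, and the branch restoring the initial walk speed is disconnected.
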(event EventTick
  (params (DeltaSeconds :type Float%20%28single-precision%29))
  (bind _shouldupdate (CallFunction|ShouldUpdateSpeed))
  (bind _desiredspeedfactor (CallFunction|GetAngleSpeed))
  (CallFunction|UpdateMovementSpeed _desiredspeedfactor))

(event EventBeginPlay
  (bind _returnvalue (Components|GetOwner))
  (bind _returnvalue_2 (Actor|GetComponentbyClass _returnvalue "/Script/Engine.CharacterMovementComponent"))
  (Utilities|IsValid _returnvalue_2
    (:Is%20Valid
      (Variables|Default|SetMovementComponent _returnvalue_2)
      (Utilities|IsValid (Actor|GetComponentbyClass _returnvalue "AC_HandleSlopeComponent_C")
        (:Is%20Valid
          (bind _asbp_player (Utilities|Casting|CastToBP_Player _returnvalue))
          (Variables|Default|SetPlayer _asbp_player)
          (Variables|Default|SetInitialMaxWalkSpeed (Variables|/Script/Engine.CharacterMovementComponent|GetMaxWalkSpeed (Variables|Default|GetMovementComponent))))))))

(fn ShouldUpdateSpeed
  (bind _player (Variables|Default|GetPlayer))
  (bind _charactermovement (Variables|/Script/Engine.Character|GetCharacterMovement _player))
  (return (and (not (AI|Components|NavMovement|IsFalling _charactermovement)) (> (Math|Vector|VectorLengthSquared (Variables|/Script/Engine.MovementComponent|GetVelocity _charactermovement)) 0.0))))

(fn GetAngleSpeed
  (bind _player (Variables|Default|GetPlayer))
  (return (Math|Curves|GetFloatValue (Variables|Default|GetSpeedCurve) (select (AI|Components|NavMovement|IsFalling (Variables|/Script/Engine.Character|GetCharacterMovement _player)) 0.0 (Math|Vector|DotProduct (.impactnormal (Default|TraceforGround (Variables|Default|GetPlayer))) (Transformation|GetActorForwardVector _player))))))

(fn UpdateMovementSpeed
  (params (DesiredSpeedFactor :type Float%20%28double-precision%29))
  (Variables|/Script/Engine.CharacterMovementComponent|SetMaxWalkSpeed (Variables|Default|GetMovementComponent) (Math|Interpolation|FInterpTo (Variables|/Script/Engine.CharacterMovementComponent|GetMaxWalkSpeed (Variables|Default|GetMovementComponent)) DesiredSpeedFactor (Utilities|Time|GetWorldDeltaSeconds) (Math|Float|MapRangeClamped DesiredSpeedFactor 1e+02 0.0 1.0 0.0))))