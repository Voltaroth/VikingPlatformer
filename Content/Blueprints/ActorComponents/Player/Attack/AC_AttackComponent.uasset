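; Player attack component that handles Leif's spin attack and Mjölnir throw, triggered by BP_Player dispatchers and gated by movement state.
; Spin attacks launch the player upward in the air, or slide when moving on ground through a looping timer, float curve and temporarily zeroed friction.
; Throwing hides the held hammer and shoots a spawned BP_Mjölnir_Projectile, with brief airtime if falling.
; Flags limit air use until landing or reset.
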(event Custom|StartAttack
  (bind _movementcomponent (Variables|Default|GetMovementComponent))
  ;[1 1 1] SpinAttack
  (if (Math|Boolean|ANDBoolean (Variables|Default|GetCanAttack?) (Variables|Default|GetCanAirAttack) (not (Variables|Default|GetThrown?)))
    (switch Utilities|FlowControl|Switch|SwitchonENUM_MovementState (Variables|/Game/Blueprints/ActorComponents/Player/MovementState/AC_MovementStateComponent.AC_MovementStateComponent_C|GetMovementState (Variables|/Game/Blueprints/Character/BP_Player.BP_Player_C|GetMovementStateComponent (Variables|Default|GetPlayer)))
      (:NewEnumerator2
        _)
      (:NewEnumerator1
        (Utilities|FlowControl|Delay 0.1))
      (:NewEnumerator5
        _)
      (:NewEnumerator16
        _)
      (:NewEnumerator0
        _)
      (:NewEnumerator11
        _))
    (Variables|/Game/Blueprints/ActorComponents/Player/MovementState/AC_MovementStateComponent.AC_MovementStateComponent_C|SetMovementState (Variables|/Game/Blueprints/Character/BP_Player.BP_Player_C|GetMovementStateComponent (Variables|Default|GetPlayer)) "NewEnumerator17")
    (if (AI|Components|NavMovement|IsFalling (Variables|Default|GetMovementComponent))
      ;;[1 1 1] If attack in the air launch character
      (Variables|Default|SetCanAirAttack false)
      (bind _player (Variables|Default|GetPlayer)
        (:then
          (Character|LaunchCharacter _player (Math|Vector|MakeVector 0.0 0.0 (Variables|Default|GetLaunch%20Velocity%20Z)) false true)
          ;;[1 1 1] Play montages
          (Animation|PlayAnimMontage _player "/Game/Assets/Characters/Leif/Skeletal_Mesh/Leif_Animations/ANIM_Leif_Spin_Attack_Montage.ANIM_Leif_Spin_Attack_Montage" 1.0 "None" :!label _label)
          (Animation|Montage|PlayMontage (Variables|/Game/Blueprints/Character/BP_Player.BP_Player_C|GetSKM_Mjölnir (Variables|Default|GetPlayer)) "/Game/Assets/Characters/Leif/Skeletal_Mesh/Mjölnir/Mjölnir_Animations/ANIM_Mjölnir_Spin_Attack_Montage.ANIM_Mjölnir_Spin_Attack_Montage"
            (:OnCompleted
              ;;[1 1 1] Reset Values and movement states
              (Variables|Default|SetCanAttack? true))
            (:OnBlendOut
              (Variables|Default|SetCanThrow? true)
              (if (AI|Components|NavMovement|IsFalling (Variables|/Script/Engine.Character|GetCharacterMovement (Variables|Default|GetPlayer)))
                (Variables|/Game/Blueprints/ActorComponents/Player/MovementState/AC_MovementStateComponent.AC_MovementStateComponent_C|SetMovementState (Variables|/Game/Blueprints/Character/BP_Player.BP_Player_C|GetMovementStateComponent (Variables|Default|GetPlayer)) "NewEnumerator0")
                (else
                  (Variables|/Game/Blueprints/ActorComponents/Player/MovementState/AC_MovementStateComponent.AC_MovementStateComponent_C|SetMovementState (Variables|/Game/Blueprints/Character/BP_Player.BP_Player_C|GetMovementStateComponent (Variables|Default|GetPlayer)) "NewEnumerator2"))))))
        (:else))
      (else
        ;;[1 1 1] If attack on ground, check if moving
        (Variables|Default|SetCanAttack? false)
        (if (> (Math|Vector2D|Vector2DLength (Math|Vector2D|MakeVector2D (.x (Variables|/Script/Engine.MovementComponent|GetVelocity (Variables|Default|GetMovementComponent))) (.y (Variables|/Script/Engine.MovementComponent|GetVelocity (Variables|Default|GetMovementComponent))))) 5e+01)
          ;;[1 1 1] Dash if player is moving, stay put if not
          (CallFunction|SetGroundValuesforSlide)
          (Variables|/Script/Engine.MovementComponent|SetVelocity _movementcomponent (Math|Vector|MakeVector (.x (Variables|/Script/Engine.MovementComponent|GetVelocity _movementcomponent)) (.y (Variables|/Script/Engine.MovementComponent|GetVelocity _movementcomponent)) 0.0))
          (bind _returnvalue (Utilities|Time|SetTimerbyEvent (delegate Custom|DashTick) (Utilities|Time|GetWorldDeltaSeconds) true))
          (Variables|Default|SetDashTimerHandle _returnvalue)
          (else
            (goto _label)))))))

(event Custom|Landed
  (params (Hit :type Hit%20Result%20Structure%20%28by%20ref%29))
  ;[1 1 1] MjölnirThrow
  ;;[1 1 1] Reset on landed
  (Variables|Default|SetCanAttack? true)
  (Variables|Default|SetCanAirAttack true)
  (Variables|Default|SetCanThrow? true)
  (Variables|Default|SetCanAirThrow? true))

(event Custom|Throw
  (bind _player (Variables|Default|GetPlayer))
  (bind _player_2 (Variables|Default|GetPlayer))
  (bind _player_3 (Variables|Default|GetPlayer))
  (bind _player_4 (Variables|Default|GetPlayer))
  (bind _movementcomponent (Variables|Default|GetMovementComponent))
  (bind _player_5 (Variables|Default|GetPlayer))
  (bind _player_6 (Variables|Default|GetPlayer))
  (bind _returnvalue (Transformation|GetActorLocation _player_6))
  (bind _returnvalue_2 (Transformation|GetVelocity _player_4))
  (bind _velocity (Variables|/Script/Engine.MovementComponent|GetVelocity _movementcomponent))
  (bind _movementstatecomponent (Variables|/Game/Blueprints/Character/BP_Player.BP_Player_C|GetMovementStateComponent _player_5))
  ;[1 1 1] MjölnirThrow
  (if (and (Variables|Default|GetCanThrow?) (Variables|Default|GetCanAirThrow?))
    (switch Utilities|FlowControl|Switch|SwitchonENUM_MovementState (Variables|/Game/Blueprints/ActorComponents/Player/MovementState/AC_MovementStateComponent.AC_MovementStateComponent_C|GetMovementState _movementstatecomponent)
      (:NewEnumerator2
        _)
      (:NewEnumerator1
        _)
      (:NewEnumerator5
        _)
      (:NewEnumerator0
        _))
    (Variables|/Game/Blueprints/ActorComponents/Player/MovementState/AC_MovementStateComponent.AC_MovementStateComponent_C|SetMovementState _movementstatecomponent "NewEnumerator18")
    (Variables|Default|SetThrown? true)
    (if (AI|Components|NavMovement|IsFalling (Variables|/Script/Engine.Character|GetCharacterMovement (Variables|Default|GetPlayer)))
      ;;[1 1 1] Give Player a bit of airtime when throwing mjölnir while falling
      (Variables|Default|SetCanAirThrow? false)
      (Character|LaunchCharacter _player_4 (Math|Vector|MakeVector (/ (.x _returnvalue_2) 8.0) (/ (.y _returnvalue_2) 8.0) 2e+02) true true)
      (else
        (Variables|Default|SetCanThrow? false)))
    ;;[1 1 1] Make mjölnir invisible
    (Rendering|SetVisibility (Variables|/Game/Blueprints/Character/BP_Player.BP_Player_C|GetSKM_Mjölnir (Variables|Default|GetPlayer)) false false)
    (bind _returnvalue_3 (Game|SpawnActorfromClass "/Game/Blueprints/ActorComponents/Player/Attack/BP_Mjölnir_Projectile.BP_Mjölnir_Projectile_C" (Math|Transform|MakeTransform (+ (* (Transformation|GetActorForwardVector (Variables|Default|GetPlayer)) (select (> (Math|Vector2D|Vector2DLength (Math|Vector2D|MakeVector2D (.x _velocity) (.y _velocity))) 5e+01) 3e+02 5e+01)) (Math|Vector|MakeVector (.x _returnvalue) (.y _returnvalue) (+ (.z _returnvalue) 2e+01))) "0.000000,-90.000000,0.000000" "1.000000,1.000000,1.000000") "AdjustIfPossibleButAlwaysSpawn" 0 0))
    ;;[1 1 1] Make it so player ignores projectile and vice versa
    (Variables|Default|SetMjölnirProjectile _returnvalue_3)
    (Collision|IgnoreActorwhenMoving (Variables|/Script/Engine.Character|GetCapsuleComponent _player_2) (Variables|Default|GetMjölnirProjectile) true)
    (Collision|IgnoreActorwhenMoving (Variables|/Game/Blueprints/ActorComponents/Player/Attack/BP_Mjölnir_Projectile.BP_Mjölnir_Projectile_C|GetSphere (Variables|Default|GetMjölnirProjectile)) _player_2 true)
    ;;[1 1 1] shoot mjölnir when spawned --> BP_Mjölnir_Projectile/otherwise, reset
    (Utilities|IsValid (Variables|Default|GetMjölnirProjectile)
      (:Is%20Valid
        (Default|Shoot (Variables|Default|GetMjölnirProjectile) _player_3 (Transformation|GetActorForwardVector _player_3) (+ (Transformation|GetActorLocation _player) (* (Transformation|GetActorForwardVector _player) (Variables|Default|GetMaxThrowDistance))))
        ;;[1 1 1] Play throw montage
        (Animation|Montage|PlayMontage (Variables|/Script/Engine.Character|GetMesh (Variables|Default|GetPlayer)) "/Game/Assets/Characters/Leif/Skeletal_Mesh/Leif_Animations/ANIM_Leif_Spin_Attack_Montage.ANIM_Leif_Spin_Attack_Montage"
          (:then
            (Variables|/Game/Blueprints/Character/BP_Player.BP_Player_C|SetIsMjölnirInHand? (Variables|Default|GetPlayer) false))
          (:OnBlendOut
            ;;[1 1 1] Set Movement States
            (if (AI|Components|NavMovement|IsFalling (Variables|/Script/Engine.Character|GetCharacterMovement (Variables|Default|GetPlayer)))
              (Variables|/Game/Blueprints/ActorComponents/Player/MovementState/AC_MovementStateComponent.AC_MovementStateComponent_C|SetMovementState (Variables|/Game/Blueprints/Character/BP_Player.BP_Player_C|GetMovementStateComponent (Variables|Default|GetPlayer)) "NewEnumerator0")
              (else
                (Variables|/Game/Blueprints/ActorComponents/Player/MovementState/AC_MovementStateComponent.AC_MovementStateComponent_C|SetMovementState (Variables|/Game/Blueprints/Character/BP_Player.BP_Player_C|GetMovementStateComponent (Variables|Default|GetPlayer)) "NewEnumerator2"))))))
      (:Is%20Not%20Valid
        (CallFunction|ResetMjölnirinHand)))))

(event Custom|DashTick
  ;[1 1 1] SpinAttack
  ;;[1 1 1] Dash if player is moving, stay put if not
  (bind _output_get (Variables|Default|SetElapsedTimer (+ (Utilities|Time|GetWorldDeltaSeconds) (Variables|Default|GetElapsedTimer))))
  (bind _output_get_2 (Variables|Default|SetEffectiveDashTime (select (AI|Components|NavMovement|IsFalling (Variables|/Script/Engine.Character|GetCharacterMovement (Variables|Default|GetPlayer))) (Variables|Default|GetAirDashTime) (Variables|Default|GetDashTime))))
  (if (> _output_get _output_get_2)
    (Utilities|Time|ClearandInvalidateTimerbyHandle (Variables|Default|GetDashTimerHandle))
    (CallFunction|ResetInitialValues)
    (goto _label Reset)
    (else
      (CallFunction|DetermineSlideVelocity)
      (Utilities|FlowControl|DoOnce false :!label _label
        (:Completed
          ;;[1 1 1] Play montages
          (Animation|PlayAnimMontage (stale Custom|StartAttack _player) "/Game/Assets/Characters/Leif/Skeletal_Mesh/Leif_Animations/ANIM_Leif_Spin_Attack_Montage.ANIM_Leif_Spin_Attack_Montage" 1.0 "None")
          (Animation|Montage|PlayMontage (Variables|/Game/Blueprints/Character/BP_Player.BP_Player_C|GetSKM_Mjölnir (Variables|Default|GetPlayer)) "/Game/Assets/Characters/Leif/Skeletal_Mesh/Mjölnir/Mjölnir_Animations/ANIM_Mjölnir_Spin_Attack_Montage.ANIM_Mjölnir_Spin_Attack_Montage"
            (:OnCompleted
              ;;[1 1 1] Reset Values and movement states
              (Variables|Default|SetCanAttack? true))
            (:OnBlendOut
              (Variables|Default|SetCanThrow? true)
              (if (AI|Components|NavMovement|IsFalling (Variables|/Script/Engine.Character|GetCharacterMovement (Variables|Default|GetPlayer)))
                (Variables|/Game/Blueprints/ActorComponents/Player/MovementState/AC_MovementStateComponent.AC_MovementStateComponent_C|SetMovementState (Variables|/Game/Blueprints/Character/BP_Player.BP_Player_C|GetMovementStateComponent (Variables|Default|GetPlayer)) "NewEnumerator0")
                (else
                  (Variables|/Game/Blueprints/ActorComponents/Player/MovementState/AC_MovementStateComponent.AC_MovementStateComponent_C|SetMovementState (Variables|/Game/Blueprints/Character/BP_Player.BP_Player_C|GetMovementStateComponent (Variables|Default|GetPlayer)) "NewEnumerator2"))))))))))

(event Custom|ResetMjölnirInHand
  ;[1 1 1] MjölnirThrow
  ;;[1 1 1] Reset when mjölnir returns or when not valid
  (Variables|Default|SetThrown? false)
  (Rendering|SetVisibility (Variables|/Game/Blueprints/Character/BP_Player.BP_Player_C|GetSKM_Mjölnir (Variables|Default|GetPlayer)) true false)
  (Variables|/Game/Blueprints/Character/BP_Player.BP_Player_C|SetIsMjölnirInHand? (Variables|Default|GetPlayer) true)
  (if (AI|Components|NavMovement|IsFalling (Variables|/Script/Engine.Character|GetCharacterMovement (Variables|Default|GetPlayer)))
    (Variables|/Game/Blueprints/ActorComponents/Player/MovementState/AC_MovementStateComponent.AC_MovementStateComponent_C|SetMovementState (Variables|/Game/Blueprints/Character/BP_Player.BP_Player_C|GetMovementStateComponent (Variables|Default|GetPlayer)) "NewEnumerator0")
    (Variables|Default|SetCanThrow? true)
    (else
      (Variables|/Game/Blueprints/ActorComponents/Player/MovementState/AC_MovementStateComponent.AC_MovementStateComponent_C|SetMovementState (Variables|/Game/Blueprints/Character/BP_Player.BP_Player_C|GetMovementStateComponent (Variables|Default|GetPlayer)) "NewEnumerator2")
      (Variables|Default|SetCanThrow? true)
      (Variables|Default|SetCanAirThrow? true))))

(event EventBeginPlay
  (bind _returnvalue (Components|GetOwner))
  (bind _returnvalue_2 (Actor|GetComponentbyClass _returnvalue "/Script/Engine.CharacterMovementComponent"))
  (Utilities|IsValid _returnvalue_2
    (:Is%20Valid
      (Variables|Default|SetMovementComponent _returnvalue_2)
      (Utilities|IsValid (Actor|GetComponentbyClass _returnvalue "AC_AttackComponent_C")
        (:Is%20Valid
          (bind _asbp_player (Utilities|Casting|CastToBP_Player _returnvalue))
          (bind _output_get (Variables|Default|SetPlayer _asbp_player))
          (EventDispatchers|BindEventtoStartAttackCall _output_get (EventDispatchers|CreateEvent :!event Custom|StartAttack))
          (EventDispatchers|BindEventtoLandedDelegate _output_get (EventDispatchers|CreateEvent :!event Custom|Landed))
          (EventDispatchers|BindEventtoStartThrowCall _output_get (EventDispatchers|CreateEvent :!event Custom|Throw))
          (Variables|Default|SetInitialRotationRate (Variables|/Script/Engine.CharacterMovementComponent|GetRotationRate (Variables|Default|GetMovementComponent)))
          (Variables|Default|SetInitialGroundFriction (Variables|/Script/Engine.CharacterMovementComponent|GetGroundFriction (Variables|Default|GetMovementComponent))))))))

(event EventTick
  (params (DeltaSeconds :type Float%20%28single-precision%29)))

(fn SetGroundValuesforSlide
  (bind _movementcomponent (Variables|Default|GetMovementComponent))
  (Variables|/Script/Engine.CharacterMovementComponent|SetRotationRate _movementcomponent "0.000000,720.000000,0.000000")
  (Variables|/Script/Engine.CharacterMovementComponent|SetBrakingDecelerationWalking _movementcomponent 0.0)
  (Variables|Default|SetPlayerForwardVector (Transformation|GetActorForwardVector (Variables|Default|GetPlayer)))
  (Variables|/Script/Engine.CharacterMovementComponent|SetGroundFriction (Variables|Default|GetMovementComponent) 0.0))

(fn DetermineSlideVelocity
  (bind _elapsedtimer (Variables|Default|GetElapsedTimer))
  (bind _dashcurve (Variables|Default|GetDashCurve))
  (bind _effectivedashtime (Variables|Default|GetEffectiveDashTime))
  (bind _player (Variables|Default|GetPlayer))
  (bind _grounddashvelocity (Variables|Default|GetGroundDashVelocity))
  (bind _returnvalue (/ _elapsedtimer _effectivedashtime))
  (bind _directioncontrol (Variables|/Game/Blueprints/Character/BP_Player.BP_Player_C|GetDirectionControl _player))
  (bind _returnvalue_2 (Math|Vector|GetForwardVector _directioncontrol))
  (bind _returnvalue_3 (Math|Curves|GetFloatValue _dashcurve _returnvalue))
  (bind _returnvalue_4 (* _returnvalue_3 _grounddashvelocity))
  (bind _returnvalue_5 (* _returnvalue_2 _returnvalue_4))
  (Variables|/Script/Engine.MovementComponent|SetVelocity (Variables|Default|GetMovementComponent) (Math|Vector|MakeVector (.x _returnvalue_5) (.y _returnvalue_5) (.z (Transformation|GetVelocity (Variables|Default|GetPlayer))))))

(fn ResetInitialValues
  (Variables|/Script/Engine.CharacterMovementComponent|SetGroundFriction (Variables|Default|GetMovementComponent) (Variables|Default|GetInitialGroundFriction))
  (Variables|/Script/Engine.CharacterMovementComponent|SetRotationRate (Variables|Default|GetMovementComponent) (Variables|Default|GetInitialRotationRate))
  (Variables|Default|SetElapsedTimer 0.0))