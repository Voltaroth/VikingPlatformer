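; Thrown Mjölnir projectile for the player's attack, which flies along the supplied player forward vector and returns after a hit.
; A timeline curve scales fly speed to drive the projectile movement velocity each tick.
; On return it pauses briefly, restarts the curve and homes in on the player, with a delayed collision shutoff in case it gets stuck.
; Once close, it resets the player's AttackComponent and destroys itself.
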(event Custom|StopSpeed
  ;[1 1 1] Calculate Travel Speed with curve
  (bind _velocitytoplayer (Timeline|VelocityToPlayer Stop)
    (:Update
      (Variables|Default|SetEffectiveFlySpeed (* _velocitytoplayer (Variables|Default|GetFlySpeed))))))

(event Custom|CalculateSpeedSpeed
  ;[1 1 1] Calculate Travel Speed with curve
  (bind _velocitytoplayer (Timeline|VelocityToPlayer PlayFromStart)
    (:Update
      (Variables|Default|SetEffectiveFlySpeed (* _velocitytoplayer (Variables|Default|GetFlySpeed))))))

(event EventBeginPlay
  ;[1 1 1] Calculate Travel Speed with curve
  (CallFunction|CalculateSpeedSpeed))

(event Collision|EventActorBeginOverlap
  (params (OtherActor :type Actor%20Object%20Reference)))

(event EventTick
  (params (DeltaSeconds :type Float%20%28single-precision%29))
  (bind _player (Variables|Default|GetPlayer))
  (Variables|Default|SetDelta%20Seconds DeltaSeconds)
  ;[1 1 1] Fly forward if no return
  (if (Variables|Default|GetReturn?)
    (Utilities|FlowControl|Sequence
      (:then_0
        ;[1 1 1] check distance between player and mjölnir on return
        (Utilities|IsValid _player
          (:Is%20Valid
            (if (> (Transformation|GetDistanceTo _player) 1e+02)
              (Utilities|FlowControl|Sequence
                (:then_0
                  ;[1 1 1] If distance not close, return to player
                  (Utilities|FlowControl|DoOnce false :!label _label
                    (:Completed
                      ;;[1 1 1] Little Delay before returning
                      (CallFunction|StopSpeed)
                      (Variables|Default|SetEffectiveFlySpeed 0.0)
                      (Utilities|FlowControl|Delay (Variables|Default|GetDelayTime))
                      (CallFunction|CalculateSpeedSpeed))))
                (:then_1
                  (bind _output_get (Variables|Default|SetVelocity (* (Math|Vector|Normalize (- (Transformation|GetActorLocation (Variables|Default|GetPlayer)) (Transformation|GetActorLocation))) (Variables|Default|GetEffectiveFlySpeed))))
                  (Variables|/Script/Engine.MovementComponent|SetVelocity (Variables|Default|GetProjectileMovement) _output_get)))
              (else
                ;[1 1 1] If distance close, reset and destroy actor
                (Variables|Default|SetReturn? false)
                (Utilities|FlowControl|Sequence
                  (:then_0
                    (goto _label Reset))
                  (:then_1
                    (goto _label_2 Reset))
                  (:then_2
                    (Default|ResetMjölnir (Variables|/Game/Blueprints/Character/BP_Player.BP_Player_C|GetAttackComponent (Variables|Default|GetPlayer)))
                    (Actor|DestroyActor))))))))
      (:then_1
        ;[1 1 1] disable collision on return (if mjönir stuck)
        (Utilities|FlowControl|DoOnce false :!label _label_2
          (:Completed
            (Utilities|FlowControl|Delay 1.0)
            (Collision|SetCollisionEnabled (Variables|Default|GetSphere) "NoCollision")))))
    (else
      (Variables|Default|SetVelocity (* (Variables|Default|GetPlayerForwardVector) (Variables|Default|GetEffectiveFlySpeed)))
      (Variables|/Script/Engine.MovementComponent|SetVelocity (Variables|Default|GetProjectileMovement) (Variables|Default|GetVelocity)))))

(event Collision|EventHit
  (params (MyComp :type Primitive%20Component%20Object%20Reference) (Other :type Actor%20Object%20Reference) (OtherComp :type Primitive%20Component%20Object%20Reference) (bSelfMoved :type Boolean) (HitLocation :type Vector :default "0, 0, 0") (HitNormal :type Vector :default "0, 0, 0") (NormalImpulse :type Vector :default "0, 0, 0") (Hit :type Hit%20Result%20Structure%20%28by%20ref%29))
  ;[1 1 1] Return when hit something (maybe filter out enemies, since mjölnir should be able to fly through multiple)
  (Variables|Default|SetReturn? true))

(fn ConstructionScript)

(fn Shoot
  (params (Player :type BP%20Player%20Object%20Reference) (PlayerForwardVector :type Vector))
  (Utilities|IsValid Player
    (:Is%20Valid
      (Variables|Default|SetPlayer Player)
      (Variables|Default|SetPlayerForwardVector PlayerForwardVector))))