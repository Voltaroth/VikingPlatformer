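; Player jump component providing variable-height jumps and a double jump, driven by the player's start, stop and landed delegates and its movement state.
; BeginPlay derives launch velocities from jump heights and apex time.
; Tick runs coyote and buffer counters, softens gravity at the apex, raises it when falling and prints coyote debug values.
; Releasing jump clamps upward velocity, landing resets state, while glide and dash-jump logic sit disconnected.
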(event Custom|StopJump
  (bind _player (Variables|Default|GetPlayer))
  (bind _movementstatecomponent (Variables|/Game/Blueprints/Character/BP_Player.BP_Player_C|GetMovementStateComponent _player))
  ;[1 1 1] StopJump
  (switch Utilities|FlowControl|Switch|SwitchonENUM_MovementState (Variables|/Game/Blueprints/ActorComponents/Player/MovementState/AC_MovementStateComponent.AC_MovementStateComponent_C|GetMovementState (Variables|/Game/Blueprints/Character/BP_Player.BP_Player_C|GetMovementStateComponent (Variables|Default|GetPlayer)))
    (:NewEnumerator6
      _)
    (:NewEnumerator1
      _)
    (:NewEnumerator5
      _)
    (:NewEnumerator0
      _)
    (:NewEnumerator12
      _))
  (if (AI|Components|NavMovement|IsFalling (Variables|Default|GetMovementComponent))
    (Variables|/Game/Blueprints/ActorComponents/Player/MovementState/AC_MovementStateComponent.AC_MovementStateComponent_C|SetMovementState _movementstatecomponent "NewEnumerator0")
    (Variables|Default|SetJumpPressed false)
    (Variables|Default|SetCoyoteTimeCounter 0.0)
    (Variables|Default|SetJumpBufferCounter 0.0)
    (Variables|Default|GetPlayer
      (:then
        (if (> (.z (Variables|/Script/Engine.MovementComponent|GetVelocity (Variables|Default|GetMovementComponent))) (Variables|Default|GetMinJumpVelocity))
          (bind _movementcomponent (Variables|Default|GetMovementComponent)
            (:then
              (Variables|/Script/Engine.MovementComponent|SetVelocity _movementcomponent (Math|Vector|MakeVector (.x (Variables|/Script/Engine.MovementComponent|GetVelocity (Variables|Default|GetMovementComponent))) (.y (Variables|/Script/Engine.MovementComponent|GetVelocity (Variables|Default|GetMovementComponent))) (Variables|Default|GetMinJumpVelocity))))
            (:else))))
      (:else))
    (else
      (Variables|/Game/Blueprints/ActorComponents/Player/MovementState/AC_MovementStateComponent.AC_MovementStateComponent_C|SetMovementState _movementstatecomponent "NewEnumerator2"))))

(event Custom|StartJump
  ;[1 1 1] StartJump
  (Variables|Default|SetJumpPressed true)
  (if (and (> (Variables|Default|GetCoyoteTimeCounter) 0.0) (>= (Variables|Default|GetJumpBufferCounter) 0.0))
    (switch Utilities|FlowControl|Switch|SwitchonENUM_MovementState (Variables|/Game/Blueprints/ActorComponents/Player/MovementState/AC_MovementStateComponent.AC_MovementStateComponent_C|GetMovementState (Variables|/Game/Blueprints/Character/BP_Player.BP_Player_C|GetMovementStateComponent (Variables|Default|GetPlayer)))
      (:NewEnumerator2
        _)
      (:NewEnumerator16
        _)
      (:NewEnumerator0
        _))
    (Variables|/Game/Blueprints/ActorComponents/Player/MovementState/AC_MovementStateComponent.AC_MovementStateComponent_C|SetMovementState (Variables|/Game/Blueprints/Character/BP_Player.BP_Player_C|GetMovementStateComponent (Variables|Default|GetPlayer)) "NewEnumerator1")
    (bind _movementcomponent (Variables|Default|GetMovementComponent)
      (:then
        (Variables|/Script/Engine.CharacterMovementComponent|SetJumpZVelocity _movementcomponent (Variables|Default|GetMaxJumpVelocity))
        (bind _player (Variables|Default|GetPlayer)
          (:then
            (Character|LaunchCharacter _player (Math|Vector|MakeVector 0.0 0.0 (Variables|Default|GetMaxJumpVelocity)) false true)
            (Variables|Default|SetCanDoubleJump true)
            (Default|JumpSqueeze (Variables|Default|GetPlayer)))
          (:else)))
      (:else))
    (elif (Variables|Default|GetCanDoubleJump)
      (switch Utilities|FlowControl|Switch|SwitchonENUM_MovementState (Variables|/Game/Blueprints/ActorComponents/Player/MovementState/AC_MovementStateComponent.AC_MovementStateComponent_C|GetMovementState (Variables|/Game/Blueprints/Character/BP_Player.BP_Player_C|GetMovementStateComponent (Variables|Default|GetPlayer)))
        (:NewEnumerator1
          _)
        (:NewEnumerator16
          _)
        (:NewEnumerator0
          _))
      (Variables|/Game/Blueprints/ActorComponents/Player/MovementState/AC_MovementStateComponent.AC_MovementStateComponent_C|SetMovementState (Variables|/Game/Blueprints/Character/BP_Player.BP_Player_C|GetMovementStateComponent (Variables|Default|GetPlayer)) "NewEnumerator5")
      (Variables|/Script/Engine.CharacterMovementComponent|SetRotationRate (Variables|Default|GetMovementComponent) (Variables|Default|GetInitialRotationRate))
      (bind _movementcomponent_2 (Variables|Default|GetMovementComponent)
        (:then
          (Variables|/Script/Engine.CharacterMovementComponent|SetJumpZVelocity _movementcomponent_2 (Variables|Default|GetMaxDoubleJumpVelocity))
          (bind _player_2 (Variables|Default|GetPlayer)
            (:then
              (Character|LaunchCharacter _player_2 (Math|Vector|MakeVector 0.0 0.0 (Variables|Default|GetMaxDoubleJumpVelocity)) false true)
              (Variables|Default|SetCanDoubleJump false)
              (Variables|Default|SetCanGlide true))
            (:else)))
        (:else)))))

(event Custom|Land
  (params (Hit :type Hit%20Result%20Structure%20%28by%20ref%29))
  (bind _player (Variables|Default|GetPlayer))
  (bind _movementcomponent (Variables|Default|GetMovementComponent))
  (bind _movementstatecomponent (Variables|/Game/Blueprints/Character/BP_Player.BP_Player_C|GetMovementStateComponent _player))
  ;[1 1 1] Landed
  (bind _movementcomponent_2 (Variables|Default|GetMovementComponent)
    (:then
      (Variables|/Script/Engine.CharacterMovementComponent|SetGravityScale _movementcomponent_2 2.8)
      (Variables|Default|SetCanDoubleJump false)
      (Variables|Default|SetCoyoteTimeCounter (Variables|Default|GetCoyoteTime))
      (Variables|Default|SetJumpBufferCounter (Variables|Default|GetJumpBufferTime))
      (Variables|Default|SetCanGlide false)
      (Variables|Default|SetDoubleJumped false)
      (switch Utilities|FlowControl|Switch|SwitchonENUM_MovementState (Variables|/Game/Blueprints/ActorComponents/Player/MovementState/AC_MovementStateComponent.AC_MovementStateComponent_C|GetMovementState _movementstatecomponent)
        (:NewEnumerator1
          _)
        (:NewEnumerator0
          _)
        (:NewEnumerator12
          _)
        (:NewEnumerator13
          _))
      (Variables|/Game/Blueprints/ActorComponents/Player/MovementState/AC_MovementStateComponent.AC_MovementStateComponent_C|SetMovementState _movementstatecomponent "NewEnumerator2")
      (Default|LandSqueeze (Variables|Default|GetPlayer))
      (bind _movementcomponent_3 (Variables|Default|GetMovementComponent)
        (:then
          (Variables|/Script/Engine.CharacterMovementComponent|SetGravityScale _movementcomponent_3 (Variables|Default|GetGravityScale))
          (Variables|/Script/Engine.CharacterMovementComponent|SetRotationRate _movementcomponent (Variables|Default|GetInitialRotationRate))
          (Variables|/Script/Engine.CharacterMovementComponent|SetAirControl _movementcomponent 1.5e+04))
        (:else)))
    (:else)))

(event Custom|FollowMovement
  (bind _player (Variables|Default|GetPlayer))
  (bind _player_2 (Variables|Default|GetPlayer))
  (bind _movementstatecomponent (Variables|/Game/Blueprints/Character/BP_Player.BP_Player_C|GetMovementStateComponent _player))
  (bind _movementstate (Variables|/Game/Blueprints/ActorComponents/Player/MovementState/AC_MovementStateComponent.AC_MovementStateComponent_C|GetMovementState _movementstatecomponent))
  ;[0 1 0.9736] LongJump (needs new implementation with crouch)
  (if (Math|Boolean|ORBoolean (Utilities|Enum|Equal(Enum) _movementstate "NewEnumerator2") (Utilities|Enum|Equal(Enum) _movementstate "NewEnumerator5") (Utilities|Enum|Equal(Enum) _movementstate "NewEnumerator0") (Utilities|Enum|Equal(Enum) _movementstate "NewEnumerator15"))
    (Utilities|Time|ClearandInvalidateTimerbyHandle (Variables|Default|GetDashJumpTimer))
    (else
      (Transformation|SetActorRotation _player_2 (Math|Rotator|MakeRotator 0.0 0.0 (.yaw (Math|Rotator|MakeRotfromX (Math|Vector|Normalize (Transformation|GetVelocity _player_2)))))))))

(event EventBeginPlay
  (bind _returnvalue (Components|GetOwner))
  (bind _returnvalue_2 (Actor|GetComponentbyClass _returnvalue "/Script/Engine.CharacterMovementComponent"))
  ;[1 1 1] Initialize
  (Utilities|IsValid _returnvalue_2
    (:Is%20Valid
      (Variables|Default|SetMovementComponent _returnvalue_2)
      (Utilities|IsValid (Actor|GetComponentbyClass _returnvalue "AC_JumpComponent_C")
        (:Is%20Valid
          (CallFunction|SetJumpVariables)
          (bind _asbp_player (Utilities|Casting|CastToBP_Player _returnvalue))
          (bind _output_get (Variables|Default|SetPlayer _asbp_player))
          (EventDispatchers|BindEventtoStartJumpCall _output_get (EventDispatchers|CreateEvent :!event Custom|StartJump))
          (EventDispatchers|BindEventtoStopJumpCall _output_get (EventDispatchers|CreateEvent :!event Custom|StopJump))
          (EventDispatchers|BindEventtoLandedDelegate _output_get (EventDispatchers|CreateEvent :!event Custom|Land))
          (Variables|Default|SetInitialRotationRate (Variables|/Script/Engine.CharacterMovementComponent|GetRotationRate (Variables|Default|GetMovementComponent))))))))

(event EventTick
  (params (DeltaSeconds :type Float%20%28single-precision%29))
  ;[1 1 1] Tick
  (Variables|Default|SetDeltaSeconds DeltaSeconds)
  (CallFunction|SetCoyoteandJumpBufferTime)
  (if (not (Utilities|Enum|Equal(Enum) (Variables|/Game/Blueprints/ActorComponents/Player/MovementState/AC_MovementStateComponent.AC_MovementStateComponent_C|GetMovementState (Variables|/Game/Blueprints/Character/BP_Player.BP_Player_C|GetMovementStateComponent (Variables|Default|GetPlayer))) "NewEnumerator12"))
    (CallFunction|HandlyGravity)
    (Development|PrintString (Utilities|String|ToString(Float) (Variables|Default|GetCoyoteTime)) true true "(R=1.000000,G=0.040439,B=0.000000,A=1.000000)" 0.0)
    (Development|PrintString (Utilities|String|ToString(Float) (Variables|Default|GetCoyoteTimeCounter)) true true "(R=1.000000,G=0.028497,B=0.000000,A=1.000000)" 0.0)))

(fn SetCoyoteandJumpBufferTime
  (bind _movementcomponent (Variables|Default|GetMovementComponent)
    (:then
      (if (AI|Components|NavMovement|IsFalling _movementcomponent)
        (Variables|Default|SetCoyoteTimeCounter (|(A-B) (Variables|Default|GetCoyoteTimeCounter) (Variables|Default|GetDeltaSeconds)))
        (if (not (Variables|Default|GetJumpPressed))
          (Variables|Default|SetJumpBufferCounter (|(A-B) (Variables|Default|GetJumpBufferCounter) (Variables|Default|GetDeltaSeconds))))))
    (:else)))

(fn SetJumpVariables
  (bind _movementcomponent (Variables|Default|GetMovementComponent))
  (bind _movementcomponent_2 (Variables|Default|GetMovementComponent)
    (:then
      (Variables|/Script/Engine.CharacterMovementComponent|SetGravityScale _movementcomponent_2 (/ (* (Variables|Default|GetMaxJumpHeight) 2.0) (Math|Float|Power (Variables|Default|GetTimeToJumpApex) 2.0)))
      (Variables|Default|SetMaxJumpVelocity (|(A*{91AF9007-4FA9-6931-C4C1-8A966F925EE7}) (Variables|/Script/Engine.CharacterMovementComponent|GetGravityScale _movementcomponent_2)))
      (Variables|Default|SetMinJumpVelocity (|(sqrt(((2*A)*{8212DF45-4C46-578B-C0D7-A98199EC0D09}))) (Variables|/Script/Engine.CharacterMovementComponent|GetGravityScale (Variables|Default|GetMovementComponent))))
      (Variables|/Script/Engine.CharacterMovementComponent|SetGravityScale _movementcomponent (|(({B5ECD4AB-49F3-A052-BA61-D096EEECA631}*2)/(Pow({91AF9007-4FA9-6931-C4C1-8A966F925EE7},2)))))
      (Variables|Default|SetMaxDoubleJumpVelocity (|(A*{91AF9007-4FA9-6931-C4C1-8A966F925EE7}) (Variables|/Script/Engine.CharacterMovementComponent|GetGravityScale _movementcomponent)))
      (Variables|Default|SetCoyoteTimeCounter (Variables|Default|GetCoyoteTime))
      (Variables|/Script/Engine.CharacterMovementComponent|SetGravityScale (Variables|Default|GetMovementComponent) (Variables|Default|GetGravityScale)))
    (:else)))

(fn HandlyGravity
  (if (and (< (Math|Float|Absolute(Float) (.z (Variables|/Script/Engine.MovementComponent|GetVelocity (Variables|Default|GetMovementComponent)))) (Variables|Default|GetApexThreshold)) (Utilities|Enum|Equal(Enum) (Variables|/Game/Blueprints/ActorComponents/Player/MovementState/AC_MovementStateComponent.AC_MovementStateComponent_C|GetMovementState (Variables|/Game/Blueprints/Character/BP_Player.BP_Player_C|GetMovementStateComponent (Variables|Default|GetPlayer))) "NewEnumerator1"))
    ;[1 1 1] Set Gravity to low number for short airtime
    (Variables|/Script/Engine.CharacterMovementComponent|SetGravityScale (Variables|Default|GetMovementComponent) 2.0)
    (elif (< (.z (Variables|/Script/Engine.MovementComponent|GetVelocity (Variables|Default|GetMovementComponent))) 0.0)
      ;[1 1 1] Higher Gravity when player falls
      (Variables|/Script/Engine.CharacterMovementComponent|SetGravityScale (Variables|Default|GetMovementComponent) (* (Variables|Default|GetGravityScale) (Variables|Default|GetGravityFallMultiplier)))
      (switch Utilities|FlowControl|Switch|SwitchonENUM_MovementState (Variables|/Game/Blueprints/ActorComponents/Player/MovementState/AC_MovementStateComponent.AC_MovementStateComponent_C|GetMovementState (Variables|/Game/Blueprints/Character/BP_Player.BP_Player_C|GetMovementStateComponent (Variables|Default|GetPlayer)))
        (:NewEnumerator1
          _)
        (:NewEnumerator5
          _)
        (:NewEnumerator12
          _))
      (Variables|/Game/Blueprints/ActorComponents/Player/MovementState/AC_MovementStateComponent.AC_MovementStateComponent_C|SetMovementState (Variables|/Game/Blueprints/Character/BP_Player.BP_Player_C|GetMovementStateComponent (Variables|Default|GetPlayer)) "NewEnumerator0")
      (else
        (Variables|/Script/Engine.CharacterMovementComponent|SetGravityScale (Variables|Default|GetMovementComponent) (Variables|Default|GetGravityScale))))))