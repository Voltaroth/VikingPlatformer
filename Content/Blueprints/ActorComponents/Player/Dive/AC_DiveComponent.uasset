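; Player component that performs a mid-air dive from jumping, double jumping or falling, re-armed on landing.
; It binds to BP_Player's dive and landed events, then launches the character along DirectionControl's forward vector with friction removed.
; A looping timer pitches the mesh along velocity until the movement state changes, then restores cached movement values.
; A scrapped curve-driven dash remains, unreachable from live events.
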(event Custom|DoDive
  (bind _player (Variables|Default|GetPlayer))
  (bind _forwarddivevelocity (Variables|Default|GetForwardDiveVelocity))
  (bind _movementcomponent (Variables|Default|GetMovementComponent))
  (bind _returnvalue (- _forwarddivevelocity 5e+02))
  (bind _directioncontrol (Variables|/Game/Blueprints/Character/BP_Player.BP_Player_C|GetDirectionControl _player))
  (bind _velocity (Variables|/Script/Engine.MovementComponent|GetVelocity _movementcomponent))
  (bind _returnvalue_2 (Math|Vector|GetForwardVector _directioncontrol))
  (bind _returnvalue_3 (Math|Vector2D|MakeVector2D (.x _velocity) (.y _velocity)))
  (bind _returnvalue_4 (Math|Vector2D|Vector2DLength _returnvalue_3))
  (bind _returnvalue_5 (> _returnvalue_4 0.0))
  (bind _returnvalue_6 (select _returnvalue_5 _forwarddivevelocity _returnvalue))
  (bind _returnvalue_7 (* _returnvalue_6 _returnvalue_2))
  ;[1 1 1] Dive
  (Character|LaunchCharacter _player (+ (Math|Vector|MakeVector 0.0 0.0 (Variables|Default|GetUpDashVelocity)) _returnvalue_7) true true)
  (Variables|/Script/Engine.CharacterMovementComponent|SetMaxWalkSpeed (Variables|Default|GetMovementComponent) (Math|Vector|VectorLength _returnvalue_7))
  (Transformation|SetActorRotation (Variables|Default|GetPlayer) (Math|Rotator|MakeRotfromX (Math|Vector|GetForwardVector (Variables|/Game/Blueprints/Character/BP_Player.BP_Player_C|GetDirectionControl (Variables|Default|GetPlayer)))))
  (Variables|/Script/Engine.CharacterMovementComponent|SetRotationRate (Variables|Default|GetMovementComponent) "0.000000,90.000000,0.000000")
  (bind _returnvalue_8 (Utilities|Time|SetTimerbyEvent (delegate Custom|FollowMovement) (Utilities|Time|GetWorldDeltaSeconds) true))
  (Variables|Default|SetDiveTimer _returnvalue_8))

(event Custom|Landed
  (params (Hit :type Hit%20Result%20Structure%20%28by%20ref%29))
  (Variables|Default|SetCanDive true)
  (Variables|/Script/Engine.CharacterMovementComponent|SetFallingLateralFriction (Variables|Default|GetMovementComponent) 1.0)
  (Variables|/Game/Blueprints/ActorComponents/Player/MovementState/AC_MovementStateComponent.AC_MovementStateComponent_C|SetMovementState (Variables|/Game/Blueprints/Character/BP_Player.BP_Player_C|GetMovementStateComponent (Variables|Default|GetPlayer)) "NewEnumerator2")
  (CallFunction|ResetInitialDiveValues))

(event Custom|DoDash
  ;[1 0 0] DASH (scrapped)
  (bind _returnvalue (Utilities|Time|SetTimerbyEvent (delegate Custom|DashTick) (Utilities|Time|GetWorldDeltaSeconds) true))
  (Variables|Default|SetDashTimer _returnvalue))

(event Custom|StartDive
  (bind _movementcomponent (Variables|Default|GetMovementComponent))
  (bind _movementcomponent_2 (Variables|Default|GetMovementComponent))
  ;[1 1 1] Start Dash
  (Variables|Default|SetInitialGravity (Variables|/Script/Engine.CharacterMovementComponent|GetGravityScale _movementcomponent))
  (if (not (Utilities|Enum|Equal(Enum) (Variables|/Game/Blueprints/ActorComponents/Player/MovementState/AC_MovementStateComponent.AC_MovementStateComponent_C|GetMovementState (Variables|/Game/Blueprints/Character/BP_Player.BP_Player_C|GetMovementStateComponent (Variables|Default|GetPlayer))) "NewEnumerator12"))
    (if (AI|Components|NavMovement|IsFalling _movementcomponent)
      (if (Variables|Default|GetCanDive)
        (switch Utilities|FlowControl|Switch|SwitchonENUM_MovementState (Variables|/Game/Blueprints/ActorComponents/Player/MovementState/AC_MovementStateComponent.AC_MovementStateComponent_C|GetMovementState (Variables|/Game/Blueprints/Character/BP_Player.BP_Player_C|GetMovementStateComponent (Variables|Default|GetPlayer)))
          (:NewEnumerator1
            _)
          (:NewEnumerator5
            _)
          (:NewEnumerator0
            _))
        (Variables|/Game/Blueprints/ActorComponents/Player/MovementState/AC_MovementStateComponent.AC_MovementStateComponent_C|SetMovementState (Variables|/Game/Blueprints/Character/BP_Player.BP_Player_C|GetMovementStateComponent (Variables|Default|GetPlayer)) "NewEnumerator15")
        (Variables|Default|SetCanDive false)
        (Variables|/Script/Engine.CharacterMovementComponent|SetRotationRate (Variables|Default|GetMovementComponent) "0.000000,720.000000,0.000000")
        (Variables|/Script/Engine.CharacterMovementComponent|SetGroundFriction _movementcomponent_2 0.0)
        (Variables|/Script/Engine.CharacterMovementComponent|SetFallingLateralFriction _movementcomponent_2 0.0)
        (CallFunction|DoDive)))))

(event Custom|DashTick
  (bind _player (Variables|Default|GetPlayer))
  (bind _movementstatecomponent (Variables|/Game/Blueprints/Character/BP_Player.BP_Player_C|GetMovementStateComponent _player))
  ;[1 0 0] DASH (scrapped)
  (bind _output_get (Variables|Default|SetElapsedTimer (+ (Utilities|Time|GetWorldDeltaSeconds) (Variables|Default|GetElapsedTimer))))
  (if (or (> _output_get (Variables|Default|GetDashTime)) (Utilities|Enum|Equal(Enum) (Variables|/Game/Blueprints/ActorComponents/Player/MovementState/AC_MovementStateComponent.AC_MovementStateComponent_C|GetMovementState (Variables|/Game/Blueprints/Character/BP_Player.BP_Player_C|GetMovementStateComponent (Variables|Default|GetPlayer))) "NewEnumerator16"))
    (Variables|Default|SetElapsedTimer (- (Variables|Default|GetElapsedTimer) (Variables|Default|GetDashTime)))
    (Utilities|Time|ClearandInvalidateTimerbyHandle (Variables|Default|GetDashTimer))
    (CallFunction|ResetInitialDashValues)
    (switch Utilities|FlowControl|Switch|SwitchonENUM_MovementState (Variables|/Game/Blueprints/ActorComponents/Player/MovementState/AC_MovementStateComponent.AC_MovementStateComponent_C|GetMovementState (Variables|/Game/Blueprints/Character/BP_Player.BP_Player_C|GetMovementStateComponent (Variables|Default|GetPlayer)))
      (:NewEnumerator11
        (if (AI|Components|NavMovement|IsFalling (Variables|Default|GetMovementComponent))
          (Variables|/Game/Blueprints/ActorComponents/Player/MovementState/AC_MovementStateComponent.AC_MovementStateComponent_C|SetMovementState _movementstatecomponent "NewEnumerator0")
          (else
            (Variables|/Game/Blueprints/ActorComponents/Player/MovementState/AC_MovementStateComponent.AC_MovementStateComponent_C|SetMovementState _movementstatecomponent "NewEnumerator2")
            (Variables|/Script/Engine.CharacterMovementComponent|SetFallingLateralFriction (Variables|Default|GetMovementComponent) 1.0)))))
    (else
      (CallFunction|DetermineDashVelocity)
      (Variables|/Script/Engine.CharacterMovementComponent|SetFallingLateralFriction (Variables|Default|GetMovementComponent) 0.0))))

(event Custom|FollowMovement
  (bind _player (Variables|Default|GetPlayer))
  (bind _player_2 (Variables|Default|GetPlayer))
  (bind _movementstatecomponent (Variables|/Game/Blueprints/Character/BP_Player.BP_Player_C|GetMovementStateComponent _player))
  (bind _mesh (Variables|/Script/Engine.Character|GetMesh _player_2))
  (bind _movementstate (Variables|/Game/Blueprints/ActorComponents/Player/MovementState/AC_MovementStateComponent.AC_MovementStateComponent_C|GetMovementState _movementstatecomponent))
  ;[1 1 1] Dive
  (if (not (Math|Boolean|ORBoolean (Utilities|Enum|Equal(Enum) _movementstate "NewEnumerator2") (Utilities|Enum|Equal(Enum) _movementstate "NewEnumerator1") (Utilities|Enum|Equal(Enum) _movementstate "NewEnumerator0")))
    (Transformation|SetRelativeRotation _mesh (Math|Rotator|MakeRotator (* (.pitch (Math|Rotator|MakeRotfromX (Math|Vector|Normalize (Transformation|GetVelocity _player_2)))) -1.0) 0.0 (+ 0.0 -9e+01)) false false)
    (else
      (Transformation|SetRelativeRotation _mesh (Math|Rotator|MakeRotator 0.0 0.0 2.7e+02) false false)
      (CallFunction|ResetInitialDiveValues)
      (Utilities|Time|ClearandInvalidateTimerbyHandle (Variables|Default|GetDiveTimer)))))

(event EventBeginPlay
  (bind _returnvalue (Components|GetOwner))
  (bind _returnvalue_2 (Actor|GetComponentbyClass _returnvalue "/Script/Engine.CharacterMovementComponent"))
  ;[1 1 1] BeginPlay
  (Utilities|IsValid _returnvalue_2
    (:Is%20Valid
      (Variables|Default|SetMovementComponent _returnvalue_2)
      (Utilities|IsValid (Actor|GetComponentbyClass _returnvalue "AC_DiveComponent_C")
        (:Is%20Valid
          (bind _asbp_player (Utilities|Casting|CastToBP_Player _returnvalue))
          (bind _output_get (Variables|Default|SetPlayer _asbp_player))
          (EventDispatchers|BindEventtoStartDiveCall _output_get (EventDispatchers|CreateEvent :!event Custom|StartDive))
          (EventDispatchers|BindEventtoLandedDelegate _output_get (EventDispatchers|CreateEvent :!event Custom|Landed))
          (Variables|Default|SetInitialRotationRate (Variables|/Script/Engine.CharacterMovementComponent|GetRotationRate (Variables|Default|GetMovementComponent)))
          (Variables|Default|SetInitialAirControl (Variables|/Script/Engine.CharacterMovementComponent|GetAirControl (Variables|Default|GetMovementComponent)))
          (Variables|Default|SetInitialGroundFriction (Variables|/Script/Engine.CharacterMovementComponent|GetGroundFriction (Variables|Default|GetMovementComponent))))))))

(fn DetermineDashVelocity
  (bind _elapsedtimer (Variables|Default|GetElapsedTimer))
  (bind _dashtime (Variables|Default|GetDashTime))
  (bind _dashcurve (Variables|Default|GetDashCurve))
  (bind _player (Variables|Default|GetPlayer))
  (bind _player_2 (Variables|Default|GetPlayer))
  (bind _forwarddashvelocity (Variables|Default|GetForwardDashVelocity))
  (bind _returnvalue (Transformation|GetActorForwardVector _player_2))
  (bind _returnvalue_2 (/ _elapsedtimer _dashtime))
  (bind _movementstatecomponent (Variables|/Game/Blueprints/Character/BP_Player.BP_Player_C|GetMovementStateComponent _player))
  (bind _directioncontrol (Variables|/Game/Blueprints/Character/BP_Player.BP_Player_C|GetDirectionControl _player_2))
  (bind _returnvalue_3 (Math|Vector|GetForwardVector _directioncontrol))
  (bind _returnvalue_4 (Math|Curves|GetFloatValue _dashcurve _returnvalue_2))
  (bind _movementstate (Variables|/Game/Blueprints/ActorComponents/Player/MovementState/AC_MovementStateComponent.AC_MovementStateComponent_C|GetMovementState _movementstatecomponent))
  (bind _returnvalue_5 (Utilities|Enum|Equal(Enum) _movementstate "NewEnumerator0"))
  (bind _returnvalue_6 (* _returnvalue_4 _forwarddashvelocity))
  (bind _returnvalue_7 (select _returnvalue_5 _returnvalue _returnvalue_3))
  (bind _returnvalue_8 (* _returnvalue_7 _returnvalue_6))
  (Variables|/Script/Engine.MovementComponent|SetVelocity (Variables|Default|GetMovementComponent) (Math|Vector|MakeVector (.x _returnvalue_8) (.y _returnvalue_8) (.z (Transformation|GetVelocity (Variables|Default|GetPlayer))))))

(fn ResetInitialDiveValues
  (bind _movementcomponent (Variables|Default|GetMovementComponent))
  (Variables|/Script/Engine.CharacterMovementComponent|SetGroundFriction (Variables|Default|GetMovementComponent) (Variables|Default|GetInitialGroundFriction))
  (Variables|/Script/Engine.CharacterMovementComponent|SetRotationRate _movementcomponent (Variables|Default|GetInitialRotationRate))
  (Variables|/Script/Engine.CharacterMovementComponent|SetAirControl _movementcomponent (Variables|Default|GetInitialAirControl))
  (Variables|/Script/Engine.CharacterMovementComponent|SetGravityScale _movementcomponent (Variables|Default|GetInitialGravity))
  (Variables|/Script/Engine.CharacterMovementComponent|SetFallingLateralFriction (Variables|Default|GetMovementComponent) 1.0))

(fn DetermineAirDashVelocity
  (bind _elapsedtimer (Variables|Default|GetElapsedTimer))
  (bind _dashcurve (Variables|Default|GetDashCurve))
  (bind _player (Variables|Default|GetPlayer))
  (bind _player_2 (Variables|Default|GetPlayer))
  (bind _dashtime (Variables|Default|GetDashTime))
  (bind _forwarddivevelocity (Variables|Default|GetForwardDiveVelocity))
  (bind _returnvalue (Transformation|GetActorForwardVector _player_2))
  (bind _returnvalue_2 (+ _dashtime 0.05))
  (bind _movementstatecomponent (Variables|/Game/Blueprints/Character/BP_Player.BP_Player_C|GetMovementStateComponent _player))
  (bind _directioncontrol (Variables|/Game/Blueprints/Character/BP_Player.BP_Player_C|GetDirectionControl _player_2))
  (bind _returnvalue_3 (Math|Vector|GetForwardVector _directioncontrol))
  (bind _returnvalue_4 (/ _elapsedtimer _returnvalue_2))
  (bind _movementstate (Variables|/Game/Blueprints/ActorComponents/Player/MovementState/AC_MovementStateComponent.AC_MovementStateComponent_C|GetMovementState _movementstatecomponent))
  (bind _returnvalue_5 (Math|Curves|GetFloatValue _dashcurve _returnvalue_4))
  (bind _returnvalue_6 (Utilities|Enum|Equal(Enum) _movementstate "NewEnumerator0"))
  (bind _returnvalue_7 (* _returnvalue_5 _forwarddivevelocity))
  (bind _returnvalue_8 (select _returnvalue_6 _returnvalue _returnvalue_3))
  (bind _returnvalue_9 (* _returnvalue_8 _returnvalue_7))
  (Variables|/Script/Engine.MovementComponent|SetVelocity (Variables|Default|GetMovementComponent) (Math|Vector|MakeVector (.x _returnvalue_9) (.y _returnvalue_9) 0.0)))

(fn ResetInitialDashValues
  (bind _movementcomponent (Variables|Default|GetMovementComponent))
  (Variables|/Script/Engine.CharacterMovementComponent|SetGroundFriction (Variables|Default|GetMovementComponent) (Variables|Default|GetInitialGroundFriction))
  (Rendering|SetVisibility (Variables|/Script/Engine.Character|GetMesh (Variables|Default|GetPlayer)) true false)
  (Variables|/Script/Engine.CharacterMovementComponent|SetRotationRate _movementcomponent (Variables|Default|GetInitialRotationRate))
  (Variables|/Script/Engine.CharacterMovementComponent|SetAirControl _movementcomponent (Variables|Default|GetInitialAirControl))
  (Variables|/Script/Engine.CharacterMovementComponent|SetGravityScale _movementcomponent (Variables|Default|GetInitialGravity))
  (Variables|Default|SetElapsedTimer 0.0))