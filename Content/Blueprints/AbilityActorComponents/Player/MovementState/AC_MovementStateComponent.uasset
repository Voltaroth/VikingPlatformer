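; AC_MovementStateComponent is an actor component that holds an enum movement state for BP_Player.
; On BeginPlay it caches the owner's CharacterMovementComponent, checks that the owner has this component, stores the owner as BP_Player and sets an initial state.
; Tick is empty, and the logic that switches state when the player is falling is disconnected, so the state never updates within this graph.
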(event EventBeginPlay
  (bind _returnvalue (Components|GetOwner))
  (bind _returnvalue_2 (Actor|GetComponentbyClass _returnvalue "/Script/Engine.CharacterMovementComponent"))
  (Utilities|IsValid _returnvalue_2
    (:Is%20Valid
      (Variables|Default|SetMovementComponent _returnvalue_2)
      (Utilities|IsValid (Actor|GetComponentbyClass _returnvalue "AC_MovementStateComponent_C")
        (:Is%20Valid
          (bind _asbp_player (Utilities|Casting|CastToBP_Player _returnvalue))
          (Variables|Default|SetPlayer _asbp_player)
          (Variables|Default|SetMovementState "NewEnumerator2"))))))

(event EventTick
  (params (DeltaSeconds :type Float%20%28single-precision%29)))