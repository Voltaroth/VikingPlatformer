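; Thrown Mjölnir projectile that flies to a target, damages overlapping actors other than the player, then returns.
; Tick moves it with swept constant interpolation, at a speed scaled by a timeline curve.
; On a hit or nearing the target, it restarts that curve and chases an offset midpoint control point that drifts toward the player, arcing back.
; Near the player, it resets the in-hand hammer through AimAndThrowComponent and destroys itself.
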(event OnComponentBeginOverlap(Box)
  (params (OverlappedComponent :type Primitive%20Component%20Object%20Reference) (OtherActor :type Actor%20Object%20Reference) (OtherComp :type Primitive%20Component%20Object%20Reference) (OtherBodyIndex :type Integer) (bFromSweep :type Boolean) (SweepResult :type Hit%20Result%20Structure%20%28by%20ref%29))
  (if (not (== OtherActor (Game|GetPlayerCharacter 0)))
    (Class|BPIDamageable|TakeDamage(Message) OtherActor (Utilities|Struct|MakeS_DamageInfo 1 "NewEnumerator2"))))

(event Custom|ArchingCurve
  (Timeline|Timeline PlayFromStart))

(event Custom|StopSpeed
  ;[1 1 1] Calculate Travel Speed with curve
  (bind _velocitytoplayer (Timeline|VelocityToPlayer Stop)
    (:Update
      (Variables|Default|SetEffectiveFlySpeed (* _velocitytoplayer (Variables|Default|GetFlySpeed))))))

(event Custom|CalculateSpeedSpeed
  ;[1 1 1] Calculate Travel Speed with curve
  (bind _velocitytoplayer (Timeline|VelocityToPlayer PlayFromStart)
    (:Update
      (Variables|Default|SetEffectiveFlySpeed (* _velocitytoplayer (Variables|Default|GetFlySpeed))))))

(event EventBeginPlay
  (CallFunction|CalculateSpeedSpeed))

(event Collision|EventActorBeginOverlap
  (params (OtherActor :type Actor%20Object%20Reference)))

(event EventTick
  (params (DeltaSeconds :type Float%20%28single-precision%29))
  (bind _player (Variables|Default|GetPlayer))
  (Variables|Default|SetDelta%20Seconds DeltaSeconds)
  (Utilities|FlowControl|Sequence
    (:then_0
      (if (Utilities|Operators|EqualEqual (Variables|Default|GetTarget%20Location) (Transformation|GetActorLocation) 1e+02)
        (Variables|Default|SetReturn? true)))
    (:then_1
      ;[1 1 1] Fly forward if no return
      (if (Variables|Default|GetReturn?)
        (Utilities|FlowControl|Sequence
          (:then_0
            ;[1 1 1] check distance between player and mjölnir on return
            (Utilities|IsValid _player
              (:Is%20Valid
                (if (> (Transformation|GetDistanceTo _player) 1e+02)
                  (Utilities|FlowControl|Sequence
                    (:then_0
                      ;[1 1 1] If distance not close, return to player
                      (Utilities|FlowControl|DoOnce false :!label _label
                        (:Completed
                          (Variables|Default|SetTarget%20Location (Transformation|GetActorLocation (Variables|Default|GetPlayer)))
                          ;;[1 1 1] Little Delay before returning
                          (CallFunction|CalculateMidPoint)
                          (CallFunction|CurveControlPoint)
                          (CallFunction|StopSpeed)
                          (Variables|Default|SetEffectiveFlySpeed 0.0)
                          (CallFunction|CalculateSpeedSpeed))))
                    (:then_1
                      (Variables|Default|SetCurvedPoint (Math|Interpolation|VInterptoConstant (Variables|Default|GetCurvedPoint) (Transformation|GetActorLocation (Variables|Default|GetPlayer)) (Variables|Default|GetDelta%20Seconds) (Variables|Default|GetEffectiveFlySpeed)))
                      (Transformation|SetActorLocation (Math|Interpolation|VInterptoConstant (Transformation|GetActorLocation) (Variables|Default|GetCurvedPoint) (Variables|Default|GetDelta%20Seconds) (Variables|Default|GetEffectiveFlySpeed)) true false)))
                  (else
                    ;[1 1 1] If distance close, reset and destroy actor
                    (Variables|Default|SetReturn? false)
                    (Utilities|FlowControl|Sequence
                      (:then_0
                        (goto _label Reset))
                      (:then_1
                        (goto _label_2 Reset))
                      (:then_2
                        (Default|ResetMjolnirinHand (Variables|/Game/Blueprints/Character/BP_Player.BP_Player_C|GetAimAndThrowComponent (Variables|Default|GetPlayer)))
                        (Actor|DestroyActor))))))))
          (:then_1
            ;[1 1 1] disable collision on return (if mjölnir stuck)
            (Utilities|FlowControl|DoOnce false :!label _label_2
              (:Completed
                (Utilities|FlowControl|Delay 0.5)
                (Collision|SetCollisionEnabled (Variables|Default|GetBox) "NoCollision")))))
        (else
          (Transformation|SetActorLocation (Math|Interpolation|VInterptoConstant (Transformation|GetActorLocation) (Variables|Default|GetTarget%20Location) (Variables|Default|GetDelta%20Seconds) (Variables|Default|GetEffectiveFlySpeed)) true false))))))

(event Collision|EventHit
  (params (MyComp :type Primitive%20Component%20Object%20Reference) (Other :type Actor%20Object%20Reference) (OtherComp :type Primitive%20Component%20Object%20Reference) (bSelfMoved :type Boolean) (HitLocation :type Vector :default "0, 0, 0") (HitNormal :type Vector :default "0, 0, 0") (NormalImpulse :type Vector :default "0, 0, 0") (Hit :type Hit%20Result%20Structure%20%28by%20ref%29))
  ;[1 1 1] Return when hit something (maybe filter out enemies, since mjölnir should be able to fly through multiple)
  (Variables|Default|SetReturn? true))

(fn ConstructionScript)

(fn Shoot
  (params (Player :type BP%20Player%20Object%20Reference) (TargetLocation :type Vector) (Rotation :type Rotator))
  (Utilities|IsValid Player
    (:Is%20Valid
      (Variables|Default|SetPlayer Player)
      (Variables|Default|SetTarget%20Location TargetLocation)
      (Variables|Default|SetRotation Rotation))))

(fn CalculateMidPoint
  (bind _returnvalue (Transformation|GetActorLocation))
  (bind _target_location (Variables|Default|GetTarget%20Location))
  (Variables|Default|SetMidPoint (Math|Vector|MakeVector (/ (+ (.x _target_location) (.x _returnvalue)) 2.0) (/ (+ (.y _target_location) (.y _returnvalue)) 2.0) (/ (+ (.z _target_location) (.z _returnvalue)) 2.0))))

(fn CurveControlPoint
  (bind _midpoint (Variables|Default|GetMidPoint))
  (bind _target_location (Variables|Default|GetTarget%20Location))
  (bind _returnvalue (Math|Rotator|FindLookatRotation _midpoint _target_location))
  (bind (_x _y) (Math|Rotator|BreakRotIntoAxes _returnvalue))
  (Variables|Default|SetCurvedPoint (+ (Variables|Default|GetMidPoint) (Math|Vector|RotateVectorAroundAxis (* (Variables|Default|GetCurveRadius) _y) 0.0 _x))))

(fn GetPlayer
  (return (Variables|Default|GetPlayer)))