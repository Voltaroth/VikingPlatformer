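; Player actor component for aiming and throwing Mjolnir.
; Aiming switches the player camera and movement state and manages a crosshair widget.
; Throwing requires aiming with hammer in hand: it hides the held mesh, then spawns and shoots a projectile at a camera line-trace target, with mutual move-collision ignore.
; A montage's blend-out restores movement state, while ResetMjolnirInHand restores the held hammer.
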(event Custom|StartAim
  (bind _player (Variables|Default|GetPlayer))
  (switch Utilities|FlowControl|Switch|SwitchonENUM_MovementState (Variables|/Game/Blueprints/AbilityActorComponents/Player/MovementState/AC_MovementStateComponent.AC_MovementStateComponent_C|GetMovementState (Variables|/Game/Blueprints/Character/BP_Player.BP_Player_C|GetMovementStateComponent (Variables|Default|GetPlayer)))
    (:NewEnumerator2
      (Default|StartAim (Variables|/Game/Blueprints/Character/BP_Player.BP_Player_C|GetPlayerCamera _player))
      (Variables|/Game/Blueprints/Character/BP_Player.BP_Player_C|SetIsAiming? _player true)
      (Variables|/Game/Blueprints/AbilityActorComponents/Player/MovementState/AC_MovementStateComponent.AC_MovementStateComponent_C|SetMovementState (Variables|/Game/Blueprints/Character/BP_Player.BP_Player_C|GetMovementStateComponent (Variables|Default|GetPlayer)) "NewEnumerator16")
      (bind _crosshairwidget (Variables|Default|GetCrosshairWidget)
        (:then
          (Widget|RemovefromParent _crosshairwidget))
        (:else
          _))
      (bind _returnvalue (UserInterface|CreateWidget "/Game/Blueprints/Widgets/WBP_Crosshair.WBP_Crosshair_C" (Game|GetPlayerController 0)))
      (bind _output_get (Variables|Default|SetCrosshairWidget _returnvalue))
      (UserInterface|Viewport|AddtoViewport _output_get 0))))

(event Custom|Landed
  (params (Hit :type Hit%20Result%20Structure%20%28by%20ref%29))
  ;[1 1 1] Throw
  ;;[1 1 1] Reset on landed
  (Variables|Default|SetCanThrow? true))

(event Custom|StartThrow
  (bind _player (Variables|Default|GetPlayer))
  (bind _player_2 (Variables|Default|GetPlayer))
  (bind _player_3 (Variables|Default|GetPlayer))
  (bind _returnvalue (Transformation|GetActorLocation _player_3))
  (bind _movementstatecomponent (Variables|/Game/Blueprints/Character/BP_Player.BP_Player_C|GetMovementStateComponent _player_2))
  ;[1 1 1] Throw
  (if (Variables|/Game/Blueprints/Character/BP_Player.BP_Player_C|GetIsMjolnirInHand? (Variables|Default|GetPlayer))
    (switch Utilities|FlowControl|Switch|SwitchonENUM_MovementState (Variables|/Game/Blueprints/AbilityActorComponents/Player/MovementState/AC_MovementStateComponent.AC_MovementStateComponent_C|GetMovementState _movementstatecomponent)
      (:NewEnumerator16
        (Variables|/Game/Blueprints/AbilityActorComponents/Player/MovementState/AC_MovementStateComponent.AC_MovementStateComponent_C|SetMovementState _movementstatecomponent "NewEnumerator18")
        (Variables|Default|SetThrown? true)
        ;;[1 1 1] Make mjolnir invisible
        (Rendering|SetVisibility (Variables|/Game/Blueprints/Character/BP_Player.BP_Player_C|GetMjolnir (Variables|Default|GetPlayer)) false false)
        (bind _output_get (Variables|Default|SetMjolnirSpawnLocation (+ (* (Math|Vector|GetForwardVector (Variables|/Game/Blueprints/Character/BP_Player.BP_Player_C|GetDirectionControl (Variables|Default|GetPlayer))) 5e+01) (Math|Vector|MakeVector (.x _returnvalue) (.y _returnvalue) (+ (.z _returnvalue) 2e+01)))))
        (bind (_targetlocation _rotation) (CallFunction|ProjectileSpheretrace))
        (bind _returnvalue_2 (Game|SpawnActorfromClass "/Game/Blueprints/AbilityActorComponents/Player/Aiming/BP_Mjolnir_Projectile.BP_Mjolnir_Projectile_C" (Math|Transform|MakeTransform _output_get _rotation "1.000000,1.000000,1.000000") "AdjustIfPossibleButAlwaysSpawn" "OverrideRootScale" 0 (Variables|Default|GetPlayer)))
        ;;[1 1 1] Make it so player ignores projectile and vice versa
        (Variables|Default|SetMjölnirProjectile _returnvalue_2)
        (Collision|IgnoreActorwhenMoving (Variables|/Script/Engine.Character|GetCapsuleComponent _player) (Variables|Default|GetMjölnirProjectile) true)
        (Collision|IgnoreActorwhenMoving (Variables|/Game/Blueprints/AbilityActorComponents/Player/Aiming/BP_Mjolnir_Projectile.BP_Mjolnir_Projectile_C|GetBox (Variables|Default|GetMjölnirProjectile)) _player true)
        ;;[1 1 1] shoot mjolnir when spawned --> BP_Mjolnir_Projectile/otherwise, reset
        (Utilities|IsValid (Variables|Default|GetMjölnirProjectile)
          (:Is%20Valid
            (Default|Shoot (Variables|Default|GetMjölnirProjectile) (Variables|Default|GetPlayer) _targetlocation)
            ;;[1 1 1] Play throw montage
            (Animation|Montage|PlayMontage (Variables|/Script/Engine.Character|GetMesh (Variables|Default|GetPlayer)) "/Game/Assets/Characters/Leif/SKM/Leif_Animations/ANIM_Leif_Spin_Attack_Montage.ANIM_Leif_Spin_Attack_Montage"
              (:then
                (Variables|/Game/Blueprints/Character/BP_Player.BP_Player_C|SetIsMjolnirInHand? (Variables|Default|GetPlayer) false))
              (:OnBlendOut
                ;;[1 1 1] Set Movement States
                (if (Variables|/Game/Blueprints/Character/BP_Player.BP_Player_C|GetIsAiming? (Variables|Default|GetPlayer))
                  (Variables|/Game/Blueprints/AbilityActorComponents/Player/MovementState/AC_MovementStateComponent.AC_MovementStateComponent_C|SetMovementState (Variables|/Game/Blueprints/Character/BP_Player.BP_Player_C|GetMovementStateComponent (Variables|Default|GetPlayer)) "NewEnumerator16")
                  (else
                    (Variables|/Game/Blueprints/AbilityActorComponents/Player/MovementState/AC_MovementStateComponent.AC_MovementStateComponent_C|SetMovementState (Variables|/Game/Blueprints/Character/BP_Player.BP_Player_C|GetMovementStateComponent (Variables|Default|GetPlayer)) "NewEnumerator2"))))))
          (:Is%20Not%20Valid
            (CallFunction|ResetMjolnirinHand)))))))

(event Custom|StopAim
  (bind _player (Variables|Default|GetPlayer))
  (bind _player_2 (Variables|Default|GetPlayer))
  (bind _movementstatecomponent (Variables|/Game/Blueprints/Character/BP_Player.BP_Player_C|GetMovementStateComponent _player))
  (Default|StopAim (Variables|/Game/Blueprints/Character/BP_Player.BP_Player_C|GetPlayerCamera _player_2))
  (Variables|/Game/Blueprints/Character/BP_Player.BP_Player_C|SetIsAiming? _player_2 false)
  (bind _crosshairwidget (Variables|Default|GetCrosshairWidget)
    (:then
      (Widget|RemovefromParent _crosshairwidget)
      (if (AI|Components|NavMovement|IsFalling (Variables|/Script/Engine.Character|GetCharacterMovement (Variables|Default|GetPlayer)))
        (Variables|/Game/Blueprints/AbilityActorComponents/Player/MovementState/AC_MovementStateComponent.AC_MovementStateComponent_C|SetMovementState _movementstatecomponent "NewEnumerator0")
        (else
          (Variables|/Game/Blueprints/AbilityActorComponents/Player/MovementState/AC_MovementStateComponent.AC_MovementStateComponent_C|SetMovementState _movementstatecomponent "NewEnumerator2"))))
    (:else)))

(event Custom|ResetMjolnirInHand
  ;[1 1 1] Throw
  ;;[1 1 1] Reset when mjolnir returns or when not valid
  (Rendering|SetVisibility (Variables|/Game/Blueprints/Character/BP_Player.BP_Player_C|GetMjolnir (Variables|Default|GetPlayer)) true false)
  (Variables|/Game/Blueprints/Character/BP_Player.BP_Player_C|SetIsMjolnirInHand? (Variables|Default|GetPlayer) true))

(event EventBeginPlay
  (bind _returnvalue (Components|GetOwner))
  (Utilities|IsValid (Actor|GetComponentbyClass _returnvalue "AC_AimAndThrowComponent_C")
    (:Is%20Valid
      (bind _asbp_player (Utilities|Casting|CastToBP_Player _returnvalue))
      (bind _output_get (Variables|Default|SetPlayer _asbp_player))
      (EventDispatchers|BindEventtoLandedDelegate _output_get (EventDispatchers|CreateEvent :!event Custom|Landed)))))

(event EventTick
  (params (DeltaSeconds :type Float%20%28single-precision%29)))

(fn ProjectileSpheretrace
  (bind _player (Variables|Default|GetPlayer))
  (bind _playercamera (Variables|/Game/Blueprints/Character/BP_Player.BP_Player_C|GetPlayerCamera _player))
  (bind _playercamera_2 (Variables|/Game/Blueprints/Camera/BP_PlayerCamera.BP_PlayerCamera_C|GetPlayerCamera _playercamera))
  (bind _returnvalue (Math|Vector|GetForwardVector _playercamera_2))
  (bind _returnvalue_2 (Transformation|GetWorldLocation _playercamera_2))
  (bind (_outhit _returnvalue_3) (Collision|LineTraceByChannel (+ _returnvalue_2 (* _returnvalue (Variables|/Game/Blueprints/Camera/BP_PlayerCamera.BP_PlayerCamera_C|GetAimTargetArmLength _playercamera))) (+ _returnvalue_2 (* _returnvalue (Variables|Default|GetMaxThrowDistance))) "TraceTypeQuery1" false 0 "ForDuration" true "(R=1.000000,G=0.000000,B=0.000000,A=1.000000)" "(R=0.000000,G=1.000000,B=0.000000,A=1.000000)" 0.5))
  (return (Math|Vector|SelectVector (.ImpactPoint (Collision|BreakHitResult _outhit)) (.TraceEnd (Collision|BreakHitResult _outhit)) _returnvalue_3) (Math|Rotator|FindLookatRotation (Math|Vector|SelectVector (.ImpactPoint (Collision|BreakHitResult _outhit)) (.TraceEnd (Collision|BreakHitResult _outhit)) _returnvalue_3) (Transformation|GetActorLocation (Variables|Default|GetPlayer)))))