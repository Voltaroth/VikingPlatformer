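; Player combat component for BP_Player: three-hit Mjölnir combo, airborne spin attack, ground pound and curve-driven ground dodge.
; Each action uses a Tick-decremented input buffer and checks movement state, with attacks and ground pound also requiring Mjölnir in hand.
; Montage notifies and looping timers drive damage traces, combo windows and movement, including lunging toward traced targets.
; Landing re-enables attacks and ends an active ground pound.
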(event Custom|Landed
  (params (Hit :type Hit%20Result%20Structure%20%28by%20ref%29))
  ;[1 1 1] Reset on landed
  (Utilities|FlowControl|Sequence
    (:then_0
      (|AttackLanded))
    (:then_1
      (|GroundPoundLanded))))

(event EventBeginPlay
  (bind _returnvalue (Components|GetOwner))
  (Utilities|IsValid (Actor|GetComponentbyClass _returnvalue "AC_CombatComponent_C")
    (:Is%20Valid
      (bind _asbp_player (Utilities|Casting|CastToBP_Player _returnvalue))
      (bind _output_get (Variables|Components|SetPlayer _asbp_player))
      (EventDispatchers|BindEventtoLandedDelegate _output_get (EventDispatchers|CreateEvent :!event Custom|Landed))
      (Variables|Dodge|SetInitialGroundFriction (Variables|/Script/Engine.CharacterMovementComponent|GetGroundFriction (Variables|/Script/Engine.Character|GetCharacterMovement (Variables|Components|GetPlayer)))))))

(event EventTick
  (params (DeltaSeconds :type Float%20%28single-precision%29))
  ;[1 1 1] InputBufferCountDown
  (Variables|Default|SetDelta%20Seconds DeltaSeconds)
  (Utilities|FlowControl|Sequence
    (:then_0
      (|AttackBufferCountDown))
    (:then_1
      (|GroundPoundBufferCountDown))
    (:then_2
      (|DodgeBufferCountDown))))

(fn GroundPoundDamage
  (bind _player (Variables|Components|GetPlayer))
  (bind _returnvalue (Transformation|GetActorLocation _player))
  (bind _returnvalue_2 (- _returnvalue "0.000000,0.000000,100.000000"))
  (bind (_outhits _returnvalue_3) (Collision|MultiSphereTraceForObjects _returnvalue_2 _returnvalue_2 (Variables|GroundPound-Editable|GetDamageRadius) (Utilities|Array|MakeArray "ObjectTypeQuery6" "ObjectTypeQuery3") false 0 "None" true "(R=1.000000,G=0.000000,B=0.000000,A=1.000000)" "(R=0.000000,G=1.000000,B=0.000000,A=1.000000)" 0.5))
  (if _returnvalue_3
    (for _array_element _outhits
      (Class|BPIDamageable|TakeDamage(Message) (.HitActor (Collision|BreakHitResult _array_element)) (Utilities|Struct|MakeS_DamageInfo 1 "NewEnumerator1" "NewEnumerator0" false false (Variables|Components|GetPlayer) 0.025)))))

(fn SpinDamage
  (bind _player (Variables|Components|GetPlayer))
  (bind _returnvalue (Transformation|GetActorLocation _player))
  (bind (_outhits _returnvalue_2) (Class|KismetSystemLibrary|BoxTraceMultiforObjects _returnvalue _returnvalue (Variables|Spin-Editable|GetSpinDamageBoxDimensions) (Math|Rotator|MakeRotator 0.0 0.0 (.yaw (Transformation|GetActorRotation _player))) (Utilities|Array|MakeArray "ObjectTypeQuery6" "ObjectTypeQuery8" "ObjectTypeQuery3") false 0 "None" true))
  (if _returnvalue_2
    (for _array_element _outhits
      (Class|BPIDamageable|TakeDamage(Message) (.HitActor (Collision|BreakHitResult _array_element)) (Utilities|Struct|MakeS_DamageInfo 1 "NewEnumerator1" "NewEnumerator0" false false (Variables|Components|GetPlayer) 0.025)))))

(fn AttackDamage
  (bind _player (Variables|Components|GetPlayer))
  (bind _returnvalue (Transformation|GetActorForwardVector _player))
  (bind _returnvalue_2 (Transformation|GetActorLocation _player))
  (bind _returnvalue_3 (* _returnvalue 1e+02))
  (bind _returnvalue_4 (+ _returnvalue_2 _returnvalue_3))
  (bind (_outhits _returnvalue_5) (Class|KismetSystemLibrary|BoxTraceMultiforObjects _returnvalue_4 _returnvalue_4 (Variables|ComboAttack-Editable|GetComboDamageBoxDimension) (Math|Rotator|MakeRotator 0.0 0.0 (.yaw (Transformation|GetActorRotation _player))) (Utilities|Array|MakeArray "ObjectTypeQuery6" "ObjectTypeQuery8" "ObjectTypeQuery3") false 0 "None" true "(R=1.000000,G=0.000000,B=0.000000,A=1.000000)" "(R=0.000000,G=1.000000,B=0.000000,A=1.000000)" 1.0))
  (if _returnvalue_5
    (for _array_element _outhits
      (Class|BPIDamageable|TakeDamage(Message) (.HitActor (Collision|BreakHitResult _array_element)) (Utilities|Struct|MakeS_DamageInfo 1 "NewEnumerator1" "NewEnumerator0" false false (Variables|Components|GetPlayer) 0.025)))))

(fn MoveandRotateTowardsEnemy
  (bind _tracedenemy (Variables|ComboAttack|GetTracedEnemy))
  (bind _player (Variables|Components|GetPlayer))
  (bind _player_2 (Variables|Components|GetPlayer))
  (bind _returnvalue (Transformation|GetActorLocation _player))
  (bind _returnvalue_2 (Transformation|GetActorLocation _tracedenemy))
  (bind _output_get (Variables|Default|SetElapsedTimer (+ (Utilities|Time|GetWorldDeltaSeconds) (Variables|Default|GetElapsedTimer))))
  (if (> _output_get (Variables|ComboAttack-Editable|GetMoveTime))
    (Utilities|Time|ClearandInvalidateTimerbyHandle (Variables|ComboAttack|GetMoveTimerHandle))
    (Variables|Default|SetElapsedTimer 0.0)
    (else
      (Utilities|IsValid (Variables|ComboAttack|GetTracedEnemy)
        (:Is%20Valid
          (Transformation|SetActorLocation (Variables|Components|GetPlayer) (Math|Interpolation|VInterpTo (Transformation|GetActorLocation (Variables|Components|GetPlayer)) (+ _returnvalue_2 (* (Math|Vector|Normalize (- (Transformation|GetActorLocation (Variables|Components|GetPlayer)) _returnvalue_2)) (Variables|ComboAttack-Editable|GetDistanceFromTarget))) (Utilities|Time|GetWorldDeltaSeconds) 2e+01) true false)
          (Transformation|SetActorRotation (Variables|Components|GetPlayer) (Math|Interpolation|RInterpTo (Math|Rotator|MakeRotator 0.0 0.0 (.yaw (Transformation|GetActorRotation (Variables|Components|GetPlayer)))) (Math|Rotator|MakeRotator 0.0 0.0 (.yaw (Math|Rotator|FindLookatRotation (Transformation|GetActorLocation (Variables|Components|GetPlayer)) (Transformation|GetActorLocation (Variables|ComboAttack|GetTracedEnemy))))) (Utilities|Time|GetWorldDeltaSeconds) 5e+01)))
        (:Is%20Not%20Valid
          (Transformation|SetActorRotation (Variables|Components|GetPlayer) (Math|Interpolation|RInterpTo (Math|Rotator|MakeRotator 0.0 0.0 (.yaw (Transformation|GetActorRotation _player_2))) (Math|Rotator|MakeRotator 0.0 0.0 (.yaw (Math|Rotator|MakeRotfromX (Math|Vector|GetForwardVector (Variables|/Game/Blueprints/Character/BP_Player.BP_Player_C|GetDirectionControl _player_2))))) (Utilities|Time|GetWorldDeltaSeconds) 5e+01))
          (if (> (Math|Vector|VectorLength (Transformation|GetVelocity (Variables|Components|GetPlayer))) 0.0)
            (Transformation|SetActorLocation (Variables|Components|GetPlayer) (Math|Interpolation|VInterpTo _returnvalue (+ _returnvalue (* (Transformation|GetActorForwardVector (Variables|Components|GetPlayer)) (Variables|ComboAttack-Editable|GetLungeDistance))) (Utilities|Time|GetWorldDeltaSeconds) 2e+01) true false)))))))

(fn SetGroundValuesforDodge
  (bind _player (Variables|Components|GetPlayer))
  (bind _charactermovement (Variables|/Script/Engine.Character|GetCharacterMovement _player))
  (Variables|/Script/Engine.CharacterMovementComponent|SetBrakingDecelerationWalking _charactermovement 0.0)
  (Variables|/Script/Engine.CharacterMovementComponent|SetGroundFriction _charactermovement 0.0))

(fn DetermineDodgeVelocity
  (bind _elapsedtimer (Variables|Default|GetElapsedTimer))
  (bind _dodgecurve (Variables|Dodge-Editable|GetDodgeCurve))
  (bind _dodgevelocity (Variables|Dodge-Editable|GetDodgeVelocity))
  (bind _dodgetime (Variables|Dodge-Editable|GetDodgeTime))
  (bind _dodgevector (Variables|Dodge|GetDodgeVector))
  (bind _returnvalue (/ _elapsedtimer _dodgetime))
  (bind _returnvalue_2 (Math|Curves|GetFloatValue _dodgecurve _returnvalue))
  (bind _returnvalue_3 (* _returnvalue_2 _dodgevelocity))
  (bind _returnvalue_4 (* _dodgevector _returnvalue_3))
  (bind _output_get (Variables|/Script/Engine.MovementComponent|SetVelocity (Variables|/Script/Engine.Character|GetCharacterMovement (Variables|Components|GetPlayer)) (Math|Vector|MakeVector (.x _returnvalue_4) (.y _returnvalue_4) (.z (Transformation|GetVelocity (Variables|Components|GetPlayer))))))
  (Variables|/Script/Engine.CharacterMovementComponent|SetMaxWalkSpeed (Variables|/Script/Engine.Character|GetCharacterMovement (Variables|Components|GetPlayer)) (Math|Vector|VectorLength _output_get)))

(fn ResetInitialValues
  (Variables|/Script/Engine.CharacterMovementComponent|SetGroundFriction (Variables|/Script/Engine.Character|GetCharacterMovement (Variables|Components|GetPlayer)) (Variables|Dodge|GetInitialGroundFriction))
  (Variables|Default|SetElapsedTimer 0.0))

(event Custom|StartAttack
  (Variables|ComboAttack|SetAttackBufferCounter (Variables|ComboAttack-Editable|GetAttackBufferTime))
  (Variables|ComboAttack|SetAttackPressed? true)
  (Utilities|FlowControl|DelayUntilNextTick)
  (Variables|ComboAttack|SetAttackPressed? false)
  (Utilities|InputBufferLoop (Variables|ComboAttack|GetAttackBufferCounter) :!label _label)
  (if (Math|Boolean|ANDBoolean (Variables|Spin|GetCanAirAttack) (Variables|/Game/Blueprints/Character/BP_Player.BP_Player_C|GetIsMjölnirInHand? (Variables|Components|GetPlayer)) (Math|Boolean|ORBoolean (Utilities|Enum|Equal(Enum) (Variables|/Game/Blueprints/AbilityActorComponents/Player/MovementState/AC_MovementStateComponent.AC_MovementStateComponent_C|GetMovementState (Variables|/Game/Blueprints/Character/BP_Player.BP_Player_C|GetMovementStateComponent (Variables|Components|GetPlayer))) "NewEnumerator0") (Utilities|Enum|Equal(Enum) (Variables|/Game/Blueprints/AbilityActorComponents/Player/MovementState/AC_MovementStateComponent.AC_MovementStateComponent_C|GetMovementState (Variables|/Game/Blueprints/Character/BP_Player.BP_Player_C|GetMovementStateComponent (Variables|Components|GetPlayer))) "NewEnumerator1") (Utilities|Enum|Equal(Enum) (Variables|/Game/Blueprints/AbilityActorComponents/Player/MovementState/AC_MovementStateComponent.AC_MovementStateComponent_C|GetMovementState (Variables|/Game/Blueprints/Character/BP_Player.BP_Player_C|GetMovementStateComponent (Variables|Components|GetPlayer))) "NewEnumerator5")))
    (Variables|/Game/Blueprints/AbilityActorComponents/Player/MovementState/AC_MovementStateComponent.AC_MovementStateComponent_C|SetMovementState (Variables|/Game/Blueprints/Character/BP_Player.BP_Player_C|GetMovementStateComponent (Variables|Components|GetPlayer)) "NewEnumerator20")
    ;[1 1 1] If attack in the air launch character
    (Variables|ComboAttack|SetAttackCount 0)
    (Variables|Spin|SetCanAirAttack false)
    (Variables|ComboAttack|SetAttackBufferCounter 0.0)
    (bind _player (Variables|Components|GetPlayer)
      (:then
        (Character|LaunchCharacter _player (Math|Vector|MakeVector 0.0 0.0 (Variables|Spin-Editable|GetSpinVelocityZ)) false true)
        ;[1 1 1] Play montages
        (Animation|Montage|PlayMontage (Variables|/Script/Engine.Character|GetMesh _player) "/Game/Assets/Characters/Leif/SKM/Leif_Animations/ANIM_Leif_Spin_Attack_Montage.ANIM_Leif_Spin_Attack_Montage"
          (:then
            (Animation|Montage|PlayMontage (Variables|/Game/Blueprints/Character/BP_Player.BP_Player_C|GetSKM_Mjölnir (Variables|Components|GetPlayer)) "/Game/Assets/Characters/Mjolnir/SKM/Mjolnir_Animations/ANIM_Mjolnir_Spin_Attack_Montage.ANIM_Mjolnir_Spin_Attack_Montage"
              (:then
                ;[1 1 1] DoDamage
                (bind _returnvalue (Utilities|Time|SetTimerbyEvent (delegate Custom|DamageTick) 0.1 true))
                (Variables|GroundPound|SetSphereTraceTimer _returnvalue))))
          (:OnBlendOut
            (Default|ResettoNextState (Variables|/Game/Blueprints/Character/BP_Player.BP_Player_C|GetMovementStateComponent (Variables|Components|GetPlayer))))))
      (:else))
    (elif (Math|Boolean|ANDBoolean (Utilities|Enum|Equal(Enum) (Variables|/Game/Blueprints/AbilityActorComponents/Player/MovementState/AC_MovementStateComponent.AC_MovementStateComponent_C|GetMovementState (Variables|/Game/Blueprints/Character/BP_Player.BP_Player_C|GetMovementStateComponent (Variables|Components|GetPlayer))) "NewEnumerator2") (Variables|/Game/Blueprints/Character/BP_Player.BP_Player_C|GetIsMjölnirInHand? (Variables|Components|GetPlayer)) (Variables|ComboAttack|GetCanAttack?))
      ;[1 1 1] If AttackCount > 2, reset to zero and try again
      (if (> (Variables|ComboAttack|GetAttackCount) 2) :!label _label_2
        (Variables|ComboAttack|SetAttackCount 0)
        (goto _label_2)
        (else
          ;[1 1 1] Trace for enemies and set target
          (bind _hitactor (Default|TraceforHittable (Variables|Components|GetPlayer)))
          (Variables|ComboAttack|SetTracedEnemy _hitactor)
          (Variables|/Game/Blueprints/AbilityActorComponents/Player/MovementState/AC_MovementStateComponent.AC_MovementStateComponent_C|SetMovementState (Variables|/Game/Blueprints/Character/BP_Player.BP_Player_C|GetMovementStateComponent (Variables|Components|GetPlayer)) "NewEnumerator17")
          ;[1 1 1] Set general variables
          (Variables|ComboAttack|SetAllowRotation false)
          (Variables|/Script/Engine.CharacterMovementComponent|SetMaxWalkSpeed (Variables|/Script/Engine.Character|GetCharacterMovement (Variables|Components|GetPlayer)) (Utilities|Select :Index (Variables|ComboAttack|GetAttackCount) :Option%200 (Variables|ComboAttack-Editable|GetMaxWalkSpeedDuringCombo) :Option%201 1.5e+02 :Option%202 2.5e+02))
          (Variables|ComboAttack|SetAttackBufferCounter 0.0)
          (Variables|ComboAttack|SetCanAttack? false)
          ;[1 1 1] Move and Rotate Towards Target
          (bind _returnvalue_2 (Utilities|Time|SetTimerbyEvent (delegate Custom|MoveToTargetTick) (Utilities|Time|GetWorldDeltaSeconds) true))
          (Variables|ComboAttack|SetMoveTimerHandle _returnvalue_2)
          (Animation|Montage|PlayMontage (Variables|/Game/Blueprints/Character/BP_Player.BP_Player_C|GetSKM_Mjölnir (Variables|Components|GetPlayer)) (Utilities|Select :Index (Variables|ComboAttack|GetAttackCount) :Option%200 "/Game/Assets/Characters/Mjolnir/SKM/Mjolnir_Animations/ANIM_Mjolnir_Attack_01_Montage.ANIM_Mjolnir_Attack_01_Montage" :Option%201 "/Game/Assets/Characters/Mjolnir/SKM/Mjolnir_Animations/ANIM_Mjolnir_Attack_02_Montage.ANIM_Mjolnir_Attack_02_Montage" :Option%202 "/Game/Assets/Characters/Mjolnir/SKM/Mjolnir_Animations/ANIM_Mjolnir_Attack_03_Montage.ANIM_Mjolnir_Attack_03_Montage")
            (:then
              ;[1 1 1] Play right montage depending on combo count
              (bind _notifyname (Animation|Montage|PlayMontage (Variables|/Script/Engine.Character|GetMesh (Variables|Components|GetPlayer)) (Utilities|Select :Index (Variables|ComboAttack|GetAttackCount) :Option%200 "/Game/Assets/Characters/Leif/SKM/Leif_Animations/ANIM_Leif_Attack_01_Montage.ANIM_Leif_Attack_01_Montage" :Option%201 "/Game/Assets/Characters/Leif/SKM/Leif_Animations/ANIM_Leif_Attack_02_Montage.ANIM_Leif_Attack_02_Montage" :Option%202 "/Game/Assets/Characters/Leif/SKM/Leif_Animations/ANIM_Leif_Attack_03_Montage.ANIM_Leif_Attack_03_Montage"))
                (:then
                  ;[1 1 1] Add to combo count, check after little delay after every combo if counter above 1, then set to 0 (Combo TimeFrame)
                  (Math|Integer|IncrementInt (Variables|ComboAttack|GetAttackCount)
                    (:%20%20
                      (Utilities|FlowControl|RetriggerableDelay 0.5)
                      (if (>= (Variables|ComboAttack|GetAttackCount) 1)
                        (Variables|ComboAttack|SetAttackCount 0)))))
                (:OnBlendOut
                  ;[1 1 1] Set variables on blend out
                  (Variables|ComboAttack|SetAllowRotation true)
                  (Variables|/Script/Engine.CharacterMovementComponent|SetMaxWalkSpeed (Variables|/Script/Engine.Character|GetCharacterMovement (Variables|Components|GetPlayer)) 1e+03)
                  (Variables|ComboAttack|SetCanAttack? true)
                  (Default|ResettoNextState (Variables|/Game/Blueprints/Character/BP_Player.BP_Player_C|GetMovementStateComponent (Variables|Components|GetPlayer))))
                (:OnNotifyBegin
                  ;[1 1 1] On Notify Events
                  (switch name _notifyname
                    (:Combo
                      (Variables|ComboAttack|SetCanAttack? true)
                      (Default|ResettoNextState (Variables|/Game/Blueprints/Character/BP_Player.BP_Player_C|GetMovementStateComponent (Variables|Components|GetPlayer))))
                    (:Attack
                      (ComboAttack|AttackDamage))
                    (:AllowRotation
                      (Variables|/Script/Engine.CharacterMovementComponent|SetMaxWalkSpeed (Variables|/Script/Engine.Character|GetCharacterMovement (Variables|Components|GetPlayer)) 1e+03)))))))))
      (else
        (goto _label Recheck)))))

(event Custom|DamageTick
  (bind _player (Variables|Components|GetPlayer))
  (bind _returnvalue (Transformation|GetVelocity _player))
  ;[1 1 1] DoDamage
  (bind _output_get (Variables|Default|SetElapsedTimer (+ 0.05 (Variables|Default|GetElapsedTimer))))
  (if (> _output_get 0.2)
    (Utilities|Time|ClearandInvalidateTimerbyHandle (Variables|GroundPound|GetSphereTraceTimer))
    (Variables|Default|SetElapsedTimer 0.0)
    (else
      (Variables|/Script/Engine.MovementComponent|SetVelocity (Variables|/Script/Engine.Character|GetCharacterMovement (Variables|Components|GetPlayer)) (Math|Vector|MakeVector (.x _returnvalue) (.y _returnvalue) (Variables|Spin-Editable|GetSpinVelocityZ)))
      (Spin|SpinDamage))))

(event Custom|MoveToTargetTick
  ;[1 1 1] Move and Rotate Towards Target
  (ComboAttack|MoveandRotateTowardsEnemy))

(event Custom|StartGroundPound
  (bind _player (Variables|Components|GetPlayer))
  (bind _player_2 (Variables|Components|GetPlayer))
  (bind _returnvalue (Transformation|GetVelocity _player_2))
  (bind _charactermovement (Variables|/Script/Engine.Character|GetCharacterMovement _player))
  (Variables|GroundPound|SetGroundPoundPressed? true)
  (Utilities|FlowControl|Sequence
    (:then_0
      (Variables|GroundPound|SetGroundPoundBufferCounter (Variables|GroundPound-Editable|GetGroundPoundBufferTime))
      (Utilities|InputBufferLoop (Variables|GroundPound|GetGroundPoundBufferCounter) :!label _label)
      (if (Math|Boolean|ANDBoolean (Variables|/Game/Blueprints/Character/BP_Player.BP_Player_C|GetIsMjölnirInHand? (Variables|Components|GetPlayer)) (Variables|GroundPound|GetCanGroundPound) (> (.distance (Default|TraceforGround (Variables|Components|GetPlayer))) 25.0) (Math|Boolean|ORBoolean (Utilities|Enum|Equal(Enum) (Variables|/Game/Blueprints/AbilityActorComponents/Player/MovementState/AC_MovementStateComponent.AC_MovementStateComponent_C|GetMovementState (Variables|/Game/Blueprints/Character/BP_Player.BP_Player_C|GetMovementStateComponent (Variables|Components|GetPlayer))) "NewEnumerator1") (Utilities|Enum|Equal(Enum) (Variables|/Game/Blueprints/AbilityActorComponents/Player/MovementState/AC_MovementStateComponent.AC_MovementStateComponent_C|GetMovementState (Variables|/Game/Blueprints/Character/BP_Player.BP_Player_C|GetMovementStateComponent (Variables|Components|GetPlayer))) "NewEnumerator5") (Utilities|Enum|Equal(Enum) (Variables|/Game/Blueprints/AbilityActorComponents/Player/MovementState/AC_MovementStateComponent.AC_MovementStateComponent_C|GetMovementState (Variables|/Game/Blueprints/Character/BP_Player.BP_Player_C|GetMovementStateComponent (Variables|Components|GetPlayer))) "NewEnumerator0")))
        (Variables|/Game/Blueprints/Character/BP_Player.BP_Player_C|SetCanMove? (Variables|Components|GetPlayer) false)
        (Variables|GroundPound|SetCanGroundPound false)
        (Variables|GroundPound|SetDidGroundPound true)
        (Variables|GroundPound|SetGroundPoundBufferCounter 0.0)
        (Variables|/Script/Engine.MovementComponent|SetVelocity _charactermovement (Math|Vector|MakeVector (.x (Variables|/Script/Engine.MovementComponent|GetVelocity _charactermovement)) (.y (Variables|/Script/Engine.MovementComponent|GetVelocity _charactermovement)) 0.0))
        (Character|LaunchCharacter _player_2 (Math|Vector|MakeVector (/ (.x _returnvalue) 8.0) (/ (.y _returnvalue) 8.0) 0.0) true false)
        (Variables|/Game/Blueprints/AbilityActorComponents/Player/MovementState/AC_MovementStateComponent.AC_MovementStateComponent_C|SetMovementState (Variables|/Game/Blueprints/Character/BP_Player.BP_Player_C|GetMovementStateComponent (Variables|Components|GetPlayer)) "NewEnumerator19")
        (bind _notifyname (Animation|Montage|PlayMontage (Variables|/Script/Engine.Character|GetMesh (Variables|Components|GetPlayer)) "/Game/Assets/Characters/Leif/SKM/Leif_Animations/ANIM_Leif_GroundPound_Montage.ANIM_Leif_GroundPound_Montage")
          (:then
            (Animation|Montage|PlayMontage (Variables|/Game/Blueprints/Character/BP_Player.BP_Player_C|GetSKM_Mjölnir (Variables|Components|GetPlayer)) "/Game/Assets/Characters/Mjolnir/SKM/Mjolnir_Animations/ANIM_Mjolnir_GroundPound_Montage.ANIM_Mjolnir_GroundPound_Montage"
              (:then
                (Default|JumpSqueeze (Variables|Components|GetPlayer))
                (Utilities|FlowControl|Delay (Variables|GroundPound|GetGroundPoundCooldown))
                (Variables|GroundPound|SetCanGroundPound true))))
          (:OnNotifyBegin
            (switch name _notifyname
              (:BeginDrop
                (Utilities|FlowControl|Delay 0.1)
                (Character|LaunchCharacter (Variables|Components|GetPlayer) (Math|Vector|MakeVector 0.0 0.0 (Variables|GroundPound-Editable|GetGroundPoundVelocityZ)) false true)
                (bind _returnvalue_2 (Utilities|Time|SetTimerbyEvent (delegate Custom|GroundPoundTick) 0.01 true))
                (Variables|Default|SetGroundPoundTimerHandle _returnvalue_2)))))
        (else
          (goto _label Recheck))))
    (:then_1
      (Utilities|FlowControl|DelayUntilNextTick)
      (Variables|GroundPound|SetGroundPoundPressed? false))))

(event Custom|GroundPoundTick
  (GroundPound|GroundPoundDamage))

(event Custom|DodgeTick
  (bind _player (Variables|Components|GetPlayer))
  ;[1 1 1] GroundDodge
  ;;[1 1 1] Set Ground Values and Start sliding
  (bind _output_get (Variables|Default|SetElapsedTimer (+ (Utilities|Time|GetWorldDeltaSeconds) (Variables|Default|GetElapsedTimer))))
  (if (or (> _output_get (Variables|Dodge-Editable|GetDodgeTime)) (Variables|Dodge|GetCancelDodge?))
    (Utilities|Time|ClearandInvalidateTimerbyHandle (Variables|Dodge|GetDashTimerHandle))
    (Dodge|ResetInitialValues)
    (Variables|Dodge|SetCancelDodge? false)
    ;;[1 1 1] Reset Movement Mode
    (Default|ResettoNextState (Variables|/Game/Blueprints/Character/BP_Player.BP_Player_C|GetMovementStateComponent (Variables|Components|GetPlayer)))
    (else
      (Transformation|SetActorRotation _player (Math|Interpolation|RInterpTo (Math|Rotator|MakeRotator 0.0 0.0 (.yaw (Transformation|GetActorRotation _player))) (Math|Rotator|MakeRotator 0.0 0.0 (.yaw (Math|Rotator|MakeRotfromX (Variables|Dodge|GetDodgeVector)))) (Utilities|Time|GetWorldDeltaSeconds) 8e+01))
      (Dodge|DetermineDodgeVelocity))))

(event Custom|GroundDodge
  ;[1 1 1] GroundDodge
  ;;[1 1 1] SetMovementMode and Play Montage
  (Variables|Dodge|SetCancelDodge? false)
  (Variables|Dodge|SetDodgeBufferCounter 0.0)
  (Variables|/Game/Blueprints/AbilityActorComponents/Player/MovementState/AC_MovementStateComponent.AC_MovementStateComponent_C|SetMovementState (Variables|/Game/Blueprints/Character/BP_Player.BP_Player_C|GetMovementStateComponent (Variables|Components|GetPlayer)) "NewEnumerator11")
  (Animation|Montage|PlayMontage (Variables|/Script/Engine.Character|GetMesh (Variables|Components|GetPlayer)) "/Game/Assets/Characters/Leif/SKM/Leif_Animations/ANIM_Leif_Dodge_Montage.ANIM_Leif_Dodge_Montage"
    (:then
      ;;[1 1 1] Set Vector to dash to
      (Variables|Dodge|SetDodgeVector (Math|Vector|GetForwardVector (Variables|/Game/Blueprints/Character/BP_Player.BP_Player_C|GetDirectionControl (Variables|Components|GetPlayer))))
      ;;[1 1 1] Set Ground Values and Start sliding
      (Dodge|SetGroundValuesforDodge)
      (bind _returnvalue (Utilities|Time|SetTimerbyEvent (delegate Custom|DodgeTick) (Utilities|Time|GetWorldDeltaSeconds) true))
      (Variables|Dodge|SetDashTimerHandle _returnvalue))))

(event Custom|StartDodge
  ;[1 1 1] StartDodge
  (Variables|Dodge|SetDodgeBufferCounter (Variables|Dodge-Editable|GetDodgeBufferTime))
  (Variables|Dodge|SetDodgePressed? true)
  (Utilities|FlowControl|Sequence
    (:then_0
      (Utilities|FlowControl|DelayUntilNextTick)
      (Variables|Dodge|SetDodgePressed? false)
      (Utilities|InputBufferLoop (Variables|Dodge|GetDodgeBufferCounter) :!label _label)
      (if (Utilities|Enum|Equal(Enum) (Variables|/Game/Blueprints/AbilityActorComponents/Player/MovementState/AC_MovementStateComponent.AC_MovementStateComponent_C|GetMovementState (Variables|/Game/Blueprints/Character/BP_Player.BP_Player_C|GetMovementStateComponent (Variables|Components|GetPlayer))) "NewEnumerator2")
        (CallFunction|GroundDodge)
        (else
          (goto _label Recheck))))))