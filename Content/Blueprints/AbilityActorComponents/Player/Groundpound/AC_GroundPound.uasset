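; Player actor component for a Mjölnir ground pound, usable in mid-air while the hammer is in hand and off cooldown.
; Starting it locks input, damps momentum and plays paired character and hammer montages, whose notify triggers a fast downward launch.
; The player's Landed delegate then applies sphere-trace damage to destructibles and another object type, adds squeeze and an upward bounce, stops the montages and restores input.
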(event Custom|StartGroundPound
  (bind _player (Variables|Default|GetPlayer))
  (bind _player_2 (Variables|Default|GetPlayer))
  (bind _returnvalue (Transformation|GetVelocity _player_2))
  (bind _charactermovement (Variables|/Script/Engine.Character|GetCharacterMovement _player))
  (if (and (Variables|/Game/Blueprints/Character/BP_Player.BP_Player_C|GetIsMjölnirInHand? (Variables|Default|GetPlayer)) (Variables|Default|GetCanGroundPound))
    (switch Utilities|FlowControl|Switch|SwitchonENUM_MovementState (Variables|/Game/Blueprints/AbilityActorComponents/Player/MovementState/AC_MovementStateComponent.AC_MovementStateComponent_C|GetMovementState (Variables|/Game/Blueprints/Character/BP_Player.BP_Player_C|GetMovementStateComponent (Variables|Default|GetPlayer)))
      (:NewEnumerator1
        _)
      (:NewEnumerator5
        _)
      (:NewEnumerator0
        _))
    (Input|DisableInput (Variables|Default|GetPlayer) (Game|GetPlayerController 0))
    (Variables|Default|SetCanGroundPound false)
    (Variables|Default|SetDidGroundPound true)
    (Variables|/Script/Engine.MovementComponent|SetVelocity _charactermovement (Math|Vector|MakeVector (.x (Variables|/Script/Engine.MovementComponent|GetVelocity _charactermovement)) (.y (Variables|/Script/Engine.MovementComponent|GetVelocity _charactermovement)) 0.0))
    (Character|LaunchCharacter _player_2 (Math|Vector|MakeVector (/ (.x _returnvalue) 8.0) (/ (.y _returnvalue) 8.0) 0.0) true false)
    (Variables|/Game/Blueprints/AbilityActorComponents/Player/MovementState/AC_MovementStateComponent.AC_MovementStateComponent_C|SetMovementState (Variables|/Game/Blueprints/Character/BP_Player.BP_Player_C|GetMovementStateComponent (Variables|Default|GetPlayer)) "NewEnumerator19")
    (bind _notifyname (Animation|Montage|PlayMontage (Variables|/Script/Engine.Character|GetMesh (Variables|Default|GetPlayer)) "/Game/Assets/Characters/Leif/SKM/Leif_Animations/ANIM_Leif_GroundPound_Montage.ANIM_Leif_GroundPound_Montage")
      (:then
        (Animation|Montage|PlayMontage (Variables|/Game/Blueprints/Character/BP_Player.BP_Player_C|GetSKM_Mjölnir (Variables|Default|GetPlayer)) "/Game/Assets/Characters/Mjölnir/SKM/Mjölnir_Animations/ANIM_Mjölnir_GroundPound_Montage.ANIM_Mjölnir_GroundPound_Montage"
          (:then
            (Default|JumpSqueeze (Variables|Default|GetPlayer))
            (Utilities|FlowControl|Delay (Variables|Default|GetDashCooldown))
            (Variables|Default|SetCanGroundPound true))))
      (:OnNotifyBegin
        (switch name _notifyname
          (:BeginDrop
            (Utilities|FlowControl|Delay 0.1)
            (Character|LaunchCharacter (Variables|Default|GetPlayer) "0.000000,0.000000,-5000.000000" false true)))))))

(event Custom|Landed
  (params (Hit :type Hit%20Result%20Structure%20%28by%20ref%29))
  (bind _player (Variables|Default|GetPlayer))
  (if (Variables|Default|GetDidGroundPound)
    (Variables|Default|SetDidGroundPound false)
    (Default|LandSqueeze _player)
    (CallFunction|DoDamage)
    (Utilities|FlowControl|Delay 0.1)
    (Character|LaunchCharacter (Variables|Default|GetPlayer) "0.000000,0.000000,400.000000" false true)
    (Animation|Montage|MontageStop (Components|SkeletalMesh|GetAnimInstance (Variables|/Script/Engine.Character|GetMesh _player)) 0.2 "/Game/Assets/Characters/Leif/SKM/Leif_Animations/ANIM_Leif_GroundPound_Montage.ANIM_Leif_GroundPound_Montage")
    (Animation|Montage|MontageStop (Components|SkeletalMesh|GetAnimInstance (Variables|/Game/Blueprints/Character/BP_Player.BP_Player_C|GetSKM_Mjölnir (Variables|Default|GetPlayer))) 0.2 "/Game/Assets/Characters/Mjölnir/SKM/Mjölnir_Animations/ANIM_Mjölnir_GroundPound_Montage.ANIM_Mjölnir_GroundPound_Montage")
    (Input|EnableInput (Variables|Default|GetPlayer) (Game|GetPlayerController 0))))

(event EventBeginPlay
  (bind _returnvalue (Components|GetOwner))
  (Utilities|IsValid (Actor|GetComponentbyClass _returnvalue "AC_GroundPound_C")
    (:Is%20Valid
      (bind _asbp_player (Utilities|Casting|CastToBP_Player _returnvalue))
      (bind _output_get (Variables|Default|SetPlayer _asbp_player))
      (EventDispatchers|BindEventtoLandedDelegate _output_get (EventDispatchers|CreateEvent :!event Custom|Landed)))))

(event EventTick
  (params (DeltaSeconds :type Float%20%28single-precision%29)))

(fn DoDamage
  (bind _player (Variables|Default|GetPlayer))
  (bind _returnvalue (Transformation|GetActorLocation _player))
  (bind (_outhits _returnvalue_2) (Collision|MultiSphereTraceForObjects _returnvalue _returnvalue (Variables|Default|GetDamageRadius) (Utilities|Array|MakeArray "ObjectTypeQuery6" "ObjectTypeQuery8") false 0 "None" true "(R=1.000000,G=0.000000,B=0.000000,A=1.000000)" "(R=0.000000,G=1.000000,B=0.000000,A=1.000000)" 1.0))
  (if _returnvalue_2
    (for _array_element _outhits
      (Class|BPIDamageable|TakeDamage(Message) (.HitActor (Collision|BreakHitResult _array_element)) (Utilities|Struct|MakeS_DamageInfo 1 "NewEnumerator1")))))