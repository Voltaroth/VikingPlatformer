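; Player dodge component that performs a montage-driven ground dash along the direction control's forward vector.
; Dodge input starts a countdown buffer, rechecking until the movement state permits a GroundDodge.
; The dodge zeroes friction, braking and rotation rate, then a looping per-frame timer turns the player and drives horizontal velocity from DashCurve.
; After DashTime it restores friction and rotation rate and advances the movement state.
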(event Custom|StartDodge
  ;[1 1 1] Only Continue if input buffer still active / is idle or walking
  (Variables|Default|SetDodgeBufferCounter (Variables|Editable|GetDodgeBufferTime))
  (Variables|Default|SetDodgePressed? true)
  (Utilities|FlowControl|Sequence
    (:then_0
      (Utilities|FlowControl|DelayUntilNextTick)
      (Variables|Default|SetDodgePressed? false)
      (Utilities|InputBufferLoop (Variables|Default|GetDodgeBufferCounter) :!label _label)
      (if (Utilities|Enum|Equal(Enum) (Variables|/Game/Blueprints/AbilityActorComponents/Player/MovementState/AC_MovementStateComponent.AC_MovementStateComponent_C|GetMovementState (Variables|/Game/Blueprints/Character/BP_Player.BP_Player_C|GetMovementStateComponent (Variables|Components|GetPlayer))) "NewEnumerator2")
        (CallFunction|GroundDodge)
        (else
          (goto _label Recheck))))))

(event Custom|DodgeTick
  (bind _player (Variables|Components|GetPlayer))
  ;[1 1 1] GroundDodge
  ;;[1 1 1] Set Ground Values and Start sliding
  (bind _output_get (Variables|Default|SetElapsedTimer (+ (Utilities|Time|GetWorldDeltaSeconds) (Variables|Default|GetElapsedTimer))))
  (if (> _output_get (Variables|Editable|GetDashTime))
    (Utilities|Time|ClearandInvalidateTimerbyHandle (Variables|Default|GetDashTimerHandle))
    (CallFunction|ResetInitialValues)
    ;;[1 1 1] Reset Movement Mode
    (Default|ResettoNextState (Variables|/Game/Blueprints/Character/BP_Player.BP_Player_C|GetMovementStateComponent (Variables|Components|GetPlayer)))
    (else
      (Transformation|SetActorRotation _player (Math|Interpolation|RInterpTo (Math|Rotator|MakeRotator 0.0 0.0 (.yaw (Transformation|GetActorRotation _player))) (Math|Rotator|MakeRotator 0.0 0.0 (.yaw (Math|Rotator|MakeRotfromX (Variables|Default|GetDashVector)))) (Utilities|Time|GetWorldDeltaSeconds) 8e+01))
      (CallFunction|DetermineDashVelocity))))

(event Custom|GroundDodge
  ;[1 1 1] GroundDodge
  ;;[1 1 1] SetMovementMode and Play Montage
  (Variables|Default|SetDodgeBufferCounter 0.0)
  (Variables|/Game/Blueprints/AbilityActorComponents/Player/MovementState/AC_MovementStateComponent.AC_MovementStateComponent_C|SetMovementState (Variables|/Game/Blueprints/Character/BP_Player.BP_Player_C|GetMovementStateComponent (Variables|Components|GetPlayer)) "NewEnumerator11")
  (Animation|Montage|PlayMontage (Variables|/Script/Engine.Character|GetMesh (Variables|Components|GetPlayer)) "/Game/Assets/Characters/Leif/SKM/Leif_Animations/ANIM_Leif_Dodge_Montage.ANIM_Leif_Dodge_Montage"
    (:then
      ;;[1 1 1] Set Vector to dash to
      (Variables|Default|SetDashVector (Math|Vector|GetForwardVector (Variables|/Game/Blueprints/Character/BP_Player.BP_Player_C|GetDirectionControl (Variables|Components|GetPlayer))))
      ;;[1 1 1] Set Ground Values and Start sliding
      (CallFunction|SetGroundValuesforSlide)
      (bind _returnvalue (Utilities|Time|SetTimerbyEvent (delegate Custom|DodgeTick) (Utilities|Time|GetWorldDeltaSeconds) true))
      (Variables|Default|SetDashTimerHandle _returnvalue))))

(event EventBeginPlay
  (Utilities|IsValid (Actor|GetComponentbyClass (Components|GetOwner) "AC_DodgeComponent_C")
    (:Is%20Valid
      (bind _asbp_player (Utilities|Casting|CastToBP_Player (Components|GetOwner)))
      (Variables|Components|SetPlayer _asbp_player)
      (Variables|Default|SetInitialRotationRate (Variables|/Script/Engine.CharacterMovementComponent|GetRotationRate (Variables|/Script/Engine.Character|GetCharacterMovement (Variables|Components|GetPlayer))))
      (Variables|Default|SetInitialGroundFriction (Variables|/Script/Engine.CharacterMovementComponent|GetGroundFriction (Variables|/Script/Engine.Character|GetCharacterMovement (Variables|Components|GetPlayer)))))))

(event EventTick
  (params (DeltaSeconds :type Float%20%28single-precision%29))
  ;[1 1 1] InputBufferCountdown
  (if (not (or (Variables|Default|GetDodgePressed?) (< (Variables|Default|GetDodgeBufferCounter) 0.0)))
    (Variables|Default|SetDodgeBufferCounter (- (Variables|Default|GetDodgeBufferCounter) DeltaSeconds))))

(fn SetGroundValuesforSlide
  (bind _player (Variables|Components|GetPlayer))
  (bind _charactermovement (Variables|/Script/Engine.Character|GetCharacterMovement _player))
  (Variables|/Script/Engine.CharacterMovementComponent|SetRotationRate _charactermovement "0, 0, 0")
  (Variables|/Script/Engine.CharacterMovementComponent|SetBrakingDecelerationWalking _charactermovement 0.0)
  (Variables|/Script/Engine.CharacterMovementComponent|SetGroundFriction _charactermovement 0.0))

(fn DetermineDashVelocity
  (bind _elapsedtimer (Variables|Default|GetElapsedTimer))
  (bind _dashcurve (Variables|Editable|GetDashCurve))
  (bind _dashtime (Variables|Editable|GetDashTime))
  (bind _grounddashvelocity (Variables|Editable|GetGroundDashVelocity))
  (bind _dashvector (Variables|Default|GetDashVector))
  (bind _returnvalue (/ _elapsedtimer _dashtime))
  (bind _returnvalue_2 (Math|Curves|GetFloatValue _dashcurve _returnvalue))
  (bind _returnvalue_3 (* _returnvalue_2 _grounddashvelocity))
  (bind _returnvalue_4 (* _dashvector _returnvalue_3))
  (bind _output_get (Variables|/Script/Engine.MovementComponent|SetVelocity (Variables|/Script/Engine.Character|GetCharacterMovement (Variables|Components|GetPlayer)) (Math|Vector|MakeVector (.x _returnvalue_4) (.y _returnvalue_4) (.z (Transformation|GetVelocity (Variables|Components|GetPlayer))))))
  (Variables|/Script/Engine.CharacterMovementComponent|SetMaxWalkSpeed (Variables|/Script/Engine.Character|GetCharacterMovement (Variables|Components|GetPlayer)) (Math|Vector|VectorLength _output_get)))

(fn ResetInitialValues
  (Variables|/Script/Engine.CharacterMovementComponent|SetGroundFriction (Variables|/Script/Engine.Character|GetCharacterMovement (Variables|Components|GetPlayer)) (Variables|Default|GetInitialGroundFriction))
  (Variables|/Script/Engine.CharacterMovementComponent|SetRotationRate (Variables|/Script/Engine.Character|GetCharacterMovement (Variables|Components|GetPlayer)) (Variables|Default|GetInitialRotationRate))
  (Variables|Default|SetElapsedTimer 0.0))