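; Player actor component that runs jump and double jump for BP_Player, with coyote time and jump input buffering.
; On BeginPlay it derives launch velocities from jump heights and time to apex, then binds to the player's jump and landed events.
; Jumps use LaunchCharacter and update the shared movement state, which landing resets.
; Each tick updates timers and shapes gravity by state: lighter at apex, heavier falling, zero during certain airborne moves.
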(event Custom|StopJump
  (bind _player (Variables|Default|GetPlayer))
  (bind _player_2 (Variables|Default|GetPlayer))
  (bind _movementstatecomponent (Variables|/Game/Blueprints/Character/BP_Player.BP_Player_C|GetMovementStateComponent _player))
  (bind _charactermovement (Variables|/Script/Engine.Character|GetCharacterMovement _player_2))
  ;[1 1 1] StopJump
  (switch Utilities|FlowControl|Switch|SwitchonENUM_MovementState (Variables|/Game/Blueprints/AbilityActorComponents/Player/MovementState/AC_MovementStateComponent.AC_MovementStateComponent_C|GetMovementState (Variables|/Game/Blueprints/Character/BP_Player.BP_Player_C|GetMovementStateComponent (Variables|Default|GetPlayer)))
    (:NewEnumerator6
      _)
    (:NewEnumerator1
      _)
    (:NewEnumerator5
      _)
    (:NewEnumerator0
      _))
  (if (AI|Components|NavMovement|IsFalling _charactermovement)
    (if (<= (.z (Variables|/Script/Engine.MovementComponent|GetVelocity _charactermovement)) 0.0)
      (Variables|/Game/Blueprints/AbilityActorComponents/Player/MovementState/AC_MovementStateComponent.AC_MovementStateComponent_C|SetMovementState _movementstatecomponent "NewEnumerator0")
      (Variables|Default|SetCoyoteTimeCounter 0.0)
      (Variables|Default|GetPlayer
        (:then
          (if (> (.z (Variables|/Script/Engine.MovementComponent|GetVelocity (Variables|/Script/Engine.Character|GetCharacterMovement (Variables|Default|GetPlayer)))) (Variables|Default|GetMinJumpVelocity))
            (bind _charactermovement_2 (Variables|/Script/Engine.Character|GetCharacterMovement (Variables|Default|GetPlayer))
              (:then
                (Variables|/Script/Engine.MovementComponent|SetVelocity _charactermovement_2 (Math|Vector|MakeVector (.x (Variables|/Script/Engine.MovementComponent|GetVelocity (Variables|/Script/Engine.Character|GetCharacterMovement (Variables|Default|GetPlayer)))) (.y (Variables|/Script/Engine.MovementComponent|GetVelocity (Variables|/Script/Engine.Character|GetCharacterMovement (Variables|Default|GetPlayer)))) (Variables|Default|GetMinJumpVelocity))))
              (:else))))
        (:else)))
    (else
      (Variables|/Game/Blueprints/AbilityActorComponents/Player/MovementState/AC_MovementStateComponent.AC_MovementStateComponent_C|SetMovementState _movementstatecomponent "NewEnumerator2"))))

(event Custom|StartJump
  ;[1 1 1] StartJump
  (if (Variables|Default|GetCanDoubleJump)
    (switch Utilities|FlowControl|Switch|SwitchonENUM_MovementState (Variables|/Game/Blueprints/AbilityActorComponents/Player/MovementState/AC_MovementStateComponent.AC_MovementStateComponent_C|GetMovementState (Variables|/Game/Blueprints/Character/BP_Player.BP_Player_C|GetMovementStateComponent (Variables|Default|GetPlayer)))
      (:NewEnumerator1
        _)
      (:NewEnumerator16
        _)
      (:NewEnumerator0
        _))
    (Variables|/Game/Blueprints/AbilityActorComponents/Player/MovementState/AC_MovementStateComponent.AC_MovementStateComponent_C|SetMovementState (Variables|/Game/Blueprints/Character/BP_Player.BP_Player_C|GetMovementStateComponent (Variables|Default|GetPlayer)) "NewEnumerator5")
    (Variables|/Script/Engine.CharacterMovementComponent|SetRotationRate (Variables|/Script/Engine.Character|GetCharacterMovement (Variables|Default|GetPlayer)) (Variables|Default|GetInitialRotationRate))
    (Variables|/Script/Engine.CharacterMovementComponent|SetJumpZVelocity (Variables|/Script/Engine.Character|GetCharacterMovement (Variables|Default|GetPlayer)) (Variables|Default|GetMaxDoubleJumpVelocity))
    (bind _player (Variables|Default|GetPlayer)
      (:then
        (Character|LaunchCharacter _player (Math|Vector|MakeVector 0.0 0.0 (Variables|Default|GetMaxDoubleJumpVelocity)) false true)
        (Variables|Default|SetCanDoubleJump false))
      (:else))
    (else
      (Variables|Default|SetJumpBufferCounter (Variables|Default|GetJumpBufferTime))
      (Variables|Default|SetJumpPressed true)
      (Utilities|FlowControl|Sequence
        (:then_0
          (Utilities|InputBufferLoop (Variables|Default|GetJumpBufferCounter) :!label _label)
          (if (and (or (Utilities|Enum|Equal(Enum) (Variables|/Game/Blueprints/AbilityActorComponents/Player/MovementState/AC_MovementStateComponent.AC_MovementStateComponent_C|GetMovementState (Variables|/Game/Blueprints/Character/BP_Player.BP_Player_C|GetMovementStateComponent (Variables|Default|GetPlayer))) "NewEnumerator2") (Utilities|Enum|Equal(Enum) (Variables|/Game/Blueprints/AbilityActorComponents/Player/MovementState/AC_MovementStateComponent.AC_MovementStateComponent_C|GetMovementState (Variables|/Game/Blueprints/Character/BP_Player.BP_Player_C|GetMovementStateComponent (Variables|Default|GetPlayer))) "NewEnumerator0")) (> (Variables|Default|GetCoyoteTimeCounter) 0.0))
            (Variables|Default|SetCanJump? false)
            (Variables|Default|SetJumpBufferCounter 0.0)
            (Variables|/Game/Blueprints/AbilityActorComponents/Player/MovementState/AC_MovementStateComponent.AC_MovementStateComponent_C|SetMovementState (Variables|/Game/Blueprints/Character/BP_Player.BP_Player_C|GetMovementStateComponent (Variables|Default|GetPlayer)) "NewEnumerator1")
            (bind _charactermovement (Variables|/Script/Engine.Character|GetCharacterMovement (Variables|Default|GetPlayer))
              (:then
                (Variables|/Script/Engine.CharacterMovementComponent|SetJumpZVelocity _charactermovement (Variables|Default|GetMaxJumpVelocity))
                (bind _player_2 (Variables|Default|GetPlayer)
                  (:then
                    (Character|LaunchCharacter _player_2 (Math|Vector|MakeVector 0.0 0.0 (Variables|Default|GetMaxJumpVelocity)) false true)
                    (Variables|Default|SetCanDoubleJump true)
                    (Default|JumpSqueeze (Variables|Default|GetPlayer)))
                  (:else)))
              (:else))
            (else
              (goto _label Recheck))))
        (:then_1
          (Utilities|FlowControl|DelayUntilNextTick)
          (Variables|Default|SetJumpPressed false))))))

(event Custom|Land
  (params (Hit :type Hit%20Result%20Structure%20%28by%20ref%29))
  (bind _player (Variables|Default|GetPlayer))
  (bind _player_2 (Variables|Default|GetPlayer))
  (bind _movementstatecomponent (Variables|/Game/Blueprints/Character/BP_Player.BP_Player_C|GetMovementStateComponent _player))
  (bind _charactermovement (Variables|/Script/Engine.Character|GetCharacterMovement _player_2))
  ;[1 1 1] Landed
  (Variables|/Script/Engine.CharacterMovementComponent|SetGravityScale (Variables|/Script/Engine.Character|GetCharacterMovement (Variables|Default|GetPlayer)) 2.8)
  (Variables|Default|SetCanJump? true)
  (Variables|Default|SetCanDoubleJump false)
  (Variables|Default|SetCoyoteTimeCounter (Variables|Default|GetCoyoteTime))
  (Variables|Default|SetDoubleJumped false)
  (switch Utilities|FlowControl|Switch|SwitchonENUM_MovementState (Variables|/Game/Blueprints/AbilityActorComponents/Player/MovementState/AC_MovementStateComponent.AC_MovementStateComponent_C|GetMovementState _movementstatecomponent)
    (:NewEnumerator1
      _)
    (:NewEnumerator5
      _)
    (:NewEnumerator16
      _)
    (:NewEnumerator0
      _)
    (:NewEnumerator13
      _))
  (Variables|/Game/Blueprints/AbilityActorComponents/Player/MovementState/AC_MovementStateComponent.AC_MovementStateComponent_C|SetMovementState _movementstatecomponent "NewEnumerator2")
  (Default|LandSqueeze (Variables|Default|GetPlayer))
  (Variables|/Script/Engine.CharacterMovementComponent|SetGravityScale (Variables|/Script/Engine.Character|GetCharacterMovement (Variables|Default|GetPlayer)) (Variables|Default|GetGravityScale))
  (Variables|/Script/Engine.CharacterMovementComponent|SetRotationRate _charactermovement (Variables|Default|GetInitialRotationRate))
  (Variables|/Script/Engine.CharacterMovementComponent|SetAirControl _charactermovement 1.5e+04))

(event EventBeginPlay
  (bind _returnvalue (Components|GetOwner))
  ;[1 1 1] Initialize
  (Utilities|IsValid (Actor|GetComponentbyClass _returnvalue "AC_JumpComponent_C")
    (:Is%20Valid
      (bind _asbp_player (Utilities|Casting|CastToBP_Player _returnvalue))
      (bind _output_get (Variables|Default|SetPlayer _asbp_player))
      (CallFunction|SetJumpVariables)
      (EventDispatchers|BindEventtoStartJumpCall _output_get (EventDispatchers|CreateEvent :!event Custom|StartJump))
      (EventDispatchers|BindEventtoStopJumpCall _output_get (EventDispatchers|CreateEvent :!event Custom|StopJump))
      (EventDispatchers|BindEventtoLandedDelegate _output_get (EventDispatchers|CreateEvent :!event Custom|Land))
      (Variables|Default|SetInitialRotationRate (Variables|/Script/Engine.CharacterMovementComponent|GetRotationRate (Variables|/Script/Engine.Character|GetCharacterMovement (Variables|Default|GetPlayer)))))))

(event EventTick
  (params (DeltaSeconds :type Float%20%28single-precision%29))
  ;[1 1 1] Tick
  (Variables|Default|SetDeltaSeconds DeltaSeconds)
  (CallFunction|SetCoyoteandJumpBufferTime)
  (CallFunction|HandlyGravity))

(fn SetCoyoteandJumpBufferTime
  (if (or (Variables|Default|GetJumpPressed) (< (Variables|Default|GetJumpBufferCounter) 0.0))
    (if (AI|Components|NavMovement|IsFalling (Variables|/Script/Engine.Character|GetCharacterMovement (Variables|Default|GetPlayer)))
      (Variables|Default|SetCoyoteTimeCounter (|(A-B) (Variables|Default|GetCoyoteTimeCounter) (Variables|Default|GetDeltaSeconds))))
    (else
      (Variables|Default|SetJumpBufferCounter (|(A-B) (Variables|Default|GetJumpBufferCounter) (Variables|Default|GetDeltaSeconds))))))

(fn SetJumpVariables
  (bind _player (Variables|Default|GetPlayer))
  (bind _player_2 (Variables|Default|GetPlayer))
  (bind _charactermovement (Variables|/Script/Engine.Character|GetCharacterMovement _player))
  (bind _charactermovement_2 (Variables|/Script/Engine.Character|GetCharacterMovement _player_2))
  (Variables|/Script/Engine.CharacterMovementComponent|SetGravityScale _charactermovement (/ (* (Variables|Default|GetMaxJumpHeight) 2.0) (Math|Float|Power (Variables|Default|GetTimeToJumpApex) 2.0)))
  (Variables|Default|SetMaxJumpVelocity (|(A*{91AF9007-4FA9-6931-C4C1-8A966F925EE7}) (Variables|/Script/Engine.CharacterMovementComponent|GetGravityScale _charactermovement)))
  (Variables|Default|SetMinJumpVelocity (|(sqrt(((2*A)*{8212DF45-4C46-578B-C0D7-A98199EC0D09}))) (Variables|/Script/Engine.CharacterMovementComponent|GetGravityScale (Variables|/Script/Engine.Character|GetCharacterMovement (Variables|Default|GetPlayer)))))
  (Variables|/Script/Engine.CharacterMovementComponent|SetGravityScale _charactermovement_2 (|(({B5ECD4AB-49F3-A052-BA61-D096EEECA631}*2)/(Pow({91AF9007-4FA9-6931-C4C1-8A966F925EE7},2)))))
  (Variables|Default|SetMaxDoubleJumpVelocity (|(A*{91AF9007-4FA9-6931-C4C1-8A966F925EE7}) (Variables|/Script/Engine.CharacterMovementComponent|GetGravityScale _charactermovement_2)))
  (Variables|Default|SetCoyoteTimeCounter (Variables|Default|GetCoyoteTime))
  (Variables|/Script/Engine.CharacterMovementComponent|SetGravityScale (Variables|/Script/Engine.Character|GetCharacterMovement (Variables|Default|GetPlayer)) (Variables|Default|GetGravityScale)))

(fn HandlyGravity
  (switch Utilities|FlowControl|Switch|SwitchonENUM_MovementState (Variables|/Game/Blueprints/AbilityActorComponents/Player/MovementState/AC_MovementStateComponent.AC_MovementStateComponent_C|GetMovementState (Variables|/Game/Blueprints/Character/BP_Player.BP_Player_C|GetMovementStateComponent (Variables|Default|GetPlayer)))
    (:NewEnumerator2
      (if (< (Math|Float|Absolute(Float) (.z (Variables|/Script/Engine.MovementComponent|GetVelocity (Variables|/Script/Engine.Character|GetCharacterMovement (Variables|Default|GetPlayer))))) (Variables|Default|GetApexThreshold)) :!label _label
        ;[1 1 1] Set Gravity to low number for short airtime
        (Variables|/Script/Engine.CharacterMovementComponent|SetGravityScale (Variables|/Script/Engine.Character|GetCharacterMovement (Variables|Default|GetPlayer)) 2.0)
        (else
          ;[1 1 1] Higher Gravity when player falls
          (if (< (.z (Variables|/Script/Engine.MovementComponent|GetVelocity (Variables|/Script/Engine.Character|GetCharacterMovement (Variables|Default|GetPlayer)))) 0.0) :!label _label_2
            (Variables|/Script/Engine.CharacterMovementComponent|SetGravityScale (Variables|/Script/Engine.Character|GetCharacterMovement (Variables|Default|GetPlayer)) (* (Variables|Default|GetGravityScale) (Variables|Default|GetGravityFallMultiplier)))
            (switch Utilities|FlowControl|Switch|SwitchonENUM_MovementState (Variables|/Game/Blueprints/AbilityActorComponents/Player/MovementState/AC_MovementStateComponent.AC_MovementStateComponent_C|GetMovementState (Variables|/Game/Blueprints/Character/BP_Player.BP_Player_C|GetMovementStateComponent (Variables|Default|GetPlayer)))
              (:NewEnumerator1
                _)
              (:NewEnumerator5
                _))
            (Variables|/Game/Blueprints/AbilityActorComponents/Player/MovementState/AC_MovementStateComponent.AC_MovementStateComponent_C|SetMovementState (Variables|/Game/Blueprints/Character/BP_Player.BP_Player_C|GetMovementStateComponent (Variables|Default|GetPlayer)) "NewEnumerator0")
            (else
              (Variables|/Script/Engine.CharacterMovementComponent|SetGravityScale (Variables|/Script/Engine.Character|GetCharacterMovement (Variables|Default|GetPlayer)) (Variables|Default|GetGravityScale)))))))
    (:NewEnumerator1
      (goto _label))
    (:NewEnumerator5
      (goto _label))
    (:NewEnumerator16
      (if (AI|Components|NavMovement|IsFalling (Variables|/Script/Engine.Character|GetCharacterMovement (Variables|Default|GetPlayer))) :!label _label_3
        (Variables|/Script/Engine.CharacterMovementComponent|SetGravityScale (Variables|/Script/Engine.Character|GetCharacterMovement (Variables|Default|GetPlayer)) 0.0)))
    (:NewEnumerator0
      (goto _label_2))
    (:NewEnumerator11
      (goto _label_2))
    (:NewEnumerator20
      (goto _label_3))
    (:NewEnumerator17
      (goto _label_2))
    (:NewEnumerator18
      (goto _label_3))
    (:NewEnumerator19
      (goto _label_3))))