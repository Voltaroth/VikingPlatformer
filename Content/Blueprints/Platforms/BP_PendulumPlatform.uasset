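; Pendulum platform that endlessly swings its root around the roll axis while keeping its pitch and yaw.
; A timeline scaled by RotateTime supplies the roll angle, using a mirrored track when Reversed is set, and restarts itself on finish.
; While the player overlaps the Box, a looping timer at roughly frame interval nudges the character back and forth with swept moves, forcing movement updates with no intended net displacement.
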(event OnComponentBeginOverlap(Box)
  (params (OverlappedComponent :type Primitive%20Component%20Object%20Reference) (OtherActor :type Actor%20Object%20Reference) (OtherComp :type Primitive%20Component%20Object%20Reference) (OtherBodyIndex :type Integer) (bFromSweep :type Boolean) (SweepResult :type Hit%20Result%20Structure%20%28by%20ref%29))
  (if (== OtherActor (Game|GetPlayerCharacter 0))
    (bind _returnvalue (Utilities|Time|SetTimerbyEvent (delegate Custom|UpdatePlayerLocation) (Utilities|Time|GetWorldDeltaSeconds) true))
    (Variables|Default|SetUpdatePlayerHandle _returnvalue)))

(event OnComponentEndOverlap(Box)
  (params (OverlappedComponent :type Primitive%20Component%20Object%20Reference) (OtherActor :type Actor%20Object%20Reference) (OtherComp :type Primitive%20Component%20Object%20Reference) (OtherBodyIndex :type Integer))
  (if (== OtherActor (Game|GetPlayerCharacter 0))
    (Utilities|Time|ClearandInvalidateTimerbyHandle (Variables|Default|GetUpdatePlayerHandle))))

(event Custom|Rotate
  (Variables|Default|SetInitialRotation (Transformation|GetWorldRotation (Variables|Components|GetRoot)))
  (bind (_direction _angles _anglesreversed) (Timeline|Rotation PlayFromStart)
    (:Update
      (Transformation|SetWorldRotation (Variables|Components|GetRoot) (Math|Rotator|Lerp(Rotator) (Variables|Default|GetInitialRotation) (Math|Rotator|MakeRotator (select (Variables|Default|GetReversed?) _anglesreversed _angles) (.pitch (Variables|Default|GetInitialRotation)) (.yaw (Variables|Default|GetInitialRotation))) 1.0) false false))
    (:Finished
      (CallFunction|Rotate))))

(event Custom|UpdatePlayerLocation
  (bind _returnvalue (Game|GetPlayerCharacter 0))
  (bind _returnvalue_2 (Transformation|GetActorRotation _returnvalue))
  (bind _charactermovement (Variables|/Script/Engine.Character|GetCharacterMovement _returnvalue))
  (Class|MovementComponent|MoveUpdatedComponent _charactermovement "0.000000,1.000000,0.000000" _returnvalue_2 true)
  (Class|MovementComponent|MoveUpdatedComponent _charactermovement "0.000000,-1.000000,0.000000" _returnvalue_2 true))

(event EventBeginPlay
  (Components|Timeline|SetPlayRate (Variables|Default|GetRotation) (/ 1.0 (Variables|Default|GetRotateTime)))
  (CallFunction|Rotate))

(fn ConstructionScript)