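; BP_DashableWall is a laser wall that the player can pass through only while dashing.
; When the player character enters the Box trigger, it reads the MovementStateComponent and disables collision on Lasers if the state is Is Dashing.
; The dash state is checked only at the moment overlap begins.
; Leaving the Box restores query and physics collision on Lasers after a short delay.
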(event OnComponentBeginOverlap(Box)
  (params (OverlappedComponent :type Primitive%20Component%20Object%20Reference) (OtherActor :type Actor%20Object%20Reference) (OtherComp :type Primitive%20Component%20Object%20Reference) (OtherBodyIndex :type Integer) (bFromSweep :type Boolean) (SweepResult :type Hit%20Result%20Structure%20%28by%20ref%29))
  (if (== OtherActor (Game|GetPlayerCharacter 0))
    (bind _asbp_player (Utilities|Casting|CastToBP_Player OtherActor))
    (Variables|Default|SetPlayer _asbp_player)
    (switch Utilities|FlowControl|Switch|SwitchonENUM_MovementState (Variables|/Game/Blueprints/ActorComponents/Player/MovementState/AC_MovementStateComponent.AC_MovementStateComponent_C|GetMovementState (Variables|/Game/Blueprints/Character/BP_Player.BP_Player_C|GetMovementStateComponent (Variables|Default|GetPlayer)))
      (:NewEnumerator11
        (Collision|SetCollisionEnabled (Variables|Default|GetLasers) "NoCollision")))))

(event OnComponentEndOverlap(Box)
  (params (OverlappedComponent :type Primitive%20Component%20Object%20Reference) (OtherActor :type Actor%20Object%20Reference) (OtherComp :type Primitive%20Component%20Object%20Reference) (OtherBodyIndex :type Integer))
  (if (== OtherActor (Game|GetPlayerCharacter 0))
    (bind _asbp_player (Utilities|Casting|CastToBP_Player OtherActor))
    (Variables|Default|SetPlayer _asbp_player)
    (Utilities|FlowControl|Delay 0.2)
    (Collision|SetCollisionEnabled (Variables|Default|GetLasers) "QueryAndPhysics")))

(event EventBeginPlay)

(event Collision|EventActorBeginOverlap
  (params (OtherActor :type Actor%20Object%20Reference)))

(event EventTick
  (params (DeltaSeconds :type Float%20%28single-precision%29)))

(fn ConstructionScript)