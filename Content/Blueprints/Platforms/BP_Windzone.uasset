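; Wind zone actor that pushes the player along the actor's up vector while they overlap its capsule.
; Overlap sets a flag that makes Tick apply a velocity-change impulse, not scaled by delta time, and zero the player's ground friction.
; On exit, a looping timer interpolates friction back up to a hardcoded target, clearing itself when reached or on re-entry.
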(event OnComponentBeginOverlap(Capsule)
  (params (OverlappedComponent :type Primitive%20Component%20Object%20Reference) (OtherActor :type Actor%20Object%20Reference) (OtherComp :type Primitive%20Component%20Object%20Reference) (OtherBodyIndex :type Integer) (bFromSweep :type Boolean) (SweepResult :type Hit%20Result%20Structure%20%28by%20ref%29))
  (if (== OtherActor (Variables|Default|GetPlayer))
    (Variables|Default|SetAddForce? true)
    (Utilities|Time|ClearandInvalidateTimerbyHandle (Variables|Default|GetGroundFrictionTimerHandle))))

(event OnComponentEndOverlap(Capsule)
  (params (OverlappedComponent :type Primitive%20Component%20Object%20Reference) (OtherActor :type Actor%20Object%20Reference) (OtherComp :type Primitive%20Component%20Object%20Reference) (OtherBodyIndex :type Integer))
  (if (== OtherActor (Variables|Default|GetPlayer))
    (Variables|Default|SetAddForce? false)
    (bind _returnvalue (Utilities|Time|SetTimerbyEvent (delegate Custom|GroundFrictionTick) (Utilities|Time|GetWorldDeltaSeconds) true))
    (Variables|Default|SetGroundFrictionTimerHandle _returnvalue)))

(event Custom|GroundFrictionTick
  (Variables|/Script/Engine.CharacterMovementComponent|SetGroundFriction (Variables|/Script/Engine.Character|GetCharacterMovement (Variables|Default|GetPlayer)) (Math|Interpolation|FInterpTo (Variables|/Script/Engine.CharacterMovementComponent|GetGroundFriction (Variables|/Script/Engine.Character|GetCharacterMovement (Variables|Default|GetPlayer))) 5e+01 (Utilities|Time|GetWorldDeltaSeconds) 2.0))
  (if (Math|Float|NearlyEqual(Float) (Variables|/Script/Engine.CharacterMovementComponent|GetGroundFriction (Variables|/Script/Engine.Character|GetCharacterMovement (Variables|Default|GetPlayer))) 5e+01 0.0)
    (Utilities|Time|ClearandInvalidateTimerbyHandle (Variables|Default|GetGroundFrictionTimerHandle))))

(event EventBeginPlay
  (bind _asbp_player (Utilities|Casting|CastToBP_Player (Game|GetPlayerCharacter 0)))
  (Variables|Default|SetPlayer _asbp_player))

(event EventTick
  (params (DeltaSeconds :type Float%20%28single-precision%29))
  (bind _player (Variables|Default|GetPlayer))
  (bind _charactermovement (Variables|/Script/Engine.Character|GetCharacterMovement _player))
  (if (Variables|Default|GetAddForce?)
    (Physics|AddImpulse _charactermovement (* (Transformation|GetActorUpVector) (Variables|Default|GetForward%20Force)) true)
    (Variables|/Script/Engine.CharacterMovementComponent|SetGroundFriction _charactermovement 0.0)))

(fn ConstructionScript)