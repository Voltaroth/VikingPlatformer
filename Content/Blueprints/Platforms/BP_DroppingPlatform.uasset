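; A platform that falls away shortly after the player character steps on it, then respawns.
; A Box overlap by player 0 briefly waits, then turns on physics so the Cube drops, and later stops it, hides it and disables its collision.
; After a longer delay the Cube returns to the world location and rotation saved at BeginPlay, with visibility and collision restored.
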(event OnComponentBeginOverlap(Box)
  (params (OverlappedComponent :type Primitive%20Component%20Object%20Reference) (OtherActor :type Actor%20Object%20Reference) (OtherComp :type Primitive%20Component%20Object%20Reference) (OtherBodyIndex :type Integer) (bFromSweep :type Boolean) (SweepResult :type Hit%20Result%20Structure%20%28by%20ref%29))
  (bind _cube (Variables|Default|GetCube))
  (bind _cube_2 (Variables|Default|GetCube))
  (if (== OtherActor (Game|GetPlayerCharacter 0))
    (Utilities|FlowControl|Delay 0.2)
    (Physics|SetSimulatePhysics (Variables|Default|GetCube) true)
    (Utilities|FlowControl|Delay 1.0)
    (Physics|SetSimulatePhysics (Variables|Default|GetCube) false)
    (Rendering|SetVisibility _cube_2 false false)
    (Collision|SetCollisionEnabled _cube_2 "NoCollision")
    (Utilities|FlowControl|Delay 5.0)
    (Transformation|SetWorldLocation _cube (Variables|Default|GetInitialLocation) false false)
    (Transformation|SetWorldRotation _cube (Variables|Default|GetInitialRotation) false false)
    (Rendering|SetVisibility _cube true false)
    (Collision|SetCollisionEnabled _cube "QueryAndPhysics")))

(event EventBeginPlay
  (bind _cube (Variables|Default|GetCube))
  (Variables|Default|SetInitialLocation (Transformation|GetWorldLocation _cube))
  (Variables|Default|SetInitialRotation (Transformation|GetWorldRotation _cube)))

(event Collision|EventActorBeginOverlap
  (params (OtherActor :type Actor%20Object%20Reference)))

(event EventTick
  (params (DeltaSeconds :type Float%20%28single-precision%29)))

(fn ConstructionScript)