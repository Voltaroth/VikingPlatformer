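; BP_Seesaw is a physics-driven seesaw platform that reacts to the player and returns to its starting rotation.
; When the player character enters the Box trigger, the Cube starts simulating physics and any running Reset timeline stops.
; When the player leaves, the Reset timeline plays, switching physics off and interpolating the Cube back to the rotation saved at BeginPlay with RInterpTo.
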(event OnComponentEndOverlap(Box)
  (params (OverlappedComponent :type Primitive%20Component%20Object%20Reference) (OtherActor :type Actor%20Object%20Reference) (OtherComp :type Primitive%20Component%20Object%20Reference) (OtherBodyIndex :type Integer))
  (if (== OtherActor (Game|GetPlayerCharacter 0))
    (Timeline|Reset PlayFromStart
      (:Update
        (Transformation|SetWorldRotation (Variables|Default|GetCube) (Math|Interpolation|RInterpTo (Transformation|GetWorldRotation (Variables|Default|GetCube)) (Variables|Default|GetInitialRotation) (Utilities|Time|GetWorldDeltaSeconds) 3.0) false false)
        (Physics|SetSimulatePhysics (Variables|Default|GetCube) false)))))

(event OnComponentBeginOverlap(Box)
  (params (OverlappedComponent :type Primitive%20Component%20Object%20Reference) (OtherActor :type Actor%20Object%20Reference) (OtherComp :type Primitive%20Component%20Object%20Reference) (OtherBodyIndex :type Integer) (bFromSweep :type Boolean) (SweepResult :type Hit%20Result%20Structure%20%28by%20ref%29))
  (if (== OtherActor (Game|GetPlayerCharacter 0))
    (Physics|SetSimulatePhysics (Variables|Default|GetCube) true)
    (Timeline|Reset Stop
      (:Update
        (Transformation|SetWorldRotation (Variables|Default|GetCube) (Math|Interpolation|RInterpTo (Transformation|GetWorldRotation (Variables|Default|GetCube)) (Variables|Default|GetInitialRotation) (Utilities|Time|GetWorldDeltaSeconds) 3.0) false false)
        (Physics|SetSimulatePhysics (Variables|Default|GetCube) false)))))

(event EventBeginPlay
  (Variables|Default|SetInitialRotation (Transformation|GetWorldRotation (Variables|Default|GetCube))))

(fn ConstructionScript)