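; BP_Platform is a platform that rotates, moves along a spline, or does both, depending on its State.
; Timelines drive repeated roll or yaw steps and back-and-forth spline travel, with configurable durations and pauses.
; While the player overlaps its box, a looping timer makes tiny opposing swept moves on the character.
; The timer also matches the player's height to the platform during ledge grabs.
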(event OnComponentBeginOverlap(Box)
  (params (OverlappedComponent :type Primitive%20Component%20Object%20Reference) (OtherActor :type Actor%20Object%20Reference) (OtherComp :type Primitive%20Component%20Object%20Reference) (OtherBodyIndex :type Integer) (bFromSweep :type Boolean) (SweepResult :type Hit%20Result%20Structure%20%28by%20ref%29))
  (bind _returnvalue (Game|GetPlayerCharacter 0))
  (if (== OtherActor _returnvalue)
    (bind _asbp_player (Utilities|Casting|CastToBP_Player _returnvalue))
    (Variables|Default|SetPlayer _asbp_player)
    (bind _returnvalue_2 (Utilities|Time|SetTimerbyEvent (delegate Custom|UpdatePlayerLocation) (Utilities|Time|GetWorldDeltaSeconds) true))
    (Variables|Default|SetUpdatePlayerHandle _returnvalue_2)))

(event OnComponentEndOverlap(Box)
  (params (OverlappedComponent :type Primitive%20Component%20Object%20Reference) (OtherActor :type Actor%20Object%20Reference) (OtherComp :type Primitive%20Component%20Object%20Reference) (OtherBodyIndex :type Integer))
  (if (== OtherActor (Game|GetPlayerCharacter 0))
    (Utilities|Time|ClearandInvalidateTimerbyHandle (Variables|Default|GetUpdatePlayerHandle))))

(event Custom|Rotate
  (|HandleRotation))

(event Custom|Move
  (|HandleMovement))

(event Custom|UpdatePlayerLocation
  (bind _returnvalue (Game|GetPlayerCharacter 0))
  (bind _returnvalue_2 (Game|GetPlayerCharacter 0))
  (bind _returnvalue_3 (Transformation|GetActorLocation _returnvalue))
  (bind _returnvalue_4 (Transformation|GetActorRotation _returnvalue_2))
  (bind _charactermovement (Variables|/Script/Engine.Character|GetCharacterMovement _returnvalue_2))
  (Class|MovementComponent|MoveUpdatedComponent _charactermovement "0.000000,1.000000,0.000000" _returnvalue_4 true)
  (Class|MovementComponent|MoveUpdatedComponent _charactermovement "0.000000,-1.000000,0.000000" _returnvalue_4 true)
  (switch Utilities|FlowControl|Switch|SwitchonENUM_MovementState (Variables|/Game/Blueprints/AbilityActorComponents/Player/MovementState/AC_MovementStateComponent.AC_MovementStateComponent_C|GetMovementState (Variables|/Game/Blueprints/Character/BP_Player.BP_Player_C|GetMovementStateComponent (Variables|Default|GetPlayer)))
    (:NewEnumerator13
      (Transformation|SetActorLocation _returnvalue (Math|Vector|MakeVector (.x _returnvalue_3) (.y _returnvalue_3) (.z (Transformation|GetWorldLocation (Variables|Default|GetPlatform)))) false false))))

(event EventTick
  (params (DeltaSeconds :type Float%20%28single-precision%29)))

(event EventBeginPlay
  (Components|Timeline|SetPlayRate (Variables|Default|GetRotationTimeline) (/ 1.0 (Variables|Default|GetRotateTime)))
  (Components|Timeline|SetPlayRate (Variables|Default|GetMovementTimeline) (/ 1.0 (Variables|Default|GetMovementTime)))
  (switch Utilities|FlowControl|Switch|SwitchonENUM_PlatformStates (Variables|Default|GetState)
    (:NewEnumerator0
      (CallFunction|Rotate))
    (:NewEnumerator1
      (CallFunction|Move))
    (:NewEnumerator2
      (CallFunction|Rotate)
      (CallFunction|Move))))

(fn ConstructionScript)