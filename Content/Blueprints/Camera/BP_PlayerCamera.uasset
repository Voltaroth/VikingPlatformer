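; Standalone third-person player camera actor that becomes the view target and follows the player, with aiming and lock-on target states.
; Tick removes roll, interpolates the spring arm toward an offset that holds its height within a screen-space zone unless ground rises, then turns the camera toward the player.
; While the player runs without camera input, arm yaw auto-rotates by movement direction or toward the locked target.
; Timelines blend arm length and socket offset for aiming.
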(event Custom|StartAim
  ;[1 1 1] Aim
  (Utilities|FlowControl|Sequence
    (:then_0
      ;[1 1 1] StopAim
      (bind _alpha (Timeline|UnAimTimeline Stop)
        (:Update
          (Variables|Default|SetUnAimAlpha _alpha)
          (Variables|/Script/Engine.SpringArmComponent|SetSocketOffset (Variables|Default|GetSpringArm) (Math|Vector|Lerp(Vector) (Variables|/Script/Engine.SpringArmComponent|GetSocketOffset (Variables|Default|GetSpringArm)) (Variables|Default|GetInitialSocketOffset) (Variables|Default|GetUnAimAlpha)))
          (Variables|/Script/Engine.SpringArmComponent|SetTargetArmLength (Variables|Default|GetSpringArm) (Math|Float|Lerp (Variables|/Script/Engine.SpringArmComponent|GetTargetArmLength (Variables|Default|GetSpringArm)) (Variables|Editable|GetXOffset) (Variables|Default|GetUnAimAlpha))))
        (:Finished
          (Variables|Default|SetWasAiming? false))))
    (:then_1
      (Variables|Default|SetIsAiming? true)
      (Variables|Default|SetCameraStates "NewEnumerator3")
      (Variables|/Script/Engine.SpringArmComponent|SetbEnableCameraLag (Variables|Default|GetSpringArm) false)
      (Components|Timeline|SetPlayRate (Variables|Default|GetAimTimeline) 2.0)
      (bind _alpha_2 (Timeline|AimTimeline PlayFromStart)
        (:Update
          (Variables|Default|SetAimAlpha _alpha_2)
          (Variables|/Script/Engine.SpringArmComponent|SetSocketOffset (Variables|Default|GetSpringArm) (Math|Vector|Lerp(Vector) (Variables|/Script/Engine.SpringArmComponent|GetSocketOffset (Variables|Default|GetSpringArm)) (Variables|Default|GetSocketAimOffset) (Variables|Default|GetAimAlpha)))
          (Variables|/Script/Engine.SpringArmComponent|SetTargetArmLength (Variables|Default|GetSpringArm) (Math|Float|Lerp (Variables|/Script/Engine.SpringArmComponent|GetTargetArmLength (Variables|Default|GetSpringArm)) (Variables|Default|GetAimTargetArmLength) (Variables|Default|GetAimAlpha))))))))

(event Custom|Target
  (params (LockedOnTarget :type Actor%20Object%20Reference))
  (Utilities|IsValid LockedOnTarget
    (:Is%20Valid
      (Variables|Default|SetLockedOnTarget LockedOnTarget)
      (Variables|Default|SetCameraStates "NewEnumerator4")
      (CallFunction|StartTargetTick))))

(event Custom|StopAim
  ;[1 1 1] StopAim
  (Variables|Default|SetWasAiming? true)
  (Utilities|FlowControl|Sequence
    (:then_0
      ;[1 1 1] Aim
      (bind _alpha (Timeline|AimTimeline Stop)
        (:Update
          (Variables|Default|SetAimAlpha _alpha)
          (Variables|/Script/Engine.SpringArmComponent|SetSocketOffset (Variables|Default|GetSpringArm) (Math|Vector|Lerp(Vector) (Variables|/Script/Engine.SpringArmComponent|GetSocketOffset (Variables|Default|GetSpringArm)) (Variables|Default|GetSocketAimOffset) (Variables|Default|GetAimAlpha)))
          (Variables|/Script/Engine.SpringArmComponent|SetTargetArmLength (Variables|Default|GetSpringArm) (Math|Float|Lerp (Variables|/Script/Engine.SpringArmComponent|GetTargetArmLength (Variables|Default|GetSpringArm)) (Variables|Default|GetAimTargetArmLength) (Variables|Default|GetAimAlpha))))))
    (:then_1
      (Variables|Default|SetCameraStates "NewEnumerator1")
      (Variables|/Script/Engine.SpringArmComponent|SetbEnableCameraLag (Variables|Default|GetSpringArm) false)
      (Variables|Default|SetIsAiming? false)
      (Components|Timeline|SetPlayRate (Variables|Default|GetUnAimTimeline) 1.0)
      (bind _alpha_2 (Timeline|UnAimTimeline PlayFromStart)
        (:Update
          (Variables|Default|SetUnAimAlpha _alpha_2)
          (Variables|/Script/Engine.SpringArmComponent|SetSocketOffset (Variables|Default|GetSpringArm) (Math|Vector|Lerp(Vector) (Variables|/Script/Engine.SpringArmComponent|GetSocketOffset (Variables|Default|GetSpringArm)) (Variables|Default|GetInitialSocketOffset) (Variables|Default|GetUnAimAlpha)))
          (Variables|/Script/Engine.SpringArmComponent|SetTargetArmLength (Variables|Default|GetSpringArm) (Math|Float|Lerp (Variables|/Script/Engine.SpringArmComponent|GetTargetArmLength (Variables|Default|GetSpringArm)) (Variables|Editable|GetXOffset) (Variables|Default|GetUnAimAlpha))))
        (:Finished
          (Variables|Default|SetWasAiming? false))))))

(event Custom|StopTarget
  (Utilities|Time|ClearandInvalidateTimerbyHandle (Variables|Default|GetTargetTickTimerHandle))
  (Variables|Default|SetCameraStates "NewEnumerator1")
  (Variables|Default|SetLockedOnTarget 0))

(event Custom|SwitchTarget
  (params (NewLockedOnTarget :type Actor%20Object%20Reference))
  (Utilities|IsValid NewLockedOnTarget
    (:Is%20Valid
      (Variables|Default|SetLockedOnTarget NewLockedOnTarget)
      (CallFunction|StartTargetTick))))

(event Custom|TargetTick
  (Variables|Default|SetLockedOnTargetLocation (Transformation|GetActorLocation (Variables|Default|GetLockedOnTarget))))

(event Custom|StartTargetTick
  (bind _returnvalue (Utilities|Time|SetTimerbyEvent (delegate Custom|TargetTick) (Utilities|Time|GetWorldDeltaSeconds)))
  (Variables|Default|SetTargetTickTimerHandle _returnvalue))

(event EventBeginPlay
  (bind _asbp_player (Utilities|Casting|CastToBP_Player (Game|GetPlayerCharacter 0)))
  (bind _output_get (Variables|Components|SetPlayer _asbp_player))
  (Transformation|SetWorldRotation (Variables|Default|GetSpringArm) (Transformation|GetActorRotation _output_get) false false)
  (Game|Player|SetViewTargetwithBlend (Game|GetPlayerController 0) self 0.0 "VTBlend_Linear" 0.0 false)
  (Variables|Default|SetInitialSocketOffset (Variables|/Script/Engine.SpringArmComponent|GetSocketOffset (Variables|Default|GetSpringArm))))

(event Custom|AllowSpringArmRotationAfterDelay
  (Utilities|FlowControl|RetriggerableDelay 0.2)
  (Variables|Default|SetAllowSpringArmRotation true)
  (Utilities|FlowControl|DoOnce false) ; enters at Reset
)

(event EventTick
  (params (DeltaSeconds :type Float%20%28single-precision%29))
  (bind _playercamera (Variables|Default|GetPlayerCamera))
  (bind _returnvalue (Transformation|GetWorldRotation _playercamera))
  ;[1 1 1] Prevent Camera from Rolling
  (Variables|Private|SetDelta%20Seconds DeltaSeconds)
  (Transformation|SetWorldRotation _playercamera (Math|Rotator|MakeRotator 0.0 (.pitch _returnvalue) (.yaw _returnvalue)) false false)
  (bind _calculatedcharacteroffset (CallFunction|CalculateOffsetLocation))
  (CallFunction|SmoothLocation _calculatedcharacteroffset)
  (switch Utilities|FlowControl|Switch|SwitchonENUM_CameraStates (Variables|Default|GetCameraStates)
    (:NewEnumerator0
      _)
    (:NewEnumerator1
      _)
    (:NewEnumerator2
      _)
    (:NewEnumerator4
      _))
  (CallFunction|SetSpringArmRotation)
  (CallFunction|LookatTarget))

(fn ConstructionScript
  (Variables|/Script/Engine.SpringArmComponent|SetTargetArmLength (Variables|Default|GetSpringArm) (Variables|Editable|GetXOffset)))

(fn SmoothLocation
  (params (TargetActorLocation :type Vector))
  (bind _player (Variables|Components|GetPlayer))
  (bind _lookatoffset (Variables|Editable|GetLookAtOffset))
  (bind _isaiming_ (Variables|Default|GetIsAiming?))
  (bind _returnvalue (Transformation|GetActorLocation _player))
  (bind _returnvalue_2 (+ _returnvalue _lookatoffset))
  (bind _returnvalue_3 (Math|Vector|SelectVector _returnvalue_2 TargetActorLocation _isaiming_))
  (Transformation|SetWorldLocation (Variables|Default|GetSpringArm) (Math|Vector|MakeVector (Math|Interpolation|FInterpTo (.x (Transformation|GetWorldLocation (Variables|Default|GetSpringArm))) (.x _returnvalue_3) (Variables|Private|GetDelta%20Seconds) (Math|Float|SelectFloat (Variables|Default|GetCamSmoothDampTimeAiming) (Variables|Editable|GetCamSmoothDampTimeHorizontal) (Variables|Default|GetIsAiming?))) (Math|Interpolation|FInterpTo (.y (Transformation|GetWorldLocation (Variables|Default|GetSpringArm))) (.y _returnvalue_3) (Variables|Private|GetDelta%20Seconds) (Math|Float|SelectFloat (Variables|Default|GetCamSmoothDampTimeAiming) (Variables|Editable|GetCamSmoothDampTimeHorizontal) (Variables|Default|GetIsAiming?))) (Math|Interpolation|FInterpTo (.z (Transformation|GetWorldLocation (Variables|Default|GetSpringArm))) (.z _returnvalue_3) (Variables|Private|GetDelta%20Seconds) (Math|Float|SelectFloat (Variables|Default|GetCamSmoothDampTimeAiming) (Variables|Editable|GetCamSmoothDampTimeVertical) (Variables|Default|GetIsAiming?)))) false false))

(fn SetSpringArmRotation
  (bind _playercamera (Variables|Default|GetPlayerCamera))
  (bind _player (Variables|Components|GetPlayer))
  (bind _player_2 (Variables|Components|GetPlayer))
  (bind _player_3 (Variables|Components|GetPlayer))
  (bind _springarm (Variables|Default|GetSpringArm))
  (bind _springarm_2 (Variables|Default|GetSpringArm))
  (bind _camautorotationspeed (Variables|Editable|GetCamAutoRotationSpeed))
  (bind _returnvalue (Math|Vector|GetRightVector _playercamera))
  (bind _returnvalue_2 (Transformation|GetVelocity _player))
  (bind _returnvalue_3 (Transformation|GetWorldRotation _springarm))
  (bind _returnvalue_4 (Transformation|GetActorLocation _player_3))
  (bind _directioncontrol (Variables|/Game/Blueprints/Character/BP_Player.BP_Player_C|GetDirectionControl _player_2))
  (bind _returnvalue_5 (Math|Vector|GetForwardVector _directioncontrol))
  (bind _returnvalue_6 (Math|Vector|DotProduct _returnvalue_5 _returnvalue))
  (bind _returnvalue_7 (Math|Float|Absolute(Float) _returnvalue_6))
  (bind _returnvalue_8 (* _camautorotationspeed _returnvalue_7))
  (if (Math|Boolean|ANDBoolean (not (Utilities|Operators|EqualEqual (Math|Vector|GetForwardVector (Transformation|GetWorldRotation (Variables|Default|GetPlayerCamera))) (* (Transformation|GetActorUpVector (Variables|Components|GetPlayer)) -1.0) (Variables|Editable|GetFaceDownRotationThreshold))) (not (Variables|/Game/Blueprints/Character/BP_Player.BP_Player_C|GetPlayerMovesCamera _player)) (> (Math|Vector2D|Vector2DLength (Math|Vector2D|MakeVector2D (.x _returnvalue_2) (.y _returnvalue_2))) 2e+02) (Variables|/Game/Blueprints/Character/BP_Player.BP_Player_C|GetPlayerMoves _player))
    (Transformation|SetWorldRotation (Variables|Default|GetSpringArm) (Math|Rotator|MakeRotator (.roll _returnvalue_3) (.pitch _returnvalue_3) (.yaw (Math|Interpolation|RInterpTo (Transformation|GetWorldRotation _springarm_2) (Math|Rotator|FindLookatRotation (Transformation|GetWorldLocation _springarm_2) (Utilities|Select :Index (Variables|Default|GetCameraStates) :NewEnumerator0 _returnvalue_4 :NewEnumerator1 _returnvalue_4 :NewEnumerator2 "0, 0, 0" :NewEnumerator3 "0, 0, 0" :NewEnumerator4 (Variables|Default|GetLockedOnTargetLocation))) (Variables|Private|GetDelta%20Seconds) (Utilities|Select :Index (Variables|Default|GetCameraStates) :NewEnumerator0 _returnvalue_8 :NewEnumerator1 _returnvalue_8 :NewEnumerator2 _returnvalue_8 :NewEnumerator3 _returnvalue_8 :NewEnumerator4 (Variables|Default|GetTargetingRotationSpeed))))) false false)))

(fn LookatTarget
  (bind _returnvalue (Utilities|InnerZoneTop))
  (bind _player (Variables|Components|GetPlayer))
  (bind _lookatoffset (Variables|Editable|GetLookAtOffset))
  (bind _characteroffset (Variables|Private|GetCharacterOffset))
  (bind _playercamera (Variables|Default|GetPlayerCamera))
  (bind _characterlookoffset_screen_ (Variables|Default|GetCharacterLookOffset%28Screen%29))
  (bind _returnvalue_2 (Transformation|GetActorLocation _player))
  (bind _returnvalue_3 (Transformation|GetWorldLocation _playercamera))
  (bind _returnvalue_4 (< (.y _characterlookoffset_screen_) _returnvalue))
  (bind _returnvalue_5 (+ _returnvalue_2 _lookatoffset))
  (bind _returnvalue_6 (select _returnvalue_4 _returnvalue_5 _characteroffset))
  (bind _returnvalue_7 (Math|Rotator|FindLookatRotation _returnvalue_3 _returnvalue_6))
  (Transformation|SetWorldRotation (Variables|Default|GetPlayerCamera) (Math|Interpolation|RInterpTo (Transformation|GetWorldRotation (Variables|Default|GetPlayerCamera)) (Math|Rotator|MakeRotator 0.0 (.pitch _returnvalue_7) (.yaw _returnvalue_7)) (Variables|Private|GetDelta%20Seconds) 2.0) false false))

(fn IsOutsideZone
  (return (not (Math|Float|InRange(Float) (.y (Variables|Default|GetCharacterLookOffset%28Screen%29)) (Utilities|InnerZoneTop) (Utilities|InnerZoneBottom) false false))))

(fn CalculateOffsetLocation
  (bind _player (Variables|Components|GetPlayer))
  (bind _returnvalue (Transformation|GetActorLocation _player))
  (Utilities|FlowControl|Sequence
    (:then_0
      (Variables|Default|SetCharacterLookOffset%28Screen%29 (/ (.ScreenPosition (Class|GameplayStatics|ProjectWorldtoScreen (Game|GetPlayerController 0) (Transformation|GetActorLocation (Variables|Components|GetPlayer)) true)) (Viewport|GetViewportSize)))
      (if (not (AI|Components|NavMovement|IsFalling (Variables|/Script/Engine.Character|GetCharacterMovement (Variables|Components|GetPlayer))))
        (Variables|Default|SetPreviousGroundHeight (Variables|Default|GetGroundHeight))
        (Variables|Default|SetGroundHeight (.Z (Math|Vector|BreakVector (.impactpoint (Default|TraceforGround (Variables|Components|GetPlayer))))))))
    (:then_1
      (if (Variables|Default|GetIsAiming?)
        (Variables|Private|SetCharacterOffset (+ (+ (Transformation|GetActorLocation (Variables|Components|GetPlayer)) (- (Variables|Editable|GetLookAtOffset) "0.000000,0.000000,100.000000")) (* (Math|Vector|GetRightVector (Variables|Default|GetSpringArm)) 2.5e+02)))
        (elif (Math|Boolean|ORBoolean (CallFunction|IsOutsideZone) (> (Variables|Default|GetGroundHeight) (select (AI|Components|NavMovement|IsFalling (Variables|/Script/Engine.Character|GetCharacterMovement (Variables|Components|GetPlayer))) (+ (Variables|Default|GetPreviousGroundHeight) (Variables|Default|GetGroundHeightTolerance)) (Variables|Default|GetPreviousGroundHeight))) (Utilities|Enum|Equal(Enum) (Variables|/Game/Blueprints/AbilityActorComponents/Player/MovementState/AC_MovementStateComponent.AC_MovementStateComponent_C|GetMovementState (Variables|/Game/Blueprints/Character/BP_Player.BP_Player_C|GetMovementStateComponent (Variables|Components|GetPlayer))) "NewEnumerator13"))
          (Variables|Private|SetCharacterOffset (+ (Transformation|GetActorLocation (Variables|Components|GetPlayer)) (Variables|Editable|GetLookAtOffset)))
          (else
            (Variables|Private|SetCharacterOffset (Math|Vector|MakeVector (.x _returnvalue) (.y _returnvalue) (.z (Variables|Private|GetCharacterOffset)))))))
      (return (Variables|Private|GetCharacterOffset)))))

(fn TraceforGround
  (bind _player (Variables|Components|GetPlayer))
  (bind _returnvalue (Transformation|GetActorLocation _player))
  (bind _capsulecomponent (Variables|/Script/Engine.Character|GetCapsuleComponent _player))
  (bind _returnvalue_2 (Components|Capsule|GetScaledCapsuleHalfHeight _capsulecomponent))
  (bind _returnvalue_3 (- (.z _returnvalue) _returnvalue_2))
  (bind _returnvalue_4 (Math|Vector|MakeVector (.x _returnvalue) (.y _returnvalue) _returnvalue_3))
  (bind (_outhit _returnvalue_5) (Collision|SphereTraceByChannel _returnvalue_4 (+ _returnvalue_4 (* (* (Transformation|GetActorUpVector (Variables|Components|GetPlayer)) -1.0) 2.5e+02)) (Variables|/Script/Engine.CapsuleComponent|GetCapsuleRadius _capsulecomponent) "TraceTypeQuery1" false 0 "ForOneFrame"))
  (if _returnvalue_5
    (return (.ImpactPoint (Collision|BreakHitResult _outhit)))))