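; Base enemy Blueprint that gives enemies health, healing and damage handling through a DamageSystemComponent.
; Its health getters, max health setter, Heal and TakeDamage functions are thin wrappers that forward to the component.
; BeginPlay binds to the component's OnDeath, and the Death event destroys the actor.
; A debug print of current health is left disconnected.
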(event Custom|Death
  (Actor|DestroyActor))

(event EventBeginPlay
  (EventDispatchers|BindEventtoOnDeath (Variables|Default|GetDamageSystemComponent) (EventDispatchers|CreateEvent :!event Custom|Death)))

(event Collision|EventActorBeginOverlap
  (params (OtherActor :type Actor%20Object%20Reference)))

(event EventTick
  (params (DeltaSeconds :type Float%20%28single-precision%29)))

(fn ConstructionScript)

(fn GetCurrentHealth
  (return (Variables|/Game/Blueprints/DamageSystem/AC_DamageSystemComponent.AC_DamageSystemComponent_C|GetHealthCurrent (Variables|Default|GetDamageSystemComponent))))

(fn GetMaxHealth
  (return (Variables|/Game/Blueprints/DamageSystem/AC_DamageSystemComponent.AC_DamageSystemComponent_C|GetHealthMax (Variables|Default|GetDamageSystemComponent))))

(fn Heal
  (params (Amount :type Integer))
  (bind _newhealth (Default|Heal (Variables|Default|GetDamageSystemComponent) Amount))
  (return _newhealth))

(fn SetMaxHealth
  (params (Amount :type Integer))
  (bind (_newmaxhealth _newhealth) (Default|SetMaxHealth (Variables|Default|GetDamageSystemComponent) Amount))
  (return _newmaxhealth _newhealth))

(fn TakeDamage
  (params (DamageInfo :type S%20Damage%20Info%20Structure))
  (bind _wasdamaged_ (Default|TakeDamage (Variables|Default|GetDamageSystemComponent) DamageInfo))
  (return _wasdamaged_))