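; BP_Checkpoint is a checkpoint actor that records the player's respawn transform and saves the game on overlap.
; An overlapping BPI_Interact actor supplies the player, whose LastSavedTransform takes the Arrow's transform; the checkpoint then turns active and blue.
; All inactive checkpoints are painted orange, though none has its Active flag cleared.
; On BeginPlay, it restores its active look if the saved transform matches its Arrow.
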(event EventBeginPlay
  (bind _savedata (Class|BPIGameInstance|GetSaveData(Message) (Game|GetGameInstance)))
  (if (== (Utilities|Struct|BreakS_PlayerStats (Utilities|Struct|BreakS_SaveData _savedata)) (Transformation|GetWorldTransform (Variables|Default|GetArrow)))
    (Variables|Default|SetActive true)
    (Rendering|Material|SetMaterial (Variables|Default|GetCylinder) 0 "/Game/Assets/Materials/Platforms/IMAT_BasicShape_Blue.IMAT_BasicShape_Blue")))

(event Collision|EventActorBeginOverlap
  (params (OtherActor :type Actor%20Object%20Reference))
  (if (Utilities|DoesObjectImplementInterface OtherActor "/Game/Blueprints/AbilityActorComponents/Player/Collection/BPI_Interact.BPI_Interact_C")
    (bind _player (Class|BPIInteract|GetPlayer(Message) OtherActor))
    (Variables|Default|SetPlayer _player)
    (Utilities|IsValid _player
      (:Is%20Valid
        (Variables|/Game/Blueprints/Character/BP_Player.BP_Player_C|SetLastSavedTransform _player (Transformation|GetWorldTransform (Variables|Default|GetArrow)))
        (Variables|Default|SetActive true)
        (Rendering|Material|SetMaterial (Variables|Default|GetCylinder) 0 "/Game/Assets/Materials/Platforms/IMAT_BasicShape_Blue.IMAT_BasicShape_Blue")
        (bind _outactors (Actor|GetAllActorsOfClass "BP_Checkpoint_C"))
        (for _array_element _outactors
          (if (not (Variables|BP_Checkpoint_C|GetActive _array_element))
            (Rendering|Material|SetMaterial (Variables|BP_Checkpoint_C|GetCylinder _array_element) 0 "/Game/Assets/Materials/Platforms/IMAT_BasicShape_Orange.IMAT_BasicShape_Orange")))
        (Class|BPIGameInstance|SaveGame(Message) (Game|GetGameInstance))))))

(fn ConstructionScript)