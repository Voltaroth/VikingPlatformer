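; BP_LeifGameMode is the game mode that initializes the player and HUD when a level begins.
; BeginPlay removes the game instance's loading screen, adds the player stats widget and applies saved stats to BP_Player.
; Portal arrivals clear their flag and keep the default spawn.
; Otherwise, a non-zero saved location restores the last saved transform on both character and controller, with zero treated as a new game.
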(event EventBeginPlay
  (bind _asbp_game_instance (Utilities|Casting|CastToBP_GameInstance (Game|GetGameInstance)))
  (bind _output_get (Variables|Default|SetGameInstance _asbp_game_instance))
  (Default|RemoveLoadingScreen _output_get)
  (bind _returnvalue (UserInterface|CreateWidget "/Game/Blueprints/Widgets/WBP_PlayerStats.WBP_PlayerStats_C" (Game|GetPlayerController 0)))
  (UserInterface|Viewport|AddtoViewport _returnvalue 0)
  ;[1 1 1] Set Player Stats
  (Default|SetPlayerStats (.AsBP%20Player (Utilities|Casting|CastToBP_Player (Game|GetPlayerCharacter 0))) (Utilities|Struct|BreakS_SaveData (Variables|/Game/Blueprints/Framework/BP_GameInstance.BP_GameInstance_C|GetSave%20Data (Variables|Default|GetGameInstance))))
  ;[1 1 1] if new game, set player transform to default transform OR if loaded game, set player transform to last saved transform
  (if (Variables|/Game/Blueprints/Framework/BP_GameInstance.BP_GameInstance_C|GetLoadedFromPortal? (Variables|Default|GetGameInstance))
    (Variables|/Game/Blueprints/Framework/BP_GameInstance.BP_GameInstance_C|SetLoadedFromPortal? (Variables|Default|GetGameInstance) false)
    (elif (not (Utilities|Operators|EqualEqual :A (.Location (Math|Transform|BreakTransform (Utilities|Struct|BreakS_SaveData (Variables|/Game/Blueprints/Framework/BP_GameInstance.BP_GameInstance_C|GetSave%20Data (Variables|Default|GetGameInstance)))))))
      (CallFunction|SetPlayerTransform (Utilities|Struct|BreakS_SaveData (Variables|/Game/Blueprints/Framework/BP_GameInstance.BP_GameInstance_C|GetSave%20Data (Variables|Default|GetGameInstance)))))))

(fn ConstructionScript)

(fn SetPlayerTransform
  (params (Transform :type Transform%20%28by%20ref%29))
  (Transformation|SetActorTransform (Game|GetPlayerCharacter 0) Transform)
  (Transformation|SetActorTransform (Game|GetPlayerController 0) Transform))