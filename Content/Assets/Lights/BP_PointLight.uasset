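; BP_PointLight is a placeable light actor that pairs a PointLight with a Sphere mesh sharing its color.
; The construction script passes color times strength and a separate opacity to the Sphere through Custom Primitive Data.
; It also sets the light's color and its intensity in lumens from the actor's variables.
; The event graph holds only disabled stub events, so the Blueprint adds no runtime logic.
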(event EventBeginPlay)

(event Collision|EventActorBeginOverlap
  (params (OtherActor :type Actor%20Object%20Reference)))

(event EventTick
  (params (DeltaSeconds :type Float%20%28single-precision%29)))

(fn ConstructionScript
  (bind _color (Variables|Default|GetColor))
  (bind _pointlight (Variables|Default|GetPointLight))
  (bind (_r _g _b) (Math|Color|BreakColor _color))
  (Rendering|Material|SetCustomPrimitiveDataVector3 (Variables|Default|GetSphere) 0 (* (Math|Vector|MakeVector _r _g _b) (Variables|Default|GetStrength)))
  (Rendering|Material|SetCustomPrimitiveDataFloat (Variables|Default|GetSphere) 3 (Variables|Default|GetOpacity))
  (Rendering|Components|Light|SetLightColor _pointlight (Variables|Default|GetColor) true)
  (Rendering|Components|Light|SetIntensity _pointlight (Variables|Default|GetLightIntensity))
  (Class|LocalLightComponent|SetIntensityUnits _pointlight "Lumens"))